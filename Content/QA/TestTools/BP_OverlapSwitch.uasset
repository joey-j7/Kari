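; BP_OverlapSwitch is a QA test tool: an on/off switch toggled by overlapping its collision component.
; On begin overlap, it compares the other actor to the one GetActorOfClass finds for OverlapActor, so only that single instance triggers it.
; Each match flips OnOff and swaps the sphere's material to green for on or red for off.
; The construction script is empty, leaving a SetSphereRadius call unconnected.
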(event OnComponentBeginOverlap(Collision)
  (params (OverlappedComponent :type Primitive%20Component%20Object%20Reference) (OtherActor :type Actor%20Object%20Reference) (OtherComp :type Primitive%20Component%20Object%20Reference) (OtherBodyIndex :type Integer) (bFromSweep :type Boolean) (SweepResult :type Hit%20Result%20Structure%20%28by%20ref%29))
  (bind _sphere (Variables|Default|GetSphere))
  (bind _returnvalue (Actor|GetActorOfClass (Variables|Default|GetOverlapActor)))
  (if (== _returnvalue OtherActor)
    (bind _output_get (Variables|Default|SetOn/Off (not (Variables|Default|GetOn/Off))))
    (if _output_get
      (Rendering|Material|SetMaterial _sphere 0 "/Game/QA/TestTools/M_SwitchColorGreen.M_SwitchColorGreen")
      (else
        (Rendering|Material|SetMaterial _sphere 0 "/Game/QA/TestTools/M_SwitchColorRed.M_SwitchColorRed")))))

(fn ConstructionScript)