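; Temporary QA test actor that smoke-tests NPC dialogue interaction by driving it automatically.
; On BeginPlay it calls Confirm on BP_Kari, then checks whether the first found BP_NPC is interacting.
; If so, a looping timer calls OnConfirm on the dialogue widget until the interaction ends, then quits the game.
; It also quits if no interaction starts, as the failed-test FinishTest nodes are unconnected.
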(event Custom|InteractionTest
  (if (Variables|Default|GetInteractionInitiated)
    (Class|NavigatableWidget|OnConfirm (Variables|Default|GetDialogueWidgetReference))
    (if (Variables|/Script/Kari.DefaultNPC|GetIsInteracting (Variables|Default|GetNPCReference))
      (Development|PrintString "Interaction is still going,")
      (else
        (Variables|Default|SetInteractionInitiated false)
        (Game|QuitGame 0 "Quit" false)))))

(event EventBeginPlay
  (bind _returnvalue (Actor|GetActorOfClass "/Game/Characters/Villagers/BP_NPC.BP_NPC_C"))
  (Variables|Default|SetNPCReference _returnvalue)
  (bind _returnvalue_2 (Actor|GetActorOfClass "/Game/Characters/Playable/Kari/BP_Kari.BP_Kari_C"))
  (Class|DefaultPlayer|Confirm _returnvalue_2)
  (if (Variables|/Script/Kari.DefaultNPC|GetIsInteracting (Variables|Default|GetNPCReference))
    (bind _output_get (Variables|Default|SetInteractionInitiated true))
    (bind _foundwidgets (Widget|GetAllWidgetsOfClass "/Game/UI/Dialogues/WBP_DialogueWidget.WBP_DialogueWidget_C" true))
    (Variables|Default|SetDialogueWidgetReference (Utilities|Array|Get(acopy) _foundwidgets))
    (Utilities|Time|SetTimerbyEvent (delegate Custom|InteractionTest) 3.0 _output_get)
    (else
      (Game|QuitGame 0 "Quit" false))))

(fn ConstructionScript)