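; Blizzard system actor that starts and stops the storm, restores it on BeginPlay and offers screen-faded apply/revert events.
; Starting swaps Forest to its poststorm level, freezes time at midnight, changes Kari's blessing drain and starts audio, post-process and player-attached weather VFX.
; An intensity timeline feeds particles, MPC_Storm and timers for thunder and rain splashes.
; Both trace random screen points outside Kari's safe radius; thunder adds material flicker and camera shake.
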(event OnComponentEndOverlap(Box)
  (params (OverlappedComponent :type Primitive%20Component%20Object%20Reference) (OtherActor :type Actor%20Object%20Reference) (OtherComp :type Primitive%20Component%20Object%20Reference) (OtherBodyIndex :type Integer))
  ;[1 1 1] Box Trigger for debug
)

(event OnComponentBeginOverlap(Box)
  (params (OverlappedComponent :type Primitive%20Component%20Object%20Reference) (OtherActor :type Actor%20Object%20Reference) (OtherComp :type Primitive%20Component%20Object%20Reference) (OtherBodyIndex :type Integer) (bFromSweep :type Boolean) (SweepResult :type Hit%20Result%20Structure%20%28by%20ref%29))
  ;[1 1 1] Box Trigger for debug
  (if (Utilities|Enum|Equal(Enum) (Collision|GetCollisionObjectType OtherComp) "ECC_Pawn")
    (Variables|/Script/Kari.DefaultGameInstance|SetIsStormActive (Variables|Default|GetGameInstance) true)
    (CallFunction|StartStorm)))

(event Custom|Thunder%20Strike
  (bind _thunder_frequency (Variables|Thunder|GetThunder%20Frequency))
  ;[1 1 1] Thunder
  (Utilities|FlowControl|RetriggerableDelay (Math|Random|RandomFloatinRange (/ _thunder_frequency 2.0) _thunder_frequency))
  (CallFunction|PrepStrike (Math|Random|RandomFloatinRange (Variables|Thunder|GetThunder%20Min%20Duration) (Variables|Thunder|GetThunder%20Max%20Duration))))

(event Custom|Start%20Post%20Process
  ;[1 1 1] Post Process Lerp
  (bind _blend_alpha (Timeline|Post%20Process%20lerp Play)
    (:Update
      (Variables|/Script/Engine.PostProcessComponent|SetBlendWeight (Variables|Default|GetPostProcess) _blend_alpha))))

(event Custom|OnApplyFaded
  (bind _gameinstance (Variables|Default|GetGameInstance))
  (bind _fadecontroller (Variables|Default|GetFadeController))
  (bind _timemanager (Variables|/Script/Kari.DefaultGameInstance|GetTimeManager _gameinstance))
  (Class|TimeManager|SetTimeSpeed _timemanager 0.0)
  (Class|TimeManager|SetTime _timemanager)
  (CallFunction|StartStorm)
  (Utilities|FlowControl|Delay 0.2)
  (Class|FadeController|ScreenFadein _fadecontroller 0.0)
  (EventDispatchers|BindEventtoOnScreenClear _fadecontroller (delegate Custom|ApplyOnClear)))

(event Custom|RevertOnClear
  (Input|EnableInput (Game|GetPlayerController 0) 0)
  (Input|EnableInput (Game|GetPlayerCharacter 0) 0))

(event Custom|ApplyOnClear
  (Input|EnableInput (Game|GetPlayerController 0) 0)
  (Input|EnableInput (Game|GetPlayerCharacter 0) 0))

(event Custom|Stop%20Post%20Process
  ;[1 1 1] Post Process Lerp
  (bind _blend_alpha (Timeline|Post%20Process%20lerp Reverse)
    (:Update
      (Variables|/Script/Engine.PostProcessComponent|SetBlendWeight (Variables|Default|GetPostProcess) _blend_alpha))))

(event Custom|Prep%20Strike
  (params (Flicker%20Duration :type Float%20%28single-precision%29))
  ;[1 1 1] Thunder
  (CallFunction|LightFlicker Flicker%20Duration)
  (Utilities|FlowControl|RetriggerableDelay Flicker%20Duration)
  (CallFunction|LightFlicker (* Flicker%20Duration -1.0))
  (Utilities|FlowControl|RetriggerableDelay (Math|Random|RandomFloatinRange Flicker%20Duration (Math|Float|Sqrt Flicker%20Duration)))
  (CallFunction|LightingStrikeVFX))

(event Custom|Start%20Storm
  (bind _wind_direction (Variables|Default|GetWind%20Direction))
  (bind _gameinstance (Variables|Default|GetGameInstance))
  (bind _gameinstance_2 (Variables|Default|GetGameInstance))
  (bind _intensity_max_time (Variables|Default|GetIntensity%20Max%20Time))
  (bind _gameinstance_3 (Variables|Default|GetGameInstance))
  (bind _audiomanager (Variables|/Script/Kari.DefaultGameInstance|GetAudioManager _gameinstance))
  (bind _audiomanager_2 (Variables|/Script/Kari.DefaultGameInstance|GetAudioManager _gameinstance_2))
  (bind _timemanager (Variables|/Script/Kari.DefaultGameInstance|GetTimeManager _gameinstance_3))
  (if (not (Variables|Default|GetIsActive))
    (Game|LoadStreamLevel(byName) "/Game/Levels/Forest/L_Forest_Poststorm" true true)
    (Game|UnloadStreamLevel(byName) "/Game/Levels/Forest/L_Forest_Prestorm" true)
    (Class|TimeManager|SetTimeSpeed _timemanager 0.0)
    (Class|TimeManager|SetTime _timemanager)
    (bind _asbp_kari (Utilities|Casting|CastToBP_Kari (Game|GetPlayerCharacter 0))
      (:then
        (Default|ApplyStormBlessingDrain _asbp_kari))
      (:CastFailed
        _))
    (Variables|/Script/Kari.DefaultGameInstance|SetIsStormActive _gameinstance_3 true)
    (Variables|Default|SetIsActive true)
    (Class|AudioManager|ClearAmbience _audiomanager_2)
    ;[1 1 1] Rain SFX
    (bind _returnvalue (Class|AudioManager|Play _audiomanager_2 (Utilities|Array|MakeArray "Global/General/Storm/Rain.amb") true 0 0 1.0 1.0 (Math|Random|RandomFloatinRange -6e+01 0.0) 0.1 false))
    (Class|Playlist|SetVolume _returnvalue 0.0)
    (Class|Playlist|FadeVolume _returnvalue 1.0 _intensity_max_time false)
    ;[1 1 1] Wind SFX
    (bind _returnvalue_2 (Class|AudioManager|Play _audiomanager_2 (Utilities|Array|MakeArray "Global/General/Storm/Wind.amb") true 0 0 1.0 1.0 (Math|Random|RandomFloatinRange -4e+01 0.0) 0.2 false))
    (Class|Playlist|SetVolume _returnvalue_2 0.0)
    (Class|Playlist|FadeVolume _returnvalue_2 1.0 (Variables|Default|GetIntensity%20Max%20Time) false)
    (bind _returnvalue_3 (Class|AudioManager|Play _audiomanager (Utilities|Array|MakeArray "Events/Queues/Storm.bgm") true 820245 4600750 1.0 1.0 0.0 1.2 false))
    (Class|AudioManager|SetOverrideBGM _audiomanager _returnvalue_3)
    (Utilities|FlowControl|Sequence
      (:then_0
        (CallFunction|StartPostProcess)
        (CallFunction|StartPersistentVFX)
        (Rendering|Material|SetVectorParameterValue "/Game/StormSystem/Materials/MPC_Storm.MPC_Storm" "WindDirection" (Math|Conversions|ToLinearColor(Vector) (Math|Rotator|GetRotationXVector (Math|Rotator|MakeRotator (.roll (.rotation _wind_direction)) 0.0 (.yaw (.rotation _wind_direction))))) :!class /Script/Engine.KismetMaterialLibrary))
      (:then_1
        (Components|Timeline|SetPlayRate (Variables|Default|GetIntensity%20Curve) (/ 1.0 _intensity_max_time))
        (bind (_direction _intensity) (Timeline|Intensity%20Curve PlayFromStart)
          (:Update
            (CallFunction|UpdateIntensity _intensity _direction)))))))

(event Custom|Stop%20Storm
  (if (Variables|Default|GetIsActive)
    (Class|TimeManager|SetTimeSpeed (Variables|/Script/Kari.DefaultGameInstance|GetTimeManager (Variables|Default|GetGameInstance)) 1e+02)
    (bind _asbp_kari (Utilities|Casting|CastToBP_Kari (Game|GetPlayerCharacter 0))
      (:then
        (Default|ApplyDefaultBlessingDrain _asbp_kari))
      (:CastFailed
        _))
    (Variables|Default|SetIsActive false)
    (Utilities|FlowControl|Sequence
      (:then_0
        (Utilities|Time|ClearandInvalidateTimerbyHandle (Variables|Runtime|GetTH_LightingStrike))
        (Utilities|Time|ClearandInvalidateTimerbyHandle (Variables|Runtime|GetTH_RainSplash))
        (CallFunction|ReverseIntensity))
      (:then_1
        (CallFunction|StopPostProcess)
        (CallFunction|StopPersistentVFX)))))

(event Custom|Reverse%20Intensity
  (bind (_direction _intensity) (Timeline|Intensity%20Curve Reverse)
    (:Update
      (CallFunction|UpdateIntensity _intensity _direction))))

(event Custom|ApplyStormState
  (bind _fadecontroller (Variables|Default|GetFadeController))
  (Class|FadeController|ScreenFadeOut _fadecontroller 0.0)
  (EventDispatchers|BindEventtoOnScreenFaded _fadecontroller (delegate Custom|OnApplyFaded)))

(event Custom|RevertStormState
  (bind _fadecontroller (Variables|Default|GetFadeController))
  (Class|FadeController|ScreenFadeOut _fadecontroller 0.0)
  (EventDispatchers|BindEventtoOnScreenClear _fadecontroller (delegate Custom|OnRevertFaded)))

(event Custom|OnRevertFaded
  (bind _fadecontroller (Variables|Default|GetFadeController))
  (CallFunction|StopStorm)
  (Utilities|FlowControl|Delay 0.2)
  (Class|FadeController|ScreenFadein _fadecontroller 0.0)
  (EventDispatchers|BindEventtoOnScreenClear _fadecontroller (delegate Custom|RevertOnClear)))

(event EventBeginPlay
  (bind _returnvalue (Actor|GetActorOfClass "/Game/General/BP_FadeController.BP_FadeController_C"))
  (Variables|Default|SetFadeController _returnvalue)
  (Collision|SetCollisionEnabled (Variables|Default|GetBox) "NoCollision")
  (bind _asgi_default_game_instance (Utilities|Casting|CastToGI_DefaultGameInstance (Game|GetGameInstance)))
  (bind _output_get (Variables|Default|SetGameInstance _asgi_default_game_instance))
  (if (Variables|/Script/Kari.DefaultGameInstance|GetIsStormActive _output_get)
    (Class|AudioManager|ClearAmbience (Variables|/Script/Kari.DefaultGameInstance|GetAudioManager _output_get))
    (Utilities|FlowControl|Delay 0.1)
    (Variables|Default|SetIntensity%20Max%20Time 0.01)
    (CallFunction|StartStorm)))

(fn ConstructionScript
  (Transformation|SetRelativeTransform (Variables|Default|GetArrow) (Variables|Default|GetWind%20Direction) false false))

(fn LightingStrikeVFX
  (bind _returnvalue (Game|GetPlayerController 0))
  (bind (_sizex _sizey) (HUD|GetViewportSize _returnvalue))
  (bind _returnvalue_2 (Math|Conversions|ToFloat(Integer) _sizex))
  (bind _returnvalue_3 (Math|Conversions|ToFloat(Integer) _sizey))
  (bind _returnvalue_4 (Math|Random|RandomFloatinRange 0.0 _returnvalue_2))
  (bind _returnvalue_5 (Math|Random|RandomFloatinRange _returnvalue_3 0.0))
  (bind (_worldlocation _worlddirection) (Class|PlayerController|DeprojectScreenPositiontoWorld _returnvalue _returnvalue_4 _returnvalue_5))
  (bind _output_get (LocalVariables|SetHitStart _worldlocation))
  (bind (_outhit _returnvalue_6) (Collision|LineTraceByChannel _output_get (+ _worldlocation (* _worlddirection 1e+04)) "TraceTypeQuery1" false 0 "None" :!label _label))
  (if _returnvalue_6
    (bind _output_get_2 (LocalVariables|SetHit%20Location (.Location (Collision|BreakHitResult _outhit))))
    (LocalVariables|SetDistanceToKari (Math|Vector|Distance2D(Vector) _output_get_2 (Transformation|GetActorLocation (Game|Player|GetPlayerPawn 0))))
    (if (>= (Math|Vector|Distance2D(Vector) _output_get_2 (Transformation|GetActorLocation (Game|Player|GetPlayerPawn 0))) (Variables|Default|GetSafe%20Distance%20around%20Kari))
      (Class|PlayerCameraManager|PlayCameraShake (Game|GetPlayerCameraManager 0) (Variables|Thunder|GetThunder%20Shake) (Math|Float|MapRangeClamped (LocalVariables|GetDistanceToKari) (Variables|Default|GetSafe%20Distance%20around%20Kari) 8e+03 (Variables|Thunder|GetMax%20Thunder%20Shake%20Intentisty) 0.0) "CameraLocal" "0, 0, 0")
      (Class|AudioManager|Play (Variables|/Script/Kari.DefaultGameInstance|GetAudioManager (Variables|Default|GetGameInstance)) (Utilities|Array|MakeArray "Global/General/Storm/Thunder0" "Global/General/Storm/Thunder1" "Global/General/Storm/Thunder2") false 0 0 0.8 1.2 0.0 0.3 true)
      (else
        (goto _label)))))

(fn LightFlicker
  (params (Effect%20Duration :type Float%20%28single-precision%29))
  (Rendering|Material|SetScalarParameterValue "/Game/StormSystem/Materials/MPC_Storm.MPC_Storm" "Start Time" (Utilities|Time|GetGameTimeinSeconds) :!class /Script/Engine.KismetMaterialLibrary)
  (Rendering|Material|SetScalarParameterValue "/Game/StormSystem/Materials/MPC_Storm.MPC_Storm" "Duration" Effect%20Duration :!class /Script/Engine.KismetMaterialLibrary)
  (return))

(fn StartPersistentVFX
  (bind _returnvalue (Game|Player|GetPlayerPawn 0))
  (bind _arrow (Variables|Default|GetArrow))
  (bind _returnvalue_2 (Math|Vector|GetForwardVector _arrow))
  (bind _returnvalue_3 (Math|Conversions|RotationFromXVector _returnvalue_2))
  (bind _returnvalue_4 (Effects|SpawnEmitterAttached (Variables|Default|GetRain%20VFX) (Variables|/Script/Engine.Actor|GetRootComponent _returnvalue) "None" (Math|Vector|Lerp(Vector) (Transformation|GetActorLocation _returnvalue) (Camera|GetCameraLocation (Game|GetPlayerCameraManager 0)) 0.5) (Math|Rotator|MakeRotfromZ (* (Math|Vector|GetForwardVector (Variables|Default|GetArrow)) -1.0)) "1.000000,1.000000,1.000000" "KeepWorldPosition"))
  (Utilities|Array|AddUnique (Variables|Runtime|GetSpawned%20PS) _returnvalue_4)
  (for _array_element (Utilities|Array|MakeArray (Variables|Default|GetLeaves%20VFX) (Variables|Default|GetWind%20VFX))
    (bind _returnvalue_5 (Niagara|SpawnSystemAttached _array_element (Variables|/Script/Engine.Actor|GetRootComponent (Game|Player|GetPlayerPawn 0)) "None" "0, 0, 0" (Math|Rotator|MakeRotator (.roll _returnvalue_3) 0.0 (.yaw _returnvalue_3)) "SnapToTarget" true))
    (Utilities|Array|AddUnique (Variables|Runtime|GetSpawned%20PS) _returnvalue_5)
    (Effects|Components|ParticleSystem|SetFloatParameter _returnvalue_5 "User.IntensityParam" (Variables|Default|GetIntensity))))

(fn StopPersistentVFX
  (bind _spawned_ps (Variables|Runtime|GetSpawned%20PS))
  (if (!= (Utilities|Array|Length (Variables|Runtime|GetSpawned%20PS)) -1)
    (for _array_element _spawned_ps
      (bind _asactor_component (Utilities|Casting|CastToActorComponent _array_element))
      (Components|DestroyComponent _asactor_component))
    (Utilities|Array|Clear _spawned_ps)
    (return)
    (else
      (return))))

(fn RainSplashes
  (bind _returnvalue (Game|GetPlayerController 0))
  (bind (_sizex _sizey) (HUD|GetViewportSize _returnvalue))
  (bind _returnvalue_2 (Math|Conversions|ToFloat(Integer) _sizex))
  (bind _returnvalue_3 (Math|Conversions|ToFloat(Integer) _sizey))
  (bind _returnvalue_4 (Math|Random|RandomFloatinRange 0.0 _returnvalue_2))
  (bind _returnvalue_5 (Math|Random|RandomFloatinRange _returnvalue_3 0.0))
  (bind (_worldlocation _worlddirection) (Class|PlayerController|DeprojectScreenPositiontoWorld _returnvalue _returnvalue_4 _returnvalue_5))
  (bind _output_get (LocalVariables|SetHitStart _worldlocation))
  (bind (_outhit _returnvalue_6) (Collision|LineTraceByChannel _output_get (+ _worldlocation (* _worlddirection 3e+03)) "TraceTypeQuery1" true (Utilities|Array|MakeArray (Game|Player|GetPlayerPawn 0)) "None" :!label _label))
  (if _returnvalue_6
    (bind _output_get_2 (LocalVariables|SetHit%20Location (.Location (Collision|BreakHitResult _outhit))))
    (LocalVariables|SetDistanceToKari (Math|Vector|Distance2D(Vector) _output_get_2 (Transformation|GetActorLocation (Game|Player|GetPlayerPawn 0))))
    (if (and (>= (Math|Vector|Distance2D(Vector) _output_get_2 (Transformation|GetActorLocation (Game|Player|GetPlayerPawn 0))) (Variables|Default|GetSafe%20Distance%20around%20Kari)) (> (Math|Vector|Distance(Vector) (Camera|GetCameraLocation (Game|GetPlayerCameraManager 0)) (.Location (Collision|BreakHitResult _outhit))) 1e+03))
      (Effects|SpawnEmitteratLocation (select (== (.PhysMat (Collision|BreakHitResult _outhit)) "/Engine/EngineMaterials/PhysMat_Ice.PhysMat_Ice") "/Game/StormSystem/VFX/Splash/PFX_WaterSplash_New.PFX_WaterSplash_New" "/Game/StormSystem/VFX/Splash/PFX_RainSplash_New.PFX_RainSplash_New") (LocalVariables|GetHit%20Location) (Math|Rotator|MakeRotfromZ (.Normal (Collision|BreakHitResult _outhit))) "1.000000,1.000000,1.000000" true "AutoRelease")
      (return)
      (else
        (goto _label)))
    (else
      (return))))

(fn UpdateIntensity
  (params (Intensity :type Float%20%28single-precision%29) (Direction :type ETimelineDirection%20Enum :default "Forward"))
  (Variables|Default|SetIntensity Intensity)
  (for _array_element (Variables|Runtime|GetSpawned%20PS)
    (bind _asparticle_system_component (Utilities|Casting|CastToParticleSystemComponent _array_element)
      (:then
        (Effects|Components|ParticleSystem|SetFloatParameter _asparticle_system_component "Intensity" (Variables|Default|GetIntensity))
        (Effects|Components|ParticleSystem|SetColorParameter _asparticle_system_component "Intensity" (Math|Conversions|ToLinearColor(Float) (Variables|Default|GetIntensity))))
      (:CastFailed
        (bind _asfxsystem_component (Utilities|Casting|CastToFXSystemComponent _array_element))
        (Effects|Components|ParticleSystem|SetFloatParameter _asfxsystem_component "User.IntensityParam" (Variables|Default|GetIntensity)))))
  (Rendering|Material|SetScalarParameterValue "/Game/StormSystem/Materials/MPC_Storm.MPC_Storm" "Intensity" (Variables|Default|GetIntensity) :!class /Script/Engine.KismetMaterialLibrary)
  (if (Utilities|Enum|Equal(Enum) Direction "Forward")
    (CallFunction|UpdateTimers (Math|Float|Lerp (Variables|Thunder|GetThunder%20Frequency%20Max) (Variables|Thunder|GetThunder%20Frequency%20Min) (Variables|Default|GetIntensity)) (Math|Float|Lerp (Variables|Thunder|GetSplash%20Frequency%20Max) (Variables|Thunder|GetSplash%20Frequency%20Min) (Variables|Default|GetIntensity)))))

(fn UpdateTimers
  (params (Thunder%20Frequency :type Float%20%28single-precision%29) (Splash%20Frequency :type Float%20%28single-precision%29))
  (bind _output_get (Variables|Thunder|SetThunder%20Frequency Thunder%20Frequency))
  (bind _returnvalue (Utilities|Time|SetTimerbyFunctionName 0 "Thunder Strike" _output_get true 1.0 0.1))
  (Variables|Runtime|SetTH_LightingStrike _returnvalue)
  (bind _output_get_2 (Variables|Default|SetSplash%20Frequency Splash%20Frequency))
  (bind _returnvalue_2 (Utilities|Time|SetTimerbyFunctionName 0 "Rain Splashes" _output_get_2 true 1.0 0.1))
  (Variables|Runtime|SetTH_RainSplash _returnvalue_2))