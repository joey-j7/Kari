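; Ghost path child Blueprint: a path that becomes visible and solid when the player has ghost pass access.
; BeginPlay applies the lit material and opens the path if access is granted, also disabling its blocking volume.
; Detection box overlaps by BP_Kari recheck access, showing or hiding the path, and flag proximity.
; While near, Tick writes a raised player location to a material parameter collection for a sphere mask.
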(event OnComponentBeginOverlap(DetectionBox)
  (params (OverlappedComponent :type Primitive%20Component%20Object%20Reference) (OtherActor :type Actor%20Object%20Reference) (OtherComp :type Primitive%20Component%20Object%20Reference) (OtherBodyIndex :type Integer) (bFromSweep :type Boolean) (SweepResult :type Hit%20Result%20Structure%20%28by%20ref%29))
  (bind _path (Variables|Default|GetPath))
  ;[1 1 1] This works but I want to make it better. But LL came up
  (Utilities|Casting|CastToBP_Kari OtherActor)
  (Variables|Default|SetPlayerNearGhostPath true)
  (bind _returnvalue (Class|PersistenceLibrary|GetGhostPassAccess))
  ;[1 1 1] Checks if player has Key item & changes the state of the path accordingly accordingly
  (if _returnvalue
    (Development|SetHiddeninGame _path false false)
    (Collision|SetCollisionEnabled _path "QueryAndPhysics")
    (Collision|SetCollisionEnabled (Variables|Default|GetBlockingVolume) "NoCollision")
    (else
      (Development|SetHiddeninGame _path true false)
      (Collision|SetCollisionEnabled _path "NoCollision"))))

(event OnComponentEndOverlap(DetectionBox)
  (params (OverlappedComponent :type Primitive%20Component%20Object%20Reference) (OtherActor :type Actor%20Object%20Reference) (OtherComp :type Primitive%20Component%20Object%20Reference) (OtherBodyIndex :type Integer))
  (Utilities|Casting|CastToBP_Kari OtherActor)
  (Variables|Default|SetPlayerNearGhostPath false))

(event EventTick
  (params (DeltaSeconds :type Float%20%28single-precision%29))
  (bind _returnvalue (Game|Player|GetPlayerPawn 0))
  (bind _returnvalue_2 (Transformation|GetActorLocation _returnvalue))
  ;[1 1 1] Gets player's location to
  (if (Variables|Default|GetPlayerNearGhostPath)
    (Rendering|Material|SetVectorParameterValue "/Game/Gameplay/Colliders/Events/MPC_MaterialVariables.MPC_MaterialVariables" "playerLocation" (Math|Conversions|ToLinearColor(Vector) (Math|Vector|MakeVector (.x _returnvalue_2) (.y _returnvalue_2) (+ (.z _returnvalue_2) 1.5e+02))) :!class /Script/Engine.KismetMaterialLibrary)))

(event EventBeginPlay
  (bind _path (Variables|Default|GetPath))
  ;[1 1 1] This works but I want to make it better. But LL came up
  (Rendering|Material|SetMaterial (Variables|Default|GetPath) 0 "/Game/Gameplay/Gates/GhostPath/MAT_GhostlyLitPath.MAT_GhostlyLitPath")
  (bind _returnvalue (Class|PersistenceLibrary|GetGhostPassAccess))
  (if _returnvalue
    ;[1 1 1] Checks if player has Key item & changes the state of the path accordingly accordingly
    (Development|SetHiddeninGame _path false false)
    (Collision|SetCollisionEnabled _path "QueryAndPhysics")
    (Collision|SetCollisionEnabled (Variables|Default|GetBlockingVolume) "NoCollision")))

(fn ConstructionScript
  (|CallParentFunction))