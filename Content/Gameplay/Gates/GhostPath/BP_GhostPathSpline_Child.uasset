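; Spline-built ghost bridge that becomes visible and solid while BP_Kari is inside its capsule and has ghost pass access.
; Construction script lays spline mesh floor segments and invisible wall collision, aligns end caps and rocks, and stretches the capsule between the spline endpoints.
; Overlap toggles bridge visibility and collision, with box colliders enabled whenever it is closed.
; While open, Tick writes player location to a material parameter collection.
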(event OnComponentBeginOverlap(Capsule)
  (params (OverlappedComponent :type Primitive%20Component%20Object%20Reference) (OtherActor :type Actor%20Object%20Reference) (OtherComp :type Primitive%20Component%20Object%20Reference) (OtherBodyIndex :type Integer) (bFromSweep :type Boolean) (SweepResult :type Hit%20Result%20Structure%20%28by%20ref%29))
  (bind _bridgecapmeshes (Variables|Default|GetBridgeCapMeshes))
  (bind _boxcollisionarray (Variables|Default|GetBoxCollisionArray))
  (bind _bridgefloormeshes (Variables|Default|GetBridgeFloorMeshes))
  (bind _bridgewallcollisionarray (Variables|Default|GetBridgeWallCollisionArray))
  (Utilities|Casting|CastToBP_Kari OtherActor)
  (Variables|Default|SetPlayerNearGhostPath true)
  ;[0 0 0] Checks if player has Key item & changes the state of the path accordingly
  (bind _returnvalue (Class|PersistenceLibrary|GetGhostPassAccess))
  (bind _output_get (Variables|Default|SetPlayerHasAccess _returnvalue))
  (if _output_get
    (Utilities|FlowControl|Sequence
      (:then_0
        (for _array_element _bridgecapmeshes
          (Development|SetHiddeninGame _array_element false false)
          (Collision|SetCollisionEnabled _array_element "QueryAndPhysics")))
      (:then_1
        (for _array_element_2 _bridgefloormeshes
          (Development|SetHiddeninGame _array_element_2 false false)
          (Collision|SetCollisionEnabled _array_element_2 "QueryAndPhysics")))
      (:then_2
        (for _array_element_3 _bridgewallcollisionarray
          (Collision|SetCollisionEnabled _array_element_3 (Variables|Default|GetBridgeWallCollision))))
      (:then_3
        (for _array_element_4 _boxcollisionarray
          (Collision|SetCollisionEnabled _array_element_4 "NoCollision"))))
    (else
      (Utilities|FlowControl|Sequence
        (:then_0
          (for _array_element_5 _bridgecapmeshes
            (Development|SetHiddeninGame _array_element_5 true false)
            (Collision|SetCollisionEnabled _array_element_5 "NoCollision")))
        (:then_1
          (for _array_element_6 _bridgefloormeshes
            (Development|SetHiddeninGame _array_element_6 true false)
            (Collision|SetCollisionEnabled _array_element_6 "NoCollision")))
        (:then_2
          (for _array_element_7 _bridgewallcollisionarray
            (Collision|SetCollisionEnabled _array_element_7 "NoCollision")))
        (:then_3
          (for _array_element_8 _boxcollisionarray
            (Collision|SetCollisionEnabled _array_element_8 "QueryAndPhysics")))))))

(event OnComponentEndOverlap(Capsule)
  (params (OverlappedComponent :type Primitive%20Component%20Object%20Reference) (OtherActor :type Actor%20Object%20Reference) (OtherComp :type Primitive%20Component%20Object%20Reference) (OtherBodyIndex :type Integer))
  (Utilities|Casting|CastToBP_Kari OtherActor)
  (Variables|Default|SetPlayerNearGhostPath false)
  ;[0 0 0] Checks if player has Key item & changes the state of the path accordingly
  (Utilities|FlowControl|Sequence
    (:then_0
      (for _array_element (Variables|Default|GetBridgeCapMeshes)
        (Development|SetHiddeninGame _array_element true false)
        (Collision|SetCollisionEnabled _array_element "NoCollision")))
    (:then_1
      (for _array_element_2 (Variables|Default|GetBridgeFloorMeshes)
        (Development|SetHiddeninGame _array_element_2 true false)
        (Collision|SetCollisionEnabled _array_element_2 "NoCollision")))
    (:then_2
      (for _array_element_3 (Variables|Default|GetBridgeWallCollisionArray)
        (Collision|SetCollisionEnabled _array_element_3 "NoCollision")))
    (:then_3
      (for _array_element_4 (Variables|Default|GetBoxCollisionArray)
        (Collision|SetCollisionEnabled _array_element_4 "QueryAndPhysics")))))

(event EventTick
  (params (DeltaSeconds :type Float%20%28single-precision%29))
  ;[0.04458 0.02211 0.1302] Gets player location and sets vector in material
  (if (and (Variables|Default|GetPlayerNearGhostPath) (Variables|Default|GetPlayerHasAccess))
    (Rendering|Material|SetVectorParameterValue "/Game/Gameplay/Colliders/Events/MPC_MaterialVariables.MPC_MaterialVariables" "PlayerLocationGhost" (Math|Conversions|ToLinearColor(Vector) (Transformation|GetActorLocation (Game|Player|GetPlayerPawn 0))) :!class /Script/Engine.KismetMaterialLibrary)))

(event EventBeginPlay
  (Variables|Default|SetPlayerHasAccess false)
  ;[0 0 0] Checks if player has Key item & changes the state of the path accordingly
  (Utilities|FlowControl|Sequence
    (:then_0
      (for _array_element (Variables|Default|GetBridgeCapMeshes)
        (Development|SetHiddeninGame _array_element true false)
        (Collision|SetCollisionEnabled _array_element "NoCollision")))
    (:then_1
      (for _array_element_2 (Variables|Default|GetBridgeFloorMeshes)
        (Development|SetHiddeninGame _array_element_2 true false)
        (Collision|SetCollisionEnabled _array_element_2 "NoCollision")))
    (:then_2
      (for _array_element_3 (Variables|Default|GetBridgeWallCollisionArray)
        (Collision|SetCollisionEnabled _array_element_3 "NoCollision")))
    (:then_3
      (for _array_element_4 (Variables|Default|GetBoxCollisionArray)
        (Collision|SetCollisionEnabled _array_element_4 "QueryAndPhysics")))))

(fn ConstructionScript
  (bind _spline (Variables|Default|GetSpline))
  (bind _meshlength (Variables|Default|GetMeshLength))
  (bind _spline_2 (Variables|Default|GetSpline))
  (bind _returnvalue (Spline|GetSplineLength _spline))
  (bind (_location _tangent) (Spline|GetLocationandTangentatSplinePoint _spline_2 0 "World"))
  (bind _returnvalue_2 (Spline|GetNumberOfSplinePoints _spline_2))
  (bind _returnvalue_3 (/ _returnvalue _meshlength))
  (bind _returnvalue_4 (- _returnvalue_2 1))
  (bind _returnvalue_5 (Math|Float|Truncate _returnvalue_3))
  (bind (_location_2 _tangent_2) (Spline|GetLocationandTangentatSplinePoint _spline_2 _returnvalue_4 "World"))
  (|CallParentFunction)
  ;[0.02246 0.0677 0.1458] Clear Arrays
  (Utilities|Array|Clear (Variables|Default|GetBridgeFloorMeshes))
  (Utilities|Array|Clear (Variables|Default|GetBridgeCapMeshes))
  (Utilities|Array|Clear (Variables|Default|GetBoxCollisionArray))
  (Utilities|Array|Clear (Variables|Default|GetBridgeWallCollisionArray))
  (Variables|Default|SetBoxCollisionArray (Utilities|Array|MakeArray (Variables|Default|GetBox) (Variables|Default|GetBox2) (Variables|Default|GetBox3) (Variables|Default|GetBox4) (Variables|Default|GetBox5) (Variables|Default|GetBox6)))
  (Variables|Default|SetSegmentLength (* (.x (Transformation|GetActorScale3D)) (/ _returnvalue (Math|Conversions|ToFloat(Integer) _returnvalue_5))))
  (bind _output_get (Variables|Default|SetSegments _returnvalue_5))
  (for _index (range 0 (- _output_get 1))
    (Variables|Default|SetIndex _index)
    (Utilities|FlowControl|Sequence
      (:then_0
        ;[0.1979 0.02371 0.1544] Ghost Bridge Floor Meshes
        (bind _returnvalue_6 (AddComponent|AddSplineMeshComponent false))
        (Rendering|Material|SetScalarParameterValueonMaterials _returnvalue_6 "TestingSwitch" (Math|Conversions|ToFloat(Boolean) (Variables|Default|GetMaterialTesting)))
        (Rendering|Material|SetScalarParameterValueonMaterials _returnvalue_6 "UVShift" (Math|Conversions|ToFloat(Integer) (Variables|Default|GetIndex)))
        (SplineMesh|SetStartandEnd _returnvalue_6 (.Start%20Pos (Utilities|SplineLocationandTangent (Variables|Default|GetIndex) (Variables|Default|GetSegmentLength))) (.Start%20Tangent (Utilities|SplineLocationandTangent (Variables|Default|GetIndex) (Variables|Default|GetSegmentLength))) (.End%20Pos (Utilities|SplineLocationandTangent (Variables|Default|GetIndex) (Variables|Default|GetSegmentLength))) (.End%20Tangent (Utilities|SplineLocationandTangent (Variables|Default|GetIndex) (Variables|Default|GetSegmentLength))) true :!class /Script/Engine.SplineMeshComponent)
        (Rendering|SetTranslucentSortPriority _returnvalue_6 1)
        (Collision|SetCollisionEnabled _returnvalue_6 (Variables|Default|GetBridgeFloorCollision))
        (Utilities|Array|Add (Variables|Default|GetBridgeFloorMeshes) _returnvalue_6))
      (:then_1
        ;[0.4271 0.1574 0] Add Wall Collision Meshes
        (bind _returnvalue_7 (AddComponent|AddSplineMeshComponent false))
        (SplineMesh|SetStartandEnd _returnvalue_7 (.Start%20Pos (Utilities|SplineLocationandTangent (Variables|Default|GetIndex) (Variables|Default|GetSegmentLength))) (.Start%20Tangent (Utilities|SplineLocationandTangent (Variables|Default|GetIndex) (Variables|Default|GetSegmentLength))) (.End%20Pos (Utilities|SplineLocationandTangent (Variables|Default|GetIndex) (Variables|Default|GetSegmentLength))) (.End%20Tangent (Utilities|SplineLocationandTangent (Variables|Default|GetIndex) (Variables|Default|GetSegmentLength))) true :!class /Script/Engine.SplineMeshComponent)
        (Rendering|SetVisibility _returnvalue_7 false false)
        (Collision|SetCollisionEnabled _returnvalue_7 (Variables|Default|GetBridgeWallCollision))
        (Utilities|Array|Add (Variables|Default|GetBridgeWallCollisionArray) _returnvalue_7))))
  (Utilities|FlowControl|Sequence
    (:then_0
      (|RockMeshesandBridgeEnds _location _tangent _location_2 _tangent_2))
    (:then_1
      (|PositionCapsule _location _location_2) ; Procedural Placement and Scaling of Interaction Capsule
    )))