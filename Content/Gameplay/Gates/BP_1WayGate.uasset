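; BP_1WayGate is a gate that lets things through from one side only.
; Beginning overlap on PassSide turns off the Cube's collision, and ending overlap on BlockSide turns it back on.
; Two DoOnce nodes re-arm each other so opening and closing alternate, with no filter on the overlapping actor.
; On BeginPlay, both side boxes switch to absolute scale.
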(event OnComponentBeginOverlap(PassSide)
  (params (OverlappedComponent :type Primitive%20Component%20Object%20Reference) (OtherActor :type Actor%20Object%20Reference) (OtherComp :type Primitive%20Component%20Object%20Reference) (OtherBodyIndex :type Integer) (bFromSweep :type Boolean) (SweepResult :type Hit%20Result%20Structure%20%28by%20ref%29))
  (bind _cube (Variables|Default|GetCube))
  ;[1 1 1] Disables collision
  (Utilities|FlowControl|DoOnce false
    (:Completed
      (Collision|SetCollisionEnabled _cube "NoCollision")
      ;[1 1 1] Enables collision
      (Utilities|FlowControl|DoOnce false) ; enters at Reset
    )))

(event OnComponentEndOverlap(Blockside)
  (params (OverlappedComponent :type Primitive%20Component%20Object%20Reference) (OtherActor :type Actor%20Object%20Reference) (OtherComp :type Primitive%20Component%20Object%20Reference) (OtherBodyIndex :type Integer))
  (bind _cube (Variables|Default|GetCube))
  ;[1 1 1] Enables collision
  (Utilities|FlowControl|DoOnce false
    (:Completed
      (Collision|SetCollisionEnabled _cube "QueryAndPhysics")
      ;[1 1 1] Disables collision
      (Utilities|FlowControl|DoOnce false) ; enters at Reset
    )))

(event EventBeginPlay
  (|CallParentFunction)
  (Transformation|SetAbsolute (Variables|Default|GetSidebox1) false false true)
  (Transformation|SetAbsolute (Variables|Default|GetSisdeBox2) false false true))

(event Collision|EventActorBeginOverlap
  (params (OtherActor :type Actor%20Object%20Reference))
  (|CallParentFunction OtherActor) ; This node is disabled and will not be called.\nDrag off pins to build functionality.
)

(event EventTick
  (params (DeltaSeconds :type Float%20%28single-precision%29))
  (|CallParentFunction DeltaSeconds) ; This node is disabled and will not be called.\nDrag off pins to build functionality.
)

(fn ConstructionScript
  (|CallParentFunction))