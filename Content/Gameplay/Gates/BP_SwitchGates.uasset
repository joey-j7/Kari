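; BP_SwitchGates is a gate actor that toggles between a solid, visible state and a passable, hidden one.
; Switch flips the Cube's collision and the actor's in-game visibility based on whether physics collision is currently enabled.
; SetInitial uses BlueType to pick the material and starting state: blue gates start solid, others start hidden; its BlueUp input is unused.
; Neither function is called within this Blueprint.
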(event Collision|EventActorBeginOverlap
  (params (OtherActor :type Actor%20Object%20Reference)))

(event EventTick
  (params (DeltaSeconds :type Float%20%28single-precision%29)))

(fn ConstructionScript)

(fn Switch
  (bind _cube (Variables|Default|GetCube))
  ;[1 1 1] Enables/Disables collison
  (if (Class|PrimitiveComponent|IsPhysicsCollisionEnabled (Variables|Default|GetCube))
    (Collision|SetCollisionEnabled _cube "NoCollision")
    (Rendering|SetActorHiddenInGame true)
    (else
      (Collision|SetCollisionEnabled _cube "QueryAndPhysics")
      (Rendering|SetActorHiddenInGame false))))

(fn SetInitial
  (params (BlueUp :type Boolean))
  (bind _bluetype (Variables|Default|GetBlueType))
  (bind _cube (Variables|Default|GetCube))
  (bind _cube_2 (Variables|Default|GetCube))
  ;[1 1 1] Assigning default type
  (if _bluetype
    (Rendering|Material|SetMaterial _cube_2 0 "/Game/Environment/Vegetation/Grass/0/MAT_Water.MAT_Water")
    (if _bluetype
      (Collision|SetCollisionEnabled _cube "QueryAndPhysics")
      (Rendering|SetActorHiddenInGame false))
    (else
      (Rendering|Material|SetMaterial _cube_2 0 "/Game/Environment/Props/Pickups/Hemp/M_HempStem.M_HempStem")
      (if (not _bluetype)
        (Collision|SetCollisionEnabled _cube "NoCollision")
        (Rendering|SetActorHiddenInGame true)))))