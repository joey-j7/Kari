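; Base gate Blueprint for locked gates that the player interacts with to open, with UnlockEffect left empty, presumably for child gates.
; Interacting while locked optionally removes ItemSets resources, then fades the screen out, plays unlock audio, runs UnlockEffect, fades back in and re-enables input.
; KeyCheck is disconnected and HasKey is forced true, so the resource requirement is never enforced.
; OnLoadUnlock reapplies the effect without the sequence.
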(event OnInteract(Interactable)
  ;[1 1 1] Check if door can be unlocked
  (if (Variables|Default|GetDoorLocked)
    (Variables|Default|SetHasKey true)
    (if (Variables|Default|GetHasKey)
      (CallFunction|RemoveResources)
      (bind _returnvalue (Actor|GetActorOfClass "/Game/General/BP_FadeController.BP_FadeController_C"))
      (bind _output_get (Variables|Default|SetFadeController _returnvalue))
      (Class|FadeController|ScreenFadeOut _output_get 0.0)
      (EventDispatchers|BindEventtoOnScreenFaded _output_get (delegate Custom|Unlock))
      (else
        (Default|OnInsufficient (Variables|Default|GetHUDInteractRef))))))

(event Custom|KeyCheck
  ;[1 1 1] Check for key resources
  (bind _asdefault_game_instance (Utilities|Casting|CastToDefaultGameInstance (Game|GetGameInstance)))
  (for _array_element (Variables|Default|GetItemSets)
    (bind _returnvalue (Class|Inventory|CountItem (Variables|/Script/Kari.DefaultGameInstance|GetInventory _asdefault_game_instance) (.itemid _array_element)))
    (if (< _returnvalue (.amount _array_element))
      (Variables|Default|SetHasKey false))))

(event Custom|Remove%20Resources
  ;[1 1 1] Remove key resources from inventory
  (if (Variables|Default|GetRemovesResources)
    (bind _asdefault_game_instance (Utilities|Casting|CastToDefaultGameInstance (Game|GetGameInstance)))
    (for _array_element (Variables|Default|GetItemSets)
      (Class|Inventory|RemoveItemsbyType (Variables|/Script/Kari.DefaultGameInstance|GetInventory _asdefault_game_instance) (.itemid _array_element) (.amount _array_element))
      (Variables|Default|SetHasKey false))))

(event Custom|Unlock
  (bind _gameinstance (Variables|Default|GetGameInstance))
  (bind _fadecontroller (Variables|Default|GetFadeController))
  (bind _audiomanager (Variables|/Script/Kari.DefaultGameInstance|GetAudioManager _gameinstance))
  (bind _returnvalue (Class|AudioManager|GetBGM _audiomanager))
  ;[1 1 1] Selects correct audio file to play
  (Class|AudioManager|Play (Variables|/Script/Kari.DefaultGameInstance|GetAudioManager (Variables|Default|GetGameInstance)) (Utilities|Array|MakeArray (Utilities|String|Append (Variables|Default|GetAudioPath) (Variables|Default|GetAudio))) false 0 0 1.0 1.0 0.0 0.3 false)
  ;[1 1 1] Unlock
  (CallFunction|UnlockEffect)
  (Utilities|FlowControl|Delay (Variables|Default|GetFadeDuration))
  ;[1 1 1] Fade Camera Back In
  (Class|FadeController|ScreenFadein _fadecontroller 0.0)
  (EventDispatchers|AssignOnScreenClear _fadecontroller (delegate Custom|EnablePlayerInput))
  ;[1 1 1] Fade out music
  (Utilities|IsValid _returnvalue
    (:Is%20Valid
      (Class|Playlist|FadeVolume _returnvalue 1.0 1.0 true))))

(event Custom|EnablePlayerInput
  (Input|EnableInput (Game|GetPlayerController 0) 0)
  (Input|EnableInput (Game|GetPlayerCharacter 0) 0))

(event EventBeginPlay
  (bind _asgi_default_game_instance (Utilities|Casting|CastToGI_DefaultGameInstance (Game|GetGameInstance)))
  (Variables|Default|SetGameInstance _asgi_default_game_instance)
  (Transformation|AddLocalOffset (Variables|Default|GetNiagara) (Variables|Default|GetGlitter%20Location) false false))

(event EventOnLoadUnlock
  ;[1 1 1] Unlock gate on load when unlocked while saving
  (CallFunction|UnlockEffect))

(fn ConstructionScript)

(fn UnlockEffect)

(fn IsLocked
  (return (Variables|Default|GetDoorLocked)))