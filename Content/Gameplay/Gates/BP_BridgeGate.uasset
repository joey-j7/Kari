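; Bridge gate that, when unlocked, applies designer-set world changes and completes the bridge quest task.
; BeginPlay derives the gate's audio from an enum, relabelling the interaction as lighting a brazier for "Flare".
; UnlockEffect uses instance command arrays to show, hide or destroy assets, actors and blocking volumes, then clears its own blocker and calls an empty child hook.
; It also increments the LUMBERJACK stat when no item sets are configured.
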(event Custom|UnlockEffectChild)

(event EventBeginPlay
  (bind _interactable (Variables|Default|GetInteractable))
  (|CallParentFunction)
  (bind _output_get (Variables|Default|SetParent%20Gate self))
  (bind _output_get_2 (Variables|/Game/Gameplay/Gates/BP_ParentGate.BP_ParentGate_C|SetAudio _output_get (Utilities|String|EnumtoString (Variables|Default|GetSounds))))
  (if (Utilities|Enum|Equal(Enum) _output_get_2 "Flare")
    (Variables|/Script/Kari.InteractableComponent|SetCharacterName _interactable "Brazier ")
    (Variables|/Script/Kari.InteractableComponent|SetAction _interactable "Light ")))

(event Collision|EventActorBeginOverlap
  (params (OtherActor :type Actor%20Object%20Reference))
  (|CallParentFunction OtherActor) ; This node is disabled and will not be called.\nDrag off pins to build functionality.
)

(event EventTick
  (params (DeltaSeconds :type Float%20%28single-precision%29))
  (|CallParentFunction DeltaSeconds) ; This node is disabled and will not be called.\nDrag off pins to build functionality.
)

(event EventUnlockEffect
  (bind _blocking_volumes_td (Variables|Default|GetBlocking%20volumes%20TD))
  ;[1 1 1] Unlock effect
  (Utilities|FlowControl|Sequence
    (:then_0
      (if (> (Utilities|Array|Length (Variables|Default|GetAssetCommands)) 0)
        (CallFunction|ActorVisibility)
        (CallFunction|SetBlockingVolume)
        (for _array_element (Variables|Default|GetAssetCommands)
          (if (.spawnasset _array_element)
            (Rendering|SetVisibility (Variables|/Script/Engine.Actor|GetRootComponent (.assetref _array_element)) true false)
            (Collision|SetCollisionEnabled (Variables|/Script/Engine.StaticMeshActor|GetStaticMeshComponent (.assetref _array_element)) "QueryAndPhysics")
            (else
              (Rendering|SetVisibility (Variables|/Script/Engine.Actor|GetRootComponent (.assetref _array_element)) false false)
              (Collision|SetCollisionEnabled (Variables|/Script/Engine.StaticMeshActor|GetStaticMeshComponent (.assetref _array_element)) "NoCollision"))))
        (Collision|SetCollisionEnabled (Variables|Default|GetBox) "NoCollision")
        (Components|DestroyComponent (Variables|Default|GetCube))
        (CallFunction|UnlockEffectChild)
        (if (> (Utilities|Array|Length _blocking_volumes_td) 0)
          (for _array_element_2 _blocking_volumes_td
            (Actor|DestroyActor _array_element_2)
            (Variables|Default|SetDoorLocked false)
            ;[1 1 1] Complete bridge task
            (bind _asgi_default_game_instance (Utilities|Casting|CastToGI_DefaultGameInstance (Game|GetGameInstance)))
            (Class|QuestLog|CompleteTask (Variables|/Script/Kari.DefaultGameInstance|GetQuestLog _asgi_default_game_instance) 7))
          (else
            (Variables|Default|SetDoorLocked false)
            (bind _asgi_default_game_instance_2 (Utilities|Casting|CastToGI_DefaultGameInstance (Game|GetGameInstance)))
            (Class|QuestLog|CompleteTask (Variables|/Script/Kari.DefaultGameInstance|GetQuestLog _asgi_default_game_instance_2) 7)))
        (else
          (Development|PrintString "Public reference not set"))))
    (:then_1
      (if (== (Utilities|Array|Length (Variables|Default|GetItemSets)) 0)
        (CallFunction|UpdateStat "LUMBERJACK" 1 true false)))))

(fn ConstructionScript
  (|CallParentFunction))

(fn ActorVisibility
  (for _array_element (Variables|Default|GetActorCommands)
    (if (.spawnasset _array_element)
      (Rendering|SetActorHiddenInGame (.actor _array_element) false)
      (else
        (Actor|DestroyActor (.actor _array_element)))))
  (return))

(fn SetBlockingVolume
  (for _array_element (Variables|Default|GetBlockingVolumeCommands)
    (if (.spawnblockingvolume _array_element)
      (Collision|SetCollisionEnabled (Variables|/Script/Engine.Brush|GetBrushComponent (.blockingvolume _array_element)) "QueryAndPhysics")
      (else
        (Actor|DestroyActor (.blockingvolume _array_element))))))