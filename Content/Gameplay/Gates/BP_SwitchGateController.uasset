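; Controller for switchable gates that flips a group of BP_SwitchGates actors whenever its unlock effect fires.
; BeginPlay finds every switch gate in the level and sets its initial state from BlueUp, regardless of group.
; UnlockEffect calls Switch on gates whose GroupIndex matches GateGroup, then toggles LoadShouldSwitch.
; IsLocked returns that toggled flag as the lock state.
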(event EventBeginPlay
  ;[1 1 1] Set initial states
  (|CallParentFunction)
  (bind _outactors (Actor|GetAllActorsOfClass "/Game/Gameplay/Gates/BP_SwitchGates.BP_SwitchGates_C"))
  (for _array_element _outactors
    (Default|SetInitial _array_element (Variables|Default|GetBlueUp))))

(event Collision|EventActorBeginOverlap
  (params (OtherActor :type Actor%20Object%20Reference))
  (|CallParentFunction OtherActor) ; This node is disabled and will not be called.\nDrag off pins to build functionality.
)

(event EventTick
  (params (DeltaSeconds :type Float%20%28single-precision%29))
  (|CallParentFunction DeltaSeconds) ; This node is disabled and will not be called.\nDrag off pins to build functionality.
)

(event EventUnlockEffect
  ;[1 1 1] Determines what which up/down needs to fire
  (bind _outactors (Actor|GetAllActorsOfClass "/Game/Gameplay/Gates/BP_SwitchGates.BP_SwitchGates_C"))
  (for _array_element _outactors
    (if (== (Variables|/Game/Gameplay/Gates/BP_SwitchGates.BP_SwitchGates_C|GetGroupIndex _array_element) (Variables|Default|GetGateGroup))
      (Default|Switch _array_element)))
  (Variables|Default|SetLoadShouldSwitch (not (Variables|Default|GetLoadShouldSwitch))))

(fn ConstructionScript
  (|CallParentFunction))

(fn IsLocked
  (return (Variables|Default|GetLoadShouldSwitch)))