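; BP_BoulderGate is a gate that slides its Cube open when unlocked.
; BeginPlay caches the relative locations of the Cube and its EndPoint component as the start and end of the movement.
; UnlockEffect plays the DoorMovement timeline, which lerps the Cube between those locations and clears DoorLocked on each update.
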(event EventBeginPlay
  ;[1 1 1] Set locations
  (|CallParentFunction)
  (Variables|Default|SetStartLocation (Variables|/Script/Engine.SceneComponent|GetRelativeLocation (Variables|Default|GetCube)))
  (Variables|Default|SetEndLocation (Variables|/Script/Engine.SceneComponent|GetRelativeLocation (Variables|Default|GetEnd%20Point))))

(event Collision|EventActorBeginOverlap
  (params (OtherActor :type Actor%20Object%20Reference))
  (|CallParentFunction OtherActor) ; This node is disabled and will not be called.\nDrag off pins to build functionality.
)

(event EventTick
  (params (DeltaSeconds :type Float%20%28single-precision%29))
  (|CallParentFunction DeltaSeconds) ; This node is disabled and will not be called.\nDrag off pins to build functionality.
)

(event EventUnlockEffect
  ;[1 1 1] Unlock effect
  (bind _newtrack_0 (Timeline|Door%20movement Play)
    (:Update
      (Transformation|SetRelativeLocation (Variables|Default|GetCube) (Math|Vector|Lerp(Vector) (Variables|Default|GetStartLocation) (Variables|Default|GetEndLocation) _newtrack_0) false false)
      (Variables|Default|SetDoorLocked false))))

(fn ConstructionScript
  (|CallParentFunction))