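; BP_TimeGate is a gate that opens its wall only when the player or another overlapper arrives at the right time of day.
; Overlapping Box1 reads the game instance's TimeManager time as an integer and compares it to UnlockTime.
; If UnlockTime falls from the current time up to six units ahead, Wall collision is disabled and never re-enabled here.
; Debug prints show the time and result.
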(event OnComponentBeginOverlap(Box1)
  (params (OverlappedComponent :type Primitive%20Component%20Object%20Reference) (OtherActor :type Actor%20Object%20Reference) (OtherComp :type Primitive%20Component%20Object%20Reference) (OtherBodyIndex :type Integer) (bFromSweep :type Boolean) (SweepResult :type Hit%20Result%20Structure%20%28by%20ref%29))
  ;[1 1 1] Checks if gate needs to unlock
  (CallFunction|CheckTOD)
  (if (and (>= (Variables|Default|GetUnlock%20Time) (Variables|Default|GetTimeOfDay)) (< (Variables|Default|GetUnlock%20Time) (+ (Variables|Default|GetTimeOfDay) 6)))
    (Collision|SetCollisionEnabled (Variables|Default|GetWall) "NoCollision")
    (Development|PrintString "unlocked")
    (else
      (Development|PrintString "wrong time"))))

(event Custom|Check%20TOD
  ;[1 1 1] Checks time of day
  (bind _asdefault_game_instance (Utilities|Casting|CastToDefaultGameInstance (Game|GetGameInstance)))
  (bind _output_get (Variables|Default|SetTimeOfDay (Math|Conversions|ToInteger(Byte) (Class|TimeManager|GetTimeString (Variables|/Script/Kari.DefaultGameInstance|GetTimeManager _asdefault_game_instance) false))))
  (Development|PrintString (Utilities|String|ToString(Integer) _output_get) true true "(R=0.000000,G=0.660000,B=1.000000,A=1.000000)" 5.0))

(event EventBeginPlay
  (|CallParentFunction))

(event Collision|EventActorBeginOverlap
  (params (OtherActor :type Actor%20Object%20Reference))
  (|CallParentFunction OtherActor) ; This node is disabled and will not be called.\nDrag off pins to build functionality.
)

(event EventTick
  (params (DeltaSeconds :type Float%20%28single-precision%29))
  (|CallParentFunction DeltaSeconds))

(fn ConstructionScript
  (|CallParentFunction))