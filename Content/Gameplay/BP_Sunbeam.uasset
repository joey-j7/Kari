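; Sunbeam hazard and puzzle actor that fades in for morning and afternoon and out for evening and night, following TimeManager period changes.
; A timeline drives the fade through a material parameter collection; while visible, Tick line-traces along the arrow to place the Niagara beam.
; Hitting BP_Kari damages their Blessing unless reflection is active, when a second trace along the player's facing draws a reflected beam that clears any BP_SunGate hit.
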(event Custom|CheckDayTime
  (params (Period :type EPeriod%20Enum :default "E_NIGHT"))
  ;[1 1 1] Checks if it is night time
  (switch Utilities|FlowControl|Switch|SwitchonEPeriod Period
    (:E_NIGHT
      (Utilities|FlowControl|Sequence :!label _label
        (:then_0
          (goto _label_4 Reset))
        (:then_1
          (Utilities|FlowControl|DoOnce false :!label _label_2
            (:Completed
              (bind _timefadertrack (Timeline|GodrayTimeline ReverseFromEnd)
                (:Update
                  (bind _output_get (Variables|Default|SetTimeFader _timefadertrack))
                  (Rendering|Material|SetScalarParameterValue "/Game/Gameplay/Colliders/Events/MPC_MaterialVariables.MPC_MaterialVariables" "SunbeamVisibility" _output_get :!class /Script/Engine.KismetMaterialLibrary)
                  (bind _circlerotation (Timeline|CircleRotation Play)
                    (:Update
                      (Transformation|SetWorldRotation (Variables|Default|GetSM_VFX_Ring) (Math|Rotator|MakeRotator 0.0 0.0 _circlerotation) false false))))
                (:Finished
                  (if (== (Variables|Default|GetTimeFader) 0.0)
                    (Rendering|SetVisibility (Variables|Default|GetOriginal) false true)))))))))
    (:E_MORNING
      (Utilities|FlowControl|Sequence :!label _label_3
        (:then_0
          (goto _label_2 Reset))
        (:then_1
          (Utilities|FlowControl|DoOnce false :!label _label_4
            (:Completed
              (Rendering|SetVisibility (Variables|Default|GetOriginal) true true)
              (Timeline|GodrayTimeline PlayFromStart))))))
    (:E_AFTERNOON
      (goto _label_3))
    (:E_EVENING
      (goto _label))))

(event EventTick
  (params (DeltaSeconds :type Float%20%28single-precision%29))
  (bind _defaultsceneroot (Variables|Default|GetDefaultSceneRoot))
  (bind _arrow (Variables|Default|GetArrow))
  (bind _returnvalue (Transformation|GetWorldLocation _defaultsceneroot))
  (bind _returnvalue_2 (Math|Vector|GetForwardVector _arrow))
  (if (> (Variables|Default|GetTimeFader) 0.0)
    (Class|NiagaraComponent|SetNiagaraVariableVec3 (Variables|Default|GetOriginal) "User.BeamStart" _returnvalue)
    (Rendering|SetVisibility (Variables|Default|GetReflected) false true)
    (bind (_outhit _returnvalue_3) (Collision|LineTraceByChannel _returnvalue (+ _returnvalue (* _returnvalue_2 (Variables|Default|GetDistance))) "TraceTypeQuery1" false 0 "None" true "(R=1.000000,G=0.000000,B=0.000000,A=1.000000)" "(R=0.000000,G=0.000000,B=0.000000,A=0.000000)" 0.0))
    (bind _asbp_kari (Utilities|Casting|CastToBP_Kari (.hitactor _outhit))
      (:then
        (bind _returnvalue_4 (Class|PersistenceLibrary|GetSunBeamReflection))
        (if _returnvalue_4
          (Class|NiagaraComponent|SetNiagaraVariableVec3 (Variables|Default|GetOriginal) "User.BeamEnd" (select _returnvalue_3 (+ (* _returnvalue_2 (- (.distance _outhit) 35.0)) _returnvalue) (.traceend _outhit)))
          (Transformation|SetWorldLocation (Variables|Default|GetHitOriginal) (select _returnvalue_3 (+ (* _returnvalue_2 (- (.distance _outhit) 35.0)) _returnvalue) (.traceend _outhit)) false false)
          (Transformation|SetWorldLocation (Variables|Default|GetSM_VFX_Cylinder) (Math|Vector|MakeVector (.X (Math|Vector|BreakVector (Transformation|GetWorldLocation (Variables|/Script/Engine.Character|GetMesh _asbp_kari)))) (.Y (Math|Vector|BreakVector (Transformation|GetWorldLocation (Variables|/Script/Engine.Character|GetMesh _asbp_kari)))) (.Z (Math|Vector|BreakVector (select _returnvalue_3 (+ (* _returnvalue_2 (- (.distance _outhit) 35.0)) _returnvalue) (.traceend _outhit))))) false false)
          (Rendering|SetVisibility (Variables|Default|GetReflected) true true)
          (bind (_forwardvector _outhit_2 _hit) (CallFunction|ReflectViewDir (Math|Vector|MakeVector (.X (Math|Vector|BreakVector (Transformation|GetWorldLocation (Variables|/Script/Engine.Character|GetMesh _asbp_kari)))) (.Y (Math|Vector|BreakVector (Transformation|GetWorldLocation (Variables|/Script/Engine.Character|GetMesh _asbp_kari)))) (.Z (Math|Vector|BreakVector (select _returnvalue_3 (+ (* _returnvalue_2 (- (.distance _outhit) 35.0)) _returnvalue) (.traceend _outhit)))))))
          (Class|NiagaraComponent|SetNiagaraVariableVec3 (Variables|Default|GetReflected) "User.BeamStart" (+ (Math|Vector|MakeVector (.X (Math|Vector|BreakVector (Transformation|GetWorldLocation (Variables|/Script/Engine.Character|GetMesh _asbp_kari)))) (.Y (Math|Vector|BreakVector (Transformation|GetWorldLocation (Variables|/Script/Engine.Character|GetMesh _asbp_kari)))) (.Z (Math|Vector|BreakVector (select _returnvalue_3 (+ (* _returnvalue_2 (- (.distance _outhit) 35.0)) _returnvalue) (.traceend _outhit))))) (* _forwardvector 45.0)))
          (Transformation|SetWorldLocation (Variables|Default|GetGlareReflected) (+ (Math|Vector|MakeVector (.X (Math|Vector|BreakVector (Transformation|GetWorldLocation (Variables|/Script/Engine.Character|GetMesh _asbp_kari)))) (.Y (Math|Vector|BreakVector (Transformation|GetWorldLocation (Variables|/Script/Engine.Character|GetMesh _asbp_kari)))) (.Z (Math|Vector|BreakVector (select _returnvalue_3 (+ (* _returnvalue_2 (- (.distance _outhit) 35.0)) _returnvalue) (.traceend _outhit))))) (* _forwardvector 45.0)) false false) ; Might only need to set this, but using the shortened vector
          (Transformation|SetWorldRotation (Variables|Default|GetGlareReflected) (Math|Conversions|RotationFromXVector _forwardvector) false false)
          (Class|NiagaraComponent|SetNiagaraVariableVec3 (Variables|Default|GetReflected) "User.BeamEnd" (select _hit (.location _outhit_2) (.traceend _outhit_2)))
          (Transformation|SetWorldLocation (Variables|Default|GetHitReflected) (select _hit (.location _outhit_2) (.traceend _outhit_2)) false false)
          (bind _asbp_sun_gate (Utilities|Casting|CastToBP_SunGate (.hitactor _outhit_2)))
          (Default|ClearPath _asbp_sun_gate)
          (else
            (Class|DefaultStatComponent|Damage (Variables|/Script/Kari.DefaultPlayer|GetBlessing _asbp_kari) (Variables|Default|GetDamage))
            (Class|NiagaraComponent|SetNiagaraVariableVec3 (Variables|Default|GetOriginal) "User.BeamEnd" (select _returnvalue_3 (.location _outhit) (.traceend _outhit)) :!label _label)
            (Transformation|SetWorldLocation (Variables|Default|GetHitOriginal) (select _returnvalue_3 (.location _outhit) (.traceend _outhit)) false false))))
      (:CastFailed
        (goto _label)))))

(event EventBeginPlay
  ;[1 1 1] Checks if it is night time
  (bind _asgi_default_game_instance (Utilities|Casting|CastToGI_DefaultGameInstance (Game|GetGameInstance)))
  (EventDispatchers|BindEventtoOnPeriodChanged (Variables|/Script/Kari.DefaultGameInstance|GetTimeManager _asgi_default_game_instance) (delegate Custom|CheckDayTime))
  (CallFunction|CheckDayTime (Class|TimeManager|GetPeriod (Variables|/Script/Kari.DefaultGameInstance|GetTimeManager _asgi_default_game_instance))))

(fn ConstructionScript
  (bind _defaultsceneroot (Variables|Default|GetDefaultSceneRoot))
  (bind _returnvalue (Transformation|GetWorldLocation _defaultsceneroot))
  (Class|NiagaraComponent|SetNiagaraVariableVec3 (Variables|Default|GetOriginal) "User.BeamStart" _returnvalue)
  (Class|NiagaraComponent|SetNiagaraVariableVec3 (Variables|Default|GetOriginal) "User.BeamEnd" (+ _returnvalue (* (Math|Vector|GetForwardVector (Variables|Default|GetArrow)) (Variables|Default|GetDistance)))))

(fn ReflectViewDir
  (params (HitLocation :type Vector))
  (bind _returnvalue (Game|GetPlayerCharacter 0))
  (bind _mesh (Variables|/Script/Engine.Character|GetMesh _returnvalue))
  (bind _returnvalue_2 (Math|Vector|GetForwardVector _mesh))
  (bind (_outhit _returnvalue_3) (Collision|LineTraceByChannel HitLocation (+ HitLocation (* _returnvalue_2 (Variables|Default|GetDistance))) "TraceTypeQuery1" false (Utilities|Array|MakeArray _returnvalue) "None" true "(R=0.223958,G=0.217826,B=0.205738,A=1.000000)" "(R=1.000000,G=0.981161,B=0.000000,A=1.000000)" 1.0))
  (return _returnvalue_2 _outhit _returnvalue_3))

(fn ReflectAroundNormal
  (params (HitLocation :type Vector))
  (Collision|LineTraceByChannel HitLocation (+ HitLocation (* (Math|Vector|MirrorVectorbyNormal (Math|Vector|GetForwardVector (Variables|Default|GetArrow)) (Math|Vector|GetForwardVector (Variables|/Script/Engine.Character|GetMesh (Game|GetPlayerCharacter 0)))) (Variables|Default|GetDistance))) "TraceTypeQuery1" false (Utilities|Array|MakeArray (Game|GetPlayerCharacter 0)) "None" true "(R=1.000000,G=0.846200,B=0.918744,A=1.000000)" "(R=0.390625,G=0.004005,B=0.388413,A=1.000000)"))