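; BP_TimePassageBlocker is a trigger volume that blocks passage during configured periods of the day.
; It binds to the game instance's TimeManager period-change event and applies the current period on BeginPlay.
; The bound box gets query and physics collision when the period is in BlockDuring, otherwise none.
; When BP_Kari hits it, it broadcasts interact on the referenced Interactable's InteractableComponent.
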(event Custom|Event%20PeriodChanged
  (params (Period :type EPeriod%20Enum :default "E_NIGHT"))
  ;[0 1 0.9955] listen to the period of the day
  (CallFunction|ChangeCollisionBasedonPeriod Period))

(event EventBeginPlay
  ;[0 1 0.9955] listen to the period of the day
  (bind _asdefault_game_instance (Utilities|Casting|CastToDefaultGameInstance (Game|GetGameInstance)))
  (EventDispatchers|BindEventtoOnPeriodChanged (Variables|/Script/Kari.DefaultGameInstance|GetTimeManager _asdefault_game_instance) (delegate Custom|Event%20PeriodChanged))
  (CallFunction|ChangeCollisionBasedonPeriod (Class|TimeManager|GetPeriod (Variables|/Script/Kari.DefaultGameInstance|GetTimeManager _asdefault_game_instance))))

(event Collision|EventHit
  (params (MyComp :type Primitive%20Component%20Object%20Reference) (Other :type Actor%20Object%20Reference) (OtherComp :type Primitive%20Component%20Object%20Reference) (bSelfMoved :type Boolean) (HitLocation :type Vector :default "0, 0, 0") (HitNormal :type Vector :default "0, 0, 0") (NormalImpulse :type Vector :default "0, 0, 0") (Hit :type Hit%20Result%20Structure%20%28by%20ref%29))
  (bind _interactable (Variables|Default|GetInteractable))
  (bind _returnvalue (Actor|GetComponentbyClass _interactable "/Script/Kari.InteractableComponent"))
  ;[0 0.9448 1] On Hit trigger the interact on the actor
  (Utilities|Casting|CastToBP_Kari Other)
  (Utilities|IsValid _returnvalue
    (:Is%20Valid
      (Class|InteractableComponent|BroadCastonInteract _returnvalue))))

(fn ConstructionScript)

(fn ChangeCollisionBasedonPeriod
  (params (Period :type EPeriod%20Enum :default "E_NIGHT"))
  (bind _boundbox (Variables|Default|GetBoundBox))
  (if (Utilities|Array|ContainsItem (Variables|Default|GetBlockDuring) Period)
    (Collision|SetCollisionEnabled _boundbox "QueryAndPhysics")
    (else
      (Collision|SetCollisionEnabled _boundbox "NoCollision"))))