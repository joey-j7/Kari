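; Camera rail trigger that switches the view to itself while the Kari player character is near its spline.
; Every tick it compares the player's horizontal distance to the rail against AffectRange, blending the view in and moving CameraTransform to the closest spline point.
; Leaving the range blends back to the player once through a DoOnce that re-arms while in range.
; Only camera position follows the rail; the rotation update is disconnected.
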(event EventBeginPlay
  (bind _asbp_kari (Utilities|Casting|CastToBP_Kari (Game|GetPlayerCharacter 0)))
  (Variables|Default|SetPlayer _asbp_kari))

(event EventTick
  (params (DeltaSeconds :type Float%20%28single-precision%29))
  (bind _railsplinecomponent (Variables|Default|GetRailSplineComponent))
  (bind _player (Variables|Default|GetPlayer))
  (bind _returnvalue (Transformation|GetActorLocation _player))
  (bind _returnvalue_2 (Spline|FindLocationClosesttoWorldLocation _railsplinecomponent _returnvalue "World"))
  (bind (_x _y) (Math|Vector|BreakVector _returnvalue))
  (if (<= (Math|Vector|Distance(Vector) (Math|Vector|MakeVector (.x _returnvalue_2) (.y _returnvalue_2) 0.0) (Math|Vector|MakeVector _x _y 0.0)) (Variables|Default|GetAffectRange))
    (Game|Player|SetViewTargetwithBlend (Game|GetPlayerController 0) self (Variables|Default|GetBlendTime) "VTBlend_Cubic" 0.0 false)
    (Variables|Default|SetApply true)
    (Transformation|SetWorldLocation (Variables|Default|GetCameraTransform) (.location (Class|SplineComponent|FindTransformClosesttoWorldLocation (Variables|Default|GetRailSplineComponent) (Transformation|GetActorLocation (Variables|Default|GetPlayer)) "World" false)) false true)
    (goto _label Reset)
    (else
      (Utilities|FlowControl|DoOnce true :!label _label
        (:Completed
          (Game|Player|SetViewTargetwithBlend (Game|GetPlayerController 0) (Variables|Default|GetPlayer) (Variables|Default|GetBlendTime) "VTBlend_Cubic" 0.0 false)
          (Variables|Default|SetApply false))))))

(fn ConstructionScript)

(fn CheckEntrance)