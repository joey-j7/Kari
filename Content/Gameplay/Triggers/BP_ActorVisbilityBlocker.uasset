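; Trigger box tied to an Interactable actor that fires that actor's interact event when BP_Kari hits it.
; On BeginPlay and on each visibility change, the box becomes query-only, or loses collision if the Interactable is hidden or its StoryComponent TableID is in RevisionIds.
; A hit refreshes that state and rechecks both conditions before broadcasting through the InteractableComponent.
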(event OnComponentHit(BoundBox)
  (params (HitComponent :type Primitive%20Component%20Object%20Reference) (OtherActor :type Actor%20Object%20Reference) (OtherComp :type Primitive%20Component%20Object%20Reference) (NormalImpulse :type Vector :default "0, 0, 0") (Hit :type Hit%20Result%20Structure%20%28by%20ref%29))
  (bind _interactable (Variables|Default|GetInteractable))
  (bind _returnvalue (Actor|GetComponentbyClass _interactable "/Script/Kari.InteractableComponent"))
  ;[0 0.9448 1] On Hit trigger the interact on the actor
  (Utilities|Casting|CastToBP_Kari OtherActor)
  (CallFunction|OnVisibilityChange)
  (if (not (Variables|/Script/Engine.Actor|GetbHidden _interactable))
    (bind _containsid (CallFunction|HasRevisionID))
    (if (not _containsid)
      (Utilities|IsValid _returnvalue
        (:Is%20Valid
          (Class|InteractableComponent|BroadCastonInteract _returnvalue))))))

(event Custom|OnVisibilityChange
  (bind _boundbox (Variables|Default|GetBoundBox))
  ;[0 1 0.9955] listen to the period of the day
  (bind _containsid (CallFunction|HasRevisionID))
  (if (or _containsid (Variables|/Script/Engine.Actor|GetbHidden (Variables|Default|GetInteractable)))
    (Collision|SetCollisionEnabled _boundbox "NoCollision")
    (else
      (Collision|SetCollisionEnabled _boundbox "QueryOnly"))))

(event EventBeginPlay
  ;[0 1 0.9955] listen to the period of the day
  (EventDispatchers|BindEventtoOnVisibilityChange (Variables|Default|GetInteractable) (delegate Custom|OnVisibilityChange))
  (CallFunction|OnVisibilityChange))

(fn ConstructionScript)

(fn HasRevisionID
  (return (Utilities|Array|ContainsItem (Variables|Default|GetRevisionIds) (Class|TableComponent|TableID (Actor|GetComponentbyClass (Variables|Default|GetInteractable) "/Script/Kari.StoryComponent")))))