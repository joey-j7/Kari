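; BP_Mushroom is a poisonous mushroom hazard that temporarily applies an energy debuff when BP_Kari's capsule enters its sphere.
; On trigger, it first asks every BP_ItemBase whether to absorb the hit, as a resistance rune check.
; Otherwise it applies the Blessing effect, plays audio, swaps burst and ambient particles, and animates via custom primitive data and a timeline-driven material parameter collection.
; Delays re-arm the trigger and later remove the debuff.
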(event OnComponentEndOverlap(SphereCollision)
  (params (OverlappedComponent :type Primitive%20Component%20Object%20Reference) (OtherActor :type Actor%20Object%20Reference) (OtherComp :type Primitive%20Component%20Object%20Reference) (OtherBodyIndex :type Integer))
  (Utilities|FlowControl|Delay 0.2)
  (Rendering|Material|SetCustomPrimitiveDataFloat (Variables|Default|GetSM_PoisonousMushroom_08) 0 0.0))

(event OnComponentBeginOverlap(SphereCollision)
  (params (OverlappedComponent :type Primitive%20Component%20Object%20Reference) (OtherActor :type Actor%20Object%20Reference) (OtherComp :type Primitive%20Component%20Object%20Reference) (OtherBodyIndex :type Integer) (bFromSweep :type Boolean) (SweepResult :type Hit%20Result%20Structure%20%28by%20ref%29))
  (bind _asbp_kari (Utilities|Casting|CastToBP_Kari OtherActor))
  (if (== (Variables|/Script/Engine.Character|GetCapsuleComponent _asbp_kari) OtherComp)
    (if (not (Variables|Default|GetWasActivated))
      (Variables|Default|SetWasActivated true)
      ;[1 1 1] Check for mushroom hazard resistance rune
      (Variables|Default|SetWasConsumed false)
      (bind _outactors (Actor|GetAllActorsOfClass "/Game/Environment/Props/Pickups/BP_ItemBase.BP_ItemBase_C"))
      (bind _array_element (Utilities|Array|ForEachLoopwithBreak _outactors :!label _label)
        (:LoopBody
          (bind _iseventconsumed (Default|OnMushroomOverlap _array_element))
          (if _iseventconsumed
            (Variables|Default|SetWasConsumed true)
            (goto _label Break)))
        (:Completed
          (if (Variables|Default|GetWasConsumed)
            (Utilities|FlowControl|Delay 3.0)
            (Variables|Default|SetWasActivated false)
            (else
              (bind _returnvalue (Actor|GetActorOfClass "/Game/Characters/Playable/Kari/BP_Kari.BP_Kari_C"))
              (bind _returnvalue_2 (Class|DefaultStatComponent|ApplyEffectUnique (Variables|/Script/Kari.DefaultPlayer|GetBlessing _returnvalue) self (Variables|Default|GetMushroomEnergyDebuff)))
              (Class|AudioManager|Play (Variables|/Script/Kari.DefaultGameInstance|GetAudioManager (Variables|Default|GetGameInstance)) (Utilities|Array|MakeArray "Events/Mushroom/Leak") false 0 0 0.9 1.1 0.0 0.3 false)
              ;[0 1 0.5355] Material animation
              (Rendering|Material|SetCustomPrimitiveDataFloat (Variables|Default|GetSM_PoisonousMushroom_08) 0 1.0)
              (bind _explosionanimation (Timeline|Timeline_0 PlayFromStart)
                (:Update
                  (Rendering|Material|SetVectorParameterValue "/Game/Gameplay/Colliders/Events/MPC_MaterialVariables.MPC_MaterialVariables" "MushroomExplosion" (Math|Conversions|ToLinearColor(Vector) _explosionanimation) :!class /Script/Engine.KismetMaterialLibrary)
                  ;[1 0.121 0.2007] Activate ShroomBurst particle effect
                  (Utilities|FlowControl|Delay 0.2) ; Activate particles with delay for better timing
                  (Components|Activation|Activate (Variables|Default|GetShroomBurst) false)
                  (CallFunction|StopMushroomBurst)
                  (Components|Activation|Deactivate (Variables|Default|GetShroomConstant))
                  ;[0 1 0.5355] Set primitive data back to 0
                  (Utilities|FlowControl|Delay 0.6)
                  (Rendering|Material|SetCustomPrimitiveDataFloat (Variables|Default|GetSM_PoisonousMushroom_08) 0 0.0)
                  ;[1 0.1824 0.8026] Turn ShroomConstant back on after delay
                  (Utilities|FlowControl|Delay 3.0)
                  (Variables|Default|SetWasActivated false)
                  (Components|Activation|Activate (Variables|Default|GetShroomConstant) false)
                  (Utilities|FlowControl|Delay 3.0)
                  (Class|DefaultStatComponent|RemoveEffect (Variables|/Script/Kari.DefaultPlayer|GetBlessing _returnvalue) _returnvalue_2 self))))))))))

(event Custom|StopMushroomBurst
  (Utilities|FlowControl|Delay 6.0)
  (Components|Activation|Deactivate (Variables|Default|GetShroomBurst)))

(event EventBeginPlay
  (Rendering|Material|SetCustomPrimitiveDataFloat (Variables|Default|GetSM_PoisonousMushroom_08) 0 0.0)
  (bind _asgi_default_game_instance (Utilities|Casting|CastToGI_DefaultGameInstance (Game|GetGameInstance)))
  (Variables|Default|SetGameInstance _asgi_default_game_instance))

(fn ConstructionScript)