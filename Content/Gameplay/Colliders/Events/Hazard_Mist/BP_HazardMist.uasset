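; BP_HazardMist is a mist hazard volume that applies a Blessing debuff to the player, Kari, while she overlaps it.
; Box overlaps toggle whispers and the in-mist flag, and add or remove the effect for her capsule only.
; While she is inside, Tick writes her raised location and a Blessing-scaled radius to a Material Parameter Collection for the mist's sphere mask.
; Getter-supplied modifiers adjust radius and damage.
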(event OnComponentBeginOverlap(Cube)
  (params (OverlappedComponent :type Primitive%20Component%20Object%20Reference) (OtherActor :type Actor%20Object%20Reference) (OtherComp :type Primitive%20Component%20Object%20Reference) (OtherBodyIndex :type Integer) (bFromSweep :type Boolean) (SweepResult :type Hit%20Result%20Structure%20%28by%20ref%29))
  (bind _mistdamage (Variables|Default|GetMistDamage))
  (bind _asbp_kari (Utilities|Casting|CastToBP_Kari OtherActor))
  (Variables|Default|SetPlayerInMist true)
  (Default|PlayWhispers _asbp_kari)
  (bind _returnvalue (Class|PersistenceLibrary|GetMistDamageMultiplier))
  (if (== OtherComp (Variables|/Script/Engine.Character|GetCapsuleComponent _asbp_kari))
    (Class|DefaultStatComponent|ApplyEffect (Variables|/Script/Kari.DefaultPlayer|GetBlessing _asbp_kari) (Variables|Default|GetMistBlessingDebuffIndex) self (Utilities|Struct|MakeStatEffect (* (.amount _mistdamage) (- (Variables|Default|GetMistDamageMultiplier) _returnvalue)) (.resistancemultiplier _mistdamage)))))

(event OnComponentEndOverlap(Cube)
  (params (OverlappedComponent :type Primitive%20Component%20Object%20Reference) (OtherActor :type Actor%20Object%20Reference) (OtherComp :type Primitive%20Component%20Object%20Reference) (OtherBodyIndex :type Integer))
  (bind _asbp_kari (Utilities|Casting|CastToBP_Kari OtherActor))
  (Variables|Default|SetPlayerInMist false)
  (Default|StopWhispers _asbp_kari)
  (if (== OtherComp (Variables|/Script/Engine.Character|GetCapsuleComponent _asbp_kari))
    (Class|DefaultStatComponent|RemoveEffect (Variables|/Script/Kari.DefaultPlayer|GetBlessing _asbp_kari) (Variables|Default|GetMistBlessingDebuffIndex) self)))

(event Custom|UpdateMistRadius
  (bind _returnvalue (Game|Player|GetPlayerPawn 0))
  (bind _returnvalue_2 (Transformation|GetActorLocation _returnvalue))
  ;[1 1 1] Gets player's location to
  (Rendering|Material|SetVectorParameterValue "/Game/Gameplay/Colliders/Events/MPC_MaterialVariables.MPC_MaterialVariables" "playerLocation" (Math|Conversions|ToLinearColor(Vector) (Math|Vector|MakeVector (.x _returnvalue_2) (.y _returnvalue_2) (+ (.z _returnvalue_2) 1.5e+02))) :!class /Script/Engine.KismetMaterialLibrary)
  ;[1 1 1] Determines Radius of mist hazard based on Player's Faith
  (bind _asbp_kari (Utilities|Casting|CastToBP_Kari (Game|GetPlayerCharacter 0)))
  (bind _returnvalue_3 (Class|PersistenceLibrary|GetMistRadiusMultiplier))
  (Rendering|Material|SetScalarParameterValue "/Game/Gameplay/Colliders/Events/MPC_MaterialVariables.MPC_MaterialVariables" "Radius" (* (Class|DefaultStatComponent|Normalized (Variables|/Script/Kari.DefaultPlayer|GetBlessing _asbp_kari)) (+ (Variables|Default|GetMistRadiusMultiplier) _returnvalue_3)) :!class /Script/Engine.KismetMaterialLibrary))

(event EventTick
  (params (DeltaSeconds :type Float%20%28single-precision%29))
  (bind _returnvalue (Game|Player|GetPlayerPawn 0))
  (bind _returnvalue_2 (Transformation|GetActorLocation _returnvalue))
  ;[1 1 1] Gets player's location to
  (if (Variables|Default|GetPlayerInMist)
    (Rendering|Material|SetVectorParameterValue "/Game/Gameplay/Colliders/Events/MPC_MaterialVariables.MPC_MaterialVariables" "playerLocation" (Math|Conversions|ToLinearColor(Vector) (Math|Vector|MakeVector (.x _returnvalue_2) (.y _returnvalue_2) (+ (.z _returnvalue_2) 1.5e+02))) :!class /Script/Engine.KismetMaterialLibrary)
    ;[1 1 1] Determines Radius of mist hazard based on Player's Faith
    (bind _asbp_kari (Utilities|Casting|CastToBP_Kari (Game|GetPlayerCharacter 0)))
    (bind _returnvalue_3 (Class|PersistenceLibrary|GetMistRadiusMultiplier))
    (Rendering|Material|SetScalarParameterValue "/Game/Gameplay/Colliders/Events/MPC_MaterialVariables.MPC_MaterialVariables" "Radius" (* (Class|DefaultStatComponent|Normalized (Variables|/Script/Kari.DefaultPlayer|GetBlessing _asbp_kari)) (+ (Variables|Default|GetMistRadiusMultiplier) _returnvalue_3)) :!class /Script/Engine.KismetMaterialLibrary)))

(fn ConstructionScript)