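; A sun-beam gate that fades out and opens while ClearPath keeps being called.
; ClearPath plays a timeline driving the SunBeamDestroying scalar in a shared material parameter collection; each update consumes the overlap flag, pausing progress and restarting a delay timeline that reverses the fade.
; Finishing at low visibility calls Unlock, which hides the cube and disables collision without destroying the actor.
; OnLoadUnlock unlocks directly, and IsLocked reports the state.
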(event Custom|ClearPath
  ;[1 1 1] Trigger + Check for overlap
  (Variables|Default|SetIsOverlapping true)
  (if (Variables|Default|GetIsOverlapping) :!label _label
    ;[1 1 1] Set the transparancy
    (bind _gate_visibility (Timeline|PathVisibilty Play)
      (:Update
        (Rendering|Material|SetScalarParameterValue "/Game/Gameplay/Colliders/Events/MPC_MaterialVariables.MPC_MaterialVariables" "SunBeamDestroying" _gate_visibility :!class /Script/Engine.KismetMaterialLibrary)
        (if (Variables|Default|GetIsOverlapping)
          (Variables|Default|SetIsOverlapping false)
          (goto _label)))
      (:Finished
        ;[1 1 1] Destroys actor on Completion
        (if (<= _gate_visibility 0.1)
          (CallFunction|Unlock))))
    (else
      (CallFunction|RestorePath)
      (Timeline|PathVisibilty Stop))))

(event Custom|RestorePath
  ;[1 1 1] Reverses Progress
  (Timeline|Delay PlayFromStart
    (:Finished
      ;[1 1 1] Set the transparancy
      (bind _gate_visibility (Timeline|PathVisibilty Reverse)
        (:Update
          (Rendering|Material|SetScalarParameterValue "/Game/Gameplay/Colliders/Events/MPC_MaterialVariables.MPC_MaterialVariables" "SunBeamDestroying" _gate_visibility :!class /Script/Engine.KismetMaterialLibrary)
          (if (Variables|Default|GetIsOverlapping)
            (Variables|Default|SetIsOverlapping false)
            ;[1 1 1] Trigger + Check for overlap
            (if (Variables|Default|GetIsOverlapping)
              (Timeline|PathVisibilty Play)
              (else
                (CallFunction|RestorePath)
                (Timeline|PathVisibilty Stop)))))
        (:Finished
          ;[1 1 1] Destroys actor on Completion
          (if (<= _gate_visibility 0.1)
            (CallFunction|Unlock)))))))

(event EventOnLoadUnlock
  (CallFunction|Unlock))

(fn ConstructionScript)

(fn IsLocked
  (return (Variables|Default|GetLocked)))

(fn Unlock
  (bind _cube (Variables|Default|GetCube))
  (Collision|SetCollisionEnabled _cube "NoCollision")
  (Rendering|SetVisibility _cube false false)
  (Variables|Default|SetLocked false))