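; Loralei hazard that threatens Kari inside its danger zone during the day, switching off with its BGM trigger box at evening and night.
; Time-manager period changes and capsule overlaps gate a Tick that applies a negative Blessing effect, strengthening as Kari nears the food drop location.
; The same distance crossfades two BGM layers and is debug-printed.
; Destroying the hazard fades the music back, disables the zone and removes the effect.
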(event OnComponentBeginOverlap(DangerZone)
  (params (OverlappedComponent :type Primitive%20Component%20Object%20Reference) (OtherActor :type Actor%20Object%20Reference) (OtherComp :type Primitive%20Component%20Object%20Reference) (OtherBodyIndex :type Integer) (bFromSweep :type Boolean) (SweepResult :type Hit%20Result%20Structure%20%28by%20ref%29))
  ;[1 1 1] Checks wether Kari is in our outside the danger zone
  (bind _asbp_kari (Utilities|Casting|CastToBP_Kari OtherActor))
  (if (== (Variables|/Script/Engine.Character|GetCapsuleComponent _asbp_kari) OtherComp)
    (Variables|Default|SetInDangerZone true)))

(event OnComponentEndOverlap(DangerZone)
  (params (OverlappedComponent :type Primitive%20Component%20Object%20Reference) (OtherActor :type Actor%20Object%20Reference) (OtherComp :type Primitive%20Component%20Object%20Reference) (OtherBodyIndex :type Integer))
  ;[1 1 1] Checks wether Kari is in our outside the danger zone
  (bind _asbp_kari (Utilities|Casting|CastToBP_Kari OtherActor))
  (if (== (Variables|/Script/Engine.Character|GetCapsuleComponent _asbp_kari) OtherComp)
    (Variables|Default|SetInDangerZone false)
    (Class|DefaultStatComponent|RemoveEffect (Variables|/Script/Kari.DefaultPlayer|GetBlessing _asbp_kari) 52 self)))

(event Custom|CheckDayTime
  (params (Period :type EPeriod%20Enum :default "E_NIGHT"))
  ;[1 1 1] Checks if it is night time
  (switch Utilities|FlowControl|Switch|SwitchonEPeriod Period
    (:E_NIGHT
      (Variables|Default|SetIsNight true :!label _label)
      (Collision|SetCollisionEnabled (Variables|Default|GetBP_BGMTriggerBox) "NoCollision"))
    (:E_MORNING
      (Variables|Default|SetIsNight false)
      (Collision|SetCollisionEnabled (Variables|Default|GetBP_BGMTriggerBox) "QueryAndPhysics"))
    (:E_EVENING
      (goto _label))))

(event Custom|OnHazardDestroy
  (bind _bp_bgmtriggerbox (Variables|Default|GetBP_BGMTriggerBox))
  (bind _bgmfader (Variables|/Script/Kari.BGMTriggerBoxComponent|GetBGMFader _bp_bgmtriggerbox))
  (bind _targetbgm (Variables|/Script/Kari.BGMFader|GetTargetBGM _bgmfader))
  (Class|Audio|FadeVolume (Class|Playlist|GetAudioLayer _targetbgm) 0.0 1.0 1.0 false)
  (Class|Audio|FadeVolume (Class|Playlist|GetAudioLayer _targetbgm 2) 1.0 0.0 1.0 false)
  (Collision|SetCollisionEnabled (Variables|Default|GetDangerZone) "NoCollision")
  (Variables|Default|SetInDangerZone false)
  (Class|DefaultStatComponent|RemoveEffect (Variables|/Script/Kari.DefaultPlayer|GetBlessing (Variables|Default|GetPlayer)) 52 self))

(event EventTick
  (params (DeltaSeconds :type Float%20%28single-precision%29))
  (bind _screechdistance (Variables|Default|GetScreechDistance))
  (bind _screechoffsetfromitem (Variables|Default|GetScreechOffsetFromItem))
  (bind _bp_bgmtriggerbox (Variables|Default|GetBP_BGMTriggerBox))
  (bind _fooddroplocation (Variables|Default|GetFoodDropLocation))
  (bind _player (Variables|Default|GetPlayer))
  (bind _returnvalue (Transformation|GetDistanceTo _player _fooddroplocation))
  (bind _bgmfader (Variables|/Script/Kari.BGMTriggerBoxComponent|GetBGMFader _bp_bgmtriggerbox))
  (bind _returnvalue_2 (Math|Float|Max(Float) _returnvalue 0.1))
  (bind _targetbgm (Variables|/Script/Kari.BGMFader|GetTargetBGM _bgmfader))
  (bind _returnvalue_3 (/ _returnvalue_2 _screechdistance))
  (bind _returnvalue_4 (- _returnvalue_3 _screechoffsetfromitem))
  (bind _returnvalue_5 (Math|Float|Clamp(Float) _returnvalue_4))
  (if (not (Variables|Default|GetIsNight))
    (if (Variables|Default|GetInDangerZone)
      (Class|DefaultStatComponent|ApplyEffect (Variables|/Script/Kari.DefaultPlayer|GetBlessing _player) 52 self (Utilities|Struct|MakeStatEffect (/ (* (Variables|Default|GetDamageDistance) -1.0) _returnvalue_2) 1.0))
      (Class|Audio|SetVolume (Class|Playlist|GetAudioLayer _targetbgm) _returnvalue_5)
      (Class|Audio|SetVolume (Class|Playlist|GetAudioLayer _targetbgm 2) (- 1.0 _returnvalue_5))
      (Development|PrintString (Utilities|String|ToString(Float) _returnvalue_5) true true "(R=0.000000,G=0.660000,B=1.000000,A=1.000000)" 0.0))))

(event EventBeginPlay
  ;[1 1 1] Checks if it is night time
  (bind _asgi_default_game_instance (Utilities|Casting|CastToGI_DefaultGameInstance (Game|GetGameInstance)))
  (EventDispatchers|BindEventtoOnPeriodChanged (Variables|/Script/Kari.DefaultGameInstance|GetTimeManager _asgi_default_game_instance) (delegate Custom|CheckDayTime))
  (bind _asbp_kari (Utilities|Casting|CastToBP_Kari (Game|GetPlayerCharacter 0)))
  (Variables|Default|SetPlayer _asbp_kari))

(fn ConstructionScript)