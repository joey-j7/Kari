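; BP_ArcherProjectile is the projectile of the archer hazard, which damages the Kari character on impact.
; It expires after a set lifetime if nothing stops it.
; When ProjectileMovement stops, the box collider ignores pawns and switches to physics simulation, and a hit BP_Kari takes damage through its Blessing.
; The projectile then lingers for a bounce lifetime before destroying itself.
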(event OnProjectileStop(ProjectileMovement)
  (params (ImpactResult :type Hit%20Result%20Structure%20%28by%20ref%29))
  (bind _boxcollider (Variables|Default|GetBoxCollider))
  (Collision|SetCollisionResponsetoChannel _boxcollider "ECC_Pawn" "ECR_Ignore")
  (Physics|SetSimulatePhysics _boxcollider true)
  (bind _asbp_kari (Utilities|Casting|CastToBP_Kari (.HitActor (Collision|BreakHitResult ImpactResult)))
    (:then
      (Class|DefaultStatComponent|Damage (Variables|/Script/Kari.DefaultPlayer|GetBlessing _asbp_kari) (Variables|Default|GetDamage)))
    (:CastFailed
      _))
  (Utilities|FlowControl|Delay (Variables|Default|GetBounceLifeTime))
  (Actor|DestroyActor))

(event EventBeginPlay
  (Actor|SetLifeSpan (Variables|Default|GetLifeTime)))

(fn ConstructionScript)