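; Resource spawner actor that places random pickups at its spawn point offsets on BeginPlay and again on a looping timer.
; SpawnResources line-traces down at each point and skips any whose hit actor is an item or BP_Kari, which prevents stacking.
; Otherwise it spawns a random class from Pickups at the impact point, with rotation built from the surface normal and a random yaw to suit sloped ground.
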(event Custom|TimeLoop
  (CallFunction|SpawnResources))

(event EventBeginPlay
  (CallFunction|SpawnResources)
  (Utilities|Time|SetTimerbyEvent (delegate Custom|TimeLoop) (Variables|Default|GetSpawnTimer) true))

(fn ConstructionScript)

(fn SpawnResources
  (bind _returnvalue (Math|Random|RandomFloatinRange 0.0 359.0))
  (bind _pickups (Variables|Default|GetPickups))
  (bind _returnvalue_2 (Math|Vector|GetRightVector (Math|Rotator|MakeRotator 0.0 0.0 _returnvalue)))
  ;[1 1 1] Gets all Spawn Point locations and loops
  (for _array_element (Variables|Default|GetSpawnPointLocation)
    ;[1 1 1] Linetraces to floor, detects what is there with angle and height.
    (bind (_outhit _returnvalue_3) (Collision|LineTraceByChannel (Math|Vector|MakeVector (.x (+ _array_element (Transformation|GetWorldLocation (Variables|Default|GetDefaultSceneRoot)))) (.y (+ _array_element (Transformation|GetWorldLocation (Variables|Default|GetDefaultSceneRoot)))) (+ (.z (+ _array_element (Transformation|GetWorldLocation (Variables|Default|GetDefaultSceneRoot)))) 5e+01)) (Math|Vector|MakeVector (.x (+ _array_element (Transformation|GetWorldLocation (Variables|Default|GetDefaultSceneRoot)))) (.y (+ _array_element (Transformation|GetWorldLocation (Variables|Default|GetDefaultSceneRoot)))) (+ (.z (+ _array_element (Transformation|GetWorldLocation (Variables|Default|GetDefaultSceneRoot)))) -2e+02)) "TraceTypeQuery1" false 0 "None" true "(R=0.000000,G=0.058855,B=1.000000,A=1.000000)" "(R=1.000000,G=0.000000,B=0.000000,A=1.000000)" 1e+01))
    (if _returnvalue_3
      ;;[1 1 1] Get the list of pickups, pick one and see if its already there and if Kari is standing on it.
      ;;;[1 1 1] Yes this is the only solution to item stacking don't hit me.
      (if (not (Utilities|ClassIsChildOf (Utilities|GetClass (.HitActor (Collision|BreakHitResult _outhit))) "/Script/Kari.ItemBase"))
        (if (not (Utilities|ClassIsChildOf (Utilities|GetClass (.HitActor (Collision|BreakHitResult _outhit))) "/Game/Environment/Props/Pickups/BP_ItemBase.BP_ItemBase_C"))
          (if (not (Utilities|ClassIsChildOf (Utilities|GetClass (.HitActor (Collision|BreakHitResult _outhit))) "/Game/Characters/Playable/Kari/BP_Kari.BP_Kari_C"))
            ;[1 1 1] Spawn Item
            (Game|SpawnActorfromClass (Utilities|Array|Get(acopy) _pickups (Math|Random|RandomInteger (Utilities|Array|Length _pickups))) (Math|Transform|MakeTransform (.Location (Collision|BreakHitResult _outhit)) (Math|Rotator|MakeRotationfromAxes (Math|Vector|CrossProduct (Math|Vector|NegateVector (.Normal (Collision|BreakHitResult _outhit))) _returnvalue_2) _returnvalue_2 (Math|Vector|NegateVector (.Normal (Collision|BreakHitResult _outhit))))) "AdjustIfPossibleButAlwaysSpawn" 0 0)))))))