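; Box-shaped spawn area that keeps itself stocked with random resource pickups during play.
; On BeginPlay and on a looping timer, it counts overlapping ItemBase actors and attempts one spawn per missing item up to MaximumInArea.
; Each attempt line-traces down from random points in the box and, on a hit, spawns a random Pickups class there, rotated using the surface normal and random yaw.
; The construction script sizes the box from BoxExtentVariable.
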(event Custom|TimeLoop
  (CallFunction|SpawnResources))

(event EventBeginPlay
  (CallFunction|SpawnResources)
  (bind _returnvalue (Utilities|Time|SetTimerbyEvent (delegate Custom|TimeLoop) (Variables|Default|GetSpawnTimer) true))
  (Variables|Default|SetRemainingTime _returnvalue))

(fn ConstructionScript
  (Components|Box|SetBoxExtent (Variables|Default|GetSpawnArea) (Variables|Default|GetBoxExtentVariable) true))

(fn SpawnResources
  (bind _returnvalue (Math|Random|RandomFloatinRange 0.0 359.0))
  (bind _pickups (Variables|Default|GetPickups))
  (bind _boxextentvariable (Variables|Default|GetBoxExtentVariable))
  (bind _maximuminarea (Variables|Default|GetMaximumInArea))
  (bind _defaultsceneroot (Variables|Default|GetDefaultSceneRoot))
  (bind _returnvalue_2 (Transformation|GetWorldLocation _defaultsceneroot))
  (bind _returnvalue_3 (Math|Vector|GetRightVector (Math|Rotator|MakeRotator 0.0 0.0 _returnvalue)))
  (bind _returnvalue_4 (Math|Random|RandomPointinBoundingBox _returnvalue_2 _boxextentvariable))
  ;[1 1 1] Get overlapping actors and set an integer
  (bind _output_get (Variables|Default|SetAmountInArea (Collision|GetOverlappingActors (Variables|Default|GetSpawnArea) "/Script/Kari.ItemBase" :!class /Script/Engine.PrimitiveComponent)))
  ;[1 1 1] Get Maximum and see if its less than maximum, then spawn till maximum
  (if (<= (Utilities|Array|Length _output_get) _maximuminarea)
    (for _index (range 1 (- _maximuminarea (Utilities|Array|Length _output_get)))
      ;[1 1 1] Linetraces to floor, detects what is there with angle and height.
      (bind (_outhit _returnvalue_5) (Collision|LineTraceByChannel (Math|Vector|MakeVector (.x _returnvalue_4) (.y _returnvalue_4) (.z _returnvalue_4)) (Math|Vector|MakeVector (.x _returnvalue_4) (.y _returnvalue_4) -1e+03) "TraceTypeQuery1" false 0 "None" true "(R=0.000000,G=0.058855,B=1.000000,A=1.000000)" "(R=1.000000,G=0.000000,B=0.000000,A=1.000000)" 1e+01))
      (if _returnvalue_5
        ;[1 1 1] Get a Pickup from the pickup array and spawn it.
        (Game|SpawnActorfromClass (Utilities|Array|Get(acopy) _pickups (Math|Random|RandomInteger (Utilities|Array|Length _pickups))) (Math|Transform|MakeTransform (.Location (Collision|BreakHitResult _outhit)) (Math|Rotator|MakeRotationfromAxes (Math|Vector|CrossProduct (Math|Vector|NegateVector (.Normal (Collision|BreakHitResult _outhit))) _returnvalue_3) _returnvalue_3 (Math|Vector|NegateVector (.Normal (Collision|BreakHitResult _outhit))))) "AdjustIfPossibleButAlwaysSpawn" 0 0)))))