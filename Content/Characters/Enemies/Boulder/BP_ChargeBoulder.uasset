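; BP_ChargeBoulder is a charging boulder enemy that damages BP_Kari's Blessing and knocks the character back on overlap.
; Sphere overlaps flag Collided on the Blackboard; hits on Kari also store the impact location and launch Kari using the negated, scaled Karidirection key.
; IncreaseRotation and DecreaseRotation events play timelines that drive RotatingMovement to spin the boulder up and down.
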(event OnComponentBeginOverlap(Sphere1)
  (params (OverlappedComponent :type Primitive%20Component%20Object%20Reference) (OtherActor :type Actor%20Object%20Reference) (OtherComp :type Primitive%20Component%20Object%20Reference) (OtherBodyIndex :type Integer) (bFromSweep :type Boolean) (SweepResult :type Hit%20Result%20Structure%20%28by%20ref%29))
  ;[1 1 1] Applies damage
  (bind _asbp_kari (Utilities|Casting|CastToBP_Kari OtherActor)
    (:then
      (bind _returnvalue (Class|DefaultStatComponent|GetCurrent (Variables|/Script/Kari.DefaultPlayer|GetBlessing _asbp_kari)))
      (Class|DefaultStatComponent|SetCurrent (Variables|/Script/Kari.DefaultPlayer|GetBlessing _asbp_kari) (- _returnvalue (Variables|Default|GetBlessing%20damage)))
      (AI|Components|Blackboard|SetValueasBool (AI|GetBlackboard 0) (Utilities|Name|MakeLiteralName "Collided") true)
      (AI|Components|Blackboard|SetValueasVector (AI|GetBlackboard 0) (Utilities|Name|MakeLiteralName "ImpactLocation") (Transformation|GetActorLocation (.HitActor (Collision|BreakHitResult SweepResult))))
      (Character|LaunchCharacter _asbp_kari (* (AI|Components|Blackboard|GetValueasVector (AI|GetBlackboard 0) (Utilities|Name|MakeLiteralName "Karidirection")) -1.5) false false))
    (:CastFailed
      (AI|Components|Blackboard|SetValueasBool (AI|GetBlackboard 0) (Utilities|Name|MakeLiteralName "Collided") true))))

(event Custom|Increase%20Rotation
  ;[1 1 1] Rotation acceleration / deceleration
  (bind _newtrack_0 (Timeline|Rotation%20Acceleration Play)
    (:Update
      (Variables|/Script/Engine.RotatingMovementComponent|SetRotationRate (Variables|Default|GetRotatingMovement) (Math|Rotator|MakeRotator _newtrack_0 _newtrack_0 0.0)))))

(event Custom|Decrease%20Rotation
  ;[1 1 1] Rotation acceleration / deceleration
  (bind _newtrack_0 (Timeline|Rotation%20Deceleration Play)
    (:Update
      (Variables|/Script/Engine.RotatingMovementComponent|SetRotationRate (Variables|Default|GetRotatingMovement) (Math|Rotator|MakeRotator _newtrack_0 _newtrack_0 0.0)))))

(event Collision|EventActorBeginOverlap
  (params (OtherActor :type Actor%20Object%20Reference)))

(fn ConstructionScript)