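; Enemy spawner that places a BP_Wisp running BT_Wisp at its own location on BeginPlay and respawns it after death.
; Each spawn passes the detection range, any valid patrol points and a reference to the spawner into the new wisp.
; SpawnEnemy waits for RespawnTimer, then reuses the same spawn logic for respawns.
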(event Custom|Spawn%20Enemy
  (bind _patrol_points (Variables|Default|GetPatrol%20points))
  ;[1 1 1] Respawn after wisp death
  (Utilities|FlowControl|Delay (Variables|Default|GetRespawn%20timer))
  ;[1 1 1] Spawns wisp
  (bind _returnvalue (AI|SpawnAIFromClass "/Game/Characters/Enemies/Wisp/BP_Wisp.BP_Wisp_C" "/Game/Characters/Enemies/Wisp/BT_Wisp.BT_Wisp" (Transformation|GetActorLocation) "0, 0, 0" false))
  ;[1 1 1] Set wisp values
  (bind _asbp_wisp (Utilities|Casting|CastToBP_Wisp _returnvalue))
  (Variables|/Game/Characters/Enemies/Wisp/BP_Wisp.BP_Wisp_C|SetDetectionRangeLocal _asbp_wisp (Variables|Default|GetdetectionRange))
  (if (Utilities|IsValid _patrol_points)
    (Variables|/Game/Characters/Enemies/Wisp/BP_Wisp.BP_Wisp_C|SetPatrolPoints _asbp_wisp _patrol_points))
  (Variables|/Game/Characters/Enemies/Wisp/BP_Wisp.BP_Wisp_C|SetSpawner _asbp_wisp self))

(event EventBeginPlay
  (bind _patrol_points (Variables|Default|GetPatrol%20points))
  ;[1 1 1] Spawns wisp
  (bind _returnvalue (AI|SpawnAIFromClass "/Game/Characters/Enemies/Wisp/BP_Wisp.BP_Wisp_C" "/Game/Characters/Enemies/Wisp/BT_Wisp.BT_Wisp" (Transformation|GetActorLocation) "0, 0, 0" false))
  ;[1 1 1] Set wisp values
  (bind _asbp_wisp (Utilities|Casting|CastToBP_Wisp _returnvalue))
  (Variables|/Game/Characters/Enemies/Wisp/BP_Wisp.BP_Wisp_C|SetDetectionRangeLocal _asbp_wisp (Variables|Default|GetdetectionRange))
  (if (Utilities|IsValid _patrol_points)
    (Variables|/Game/Characters/Enemies/Wisp/BP_Wisp.BP_Wisp_C|SetPatrolPoints _asbp_wisp _patrol_points))
  (Variables|/Game/Characters/Enemies/Wisp/BP_Wisp.BP_Wisp_C|SetSpawner _asbp_wisp self))

(fn ConstructionScript)