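; Wisp enemy that drains Kari's Blessing on contact and feeds patrol, detection and temporary freak-out state to its AI Blackboard.
; DoOnce-gated overlaps rescale it per hit; a third hit, or a grave while the player is in range, calls the spawner, plays the impact animation and destroys it.
; Bait boxes also trigger freak-out.
; Timelines animate meshes and light flicker, while player distance drives Niagara parameters and light color and intensity.
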(event OnComponentBeginOverlap(Collider)
  (params (OverlappedComponent :type Primitive%20Component%20Object%20Reference) (OtherActor :type Actor%20Object%20Reference) (OtherComp :type Primitive%20Component%20Object%20Reference) (OtherBodyIndex :type Integer) (bFromSweep :type Boolean) (SweepResult :type Hit%20Result%20Structure%20%28by%20ref%29))
  (bind _returnvalue (AI|GetBlackboard 0))
  ;[1 1 1] Reduce blessing on collision
  (Utilities|Casting|CastToBlockingVolume OtherActor
    (:CastFailed
      (Utilities|FlowControl|DoOnce false :!label _label
        (:Completed
          (Utilities|Casting|CastToBP_WispGrave OtherActor
            (:then
              (if (ScalableFloat|GetValueasBool _returnvalue (Utilities|Name|MakeLiteralName "PlayerInRange"))
                (Variables|Default|SetHitCount 3.0)
                (if (>= (Variables|Default|GetHitCount) 3.0) :!label _label_2
                  (Default|SpawnEnemy (Variables|Default|GetSpawner))
                  (|AnimationImpact ; This animation should be played when the wisp disappears or collides with the player or whatever.
                    (:Out
                      (Actor|DestroyActor)
                      (Utilities|FlowControl|Delay 2.0 :!label _label_3)
                      (AI|Components|Blackboard|SetValueasBool (AI|GetBlackboard (Pawn|GetController)) (Utilities|Name|MakeLiteralName "ShouldFreakOut") false)
                      (goto _label Reset)))
                  (else
                    (bind (_direction _set_scale_1 _set_scale_2) (Timeline|Set%20Scale PlayFromStart)
                      (:Update
                        (switch int (Math|Float|Truncate (Variables|Default|GetHitCount))
                          (:1
                            (Transformation|SetRelativeScale3D (Variables|Default|GetWispMeshes) (Math|Vector|MakeVector _set_scale_1 _set_scale_1 _set_scale_1)))
                          (:2
                            (Transformation|SetRelativeScale3D (Variables|Default|GetWispMeshes) (Math|Vector|MakeVector _set_scale_2 _set_scale_2 _set_scale_2))))
                        (Variables|Default|SetSize%20set (Variables|/Script/Engine.SceneComponent|GetRelativeScale3D (Variables|Default|GetWispMeshes)))
                        (goto _label_3))
                      (:Impact%20Animation
                        _))))
                (else
                  (goto _label Reset))))
            (:CastFailed
              (Utilities|Casting|CastToBP_BaitBox OtherActor
                (:then
                  (AI|Components|Blackboard|SetValueasBool _returnvalue (Utilities|Name|MakeLiteralName "ShouldFreakOut") true)
                  (goto _label_3))
                (:CastFailed
                  (AI|Components|Blackboard|SetValueasBool (AI|GetBlackboard 0) (Utilities|Name|MakeLiteralName "ShouldFreakOut") true)
                  (Variables|Default|SetHitCount (+ (Variables|Default|GetHitCount) 1.0))
                  (bind _asbp_kari (Utilities|Casting|CastToBP_Kari OtherActor)
                    (:then
                      (Class|DefaultStatComponent|Damage (Variables|/Script/Kari.DefaultPlayer|GetBlessing _asbp_kari) (Variables|Default|GetBlessing%20Damage) self)
                      (goto _label_2))
                    (:CastFailed
                      (goto _label Reset)))))))
          (Components|Activation|Activate (Variables|Default|GetPS_ImpactEffect) true))))))

(event Custom|Checks%20patrol%20points
  ;[1 1 1] Set patrol points
  (AI|Components|Blackboard|SetValueasBool (AI|GetBlackboard 0) (Utilities|Name|MakeLiteralName "HasPatrolPoints") true))

(event EventBeginPlay
  ;[1 1 1] Checks for patrol paths
  (|AnimationContinuous ; This animation should be played continuously
    (:Out
      (if (Utilities|IsValid (Variables|Default|GetPatrolPoints))
        (CallFunction|ChecksPatrolPoints))
      (AI|Components|Blackboard|SetValueasFloat (AI|GetBlackboard 0) (Utilities|Name|MakeLiteralName "Detection Range") (Variables|Default|GetDetectionRangeLocal)))))

(event EventTick
  (params (DeltaSeconds :type Float%20%28single-precision%29))
  ;[1 1 1] Distance Based Effects
  (Variables|Default|SetWispEffectDistance (|DistanceCalculation (Variables|Default|GetVisualsActivationDistance)))
  (|DistanceBasedEffects))

(fn ConstructionScript)