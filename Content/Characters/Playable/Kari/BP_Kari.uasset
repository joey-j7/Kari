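; BP_Kari is the playable character Kari, built around a Blessing resource that drains by default, with an extra storm drain effect.
; Blessing changes drive low-blessing and external-damage visuals through a Material Parameter Collection, and respawn refills Blessing with a timeline-driven god-ray effect.
; It also manages screen HUD visibility, torch visibility from inventory, pickup and tutorial hooks, range-checked interaction, a camera-facing waypoint, whisper audio and auto-walk cancelling.
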(event OnDamaged(Blessing)
  (params (IsEffectDamage :type Boolean) (Amount :type Float%20%28single-precision%29) (Source :type Actor%20Object%20Reference))
  (bind _damageindicatortimeline (Variables|Default|GetDamageIndicatorTimeline))
  (Utilities|FlowControl|Sequence
    (:then_0
      ;[0.2502 0.8148 1] Sets lowblessing parameter in material based on blessing
      (Rendering|Material|SetScalarParameterValue "/Game/Gameplay/Colliders/Events/MPC_MaterialVariables.MPC_MaterialVariables" "KariLowBlessing" (Math|Curves|GetFloatValue (Variables|Default|GetLowBlessing) (Class|DefaultStatComponent|Normalized (Variables|Default|GetBlessing))) :!class /Script/Engine.KismetMaterialLibrary))
    (:then_1
      ;[1 1 1] OnDamage Effect
      (Utilities|Casting|CastToBP_Kari Source ; Only show damage effect on damage inflicted by hazard (external damage sources)
        (:CastFailed
          (if (not (Audio|Components|Audio|IsPlaying _damageindicatortimeline))
            (bind _karidamageindicator (Timeline|DamageIndicatorTimeline Play)
              (:Update
                (Rendering|Material|SetScalarParameterValue "/Game/Gameplay/Colliders/Events/MPC_MaterialVariables.MPC_MaterialVariables" "KariDamageIndicator" _karidamageindicator :!class /Script/Engine.KismetMaterialLibrary))
              (:Finished
                (Components|Timeline|SetNewTime _damageindicatortimeline 0.0)))))))))

(event Custom|PlayWhispers
  ;[1 1 1] Player whisper audio when taking damage
  (Utilities|IsValid (Variables|Default|GetWhispersSFX)
    (:Is%20Valid
      (Class|Playlist|FadeVolume (Variables|Default|GetWhispersSFX) 0.5 1.0 false))
    (:Is%20Not%20Valid
      (bind _returnvalue (Class|AudioManager|Play (Variables|/Script/Kari.DefaultGameInstance|GetAudioManager (Variables|Default|GetGameInstance)) (Utilities|Array|MakeArray "Global/Overworld/Mist/Mist.amb") true 0 0 1.0 1.0 0.0 0.5 false))
      (Class|Playlist|FadeVolume _returnvalue 0.5 1.0 false)
      (Variables|Default|SetWhispersSFX _returnvalue))))

(event Custom|OnItemPickup
  (params (Item :type Item%20Structure))
  ;[1 1 1] Checks if Item is being picked up
  (bind _asdefault_game_instance (Utilities|Casting|CastToDefaultGameInstance (Game|GetGameInstance)))
  (bind _returnvalue (Class|Inventory|CheckAvailableItemSlot (Variables|/Script/Kari.DefaultGameInstance|GetInventory _asdefault_game_instance) (.ID (Utilities|Struct|BreakItem Item))))
  (if _returnvalue
    (Animation|Montage|PlayMontage (Variables|Character|GetMesh) "/Game/Characters/Playable/Kari/ANIMON_Kari_PickupLow.ANIMON_Kari_PickupLow"
      (:then
        (Class|AudioManager|Play (Variables|/Script/Kari.DefaultGameInstance|GetAudioManager (Variables|Default|GetGameInstance)) (Utilities|Array|MakeArray "Global/Player/Pickup") false 0 0 0.9 1.1 0.0 0.5 false)
        (Default|CallDespawnBagtutorial)))))

(event Custom|StopWhispers
  (bind _whisperssfx (Variables|Default|GetWhispersSFX))
  (if (Utilities|IsValid _whisperssfx)
    (Class|Playlist|FadeVolume _whisperssfx 0.0 1.0 false)))

(event Custom|ApplyStormBlessingDrain
  (bind _returnvalue (Class|DefaultStatComponent|ApplyEffectUnique (Variables|Default|GetBlessing) self (Variables|Default|GetStormBlessingDecreaseRate)))
  (Variables|Default|SetStormBlessingDecreaseEffectId _returnvalue))

(event Custom|ApplyDefaultBlessingDrain
  (if (>= (Variables|Default|GetStormBlessingDecreaseEffectId) 0)
    (Class|DefaultStatComponent|RemoveEffect (Variables|Default|GetBlessing) (Variables|Default|GetStormBlessingDecreaseEffectId) self)))

(event Custom|SetWaypoint
  (params (Show :type Boolean) (Position :type Vector))
  (bind _waypoint (Variables|Default|GetWaypoint))
  (Rendering|SetVisibility _waypoint Show false)
  (Transformation|SetWorldLocation _waypoint Position false true)
  (Transformation|SetWorldRotation (Variables|Default|GetWaypoint) (Math|Conversions|RotationFromXVector (* (Math|Vector|GetForwardVector (Class|DefaultCameraSystemComponent|GetCamera (Variables|Default|GetCameraSystem))) -1.0)) false false))

(event EventBeginPlay
  (|CallParentFunction)
  (Utilities|FlowControl|Sequence
    (:then_0
      ;[0.2502 0.8148 1] Sets lowblessing parameter in material based on blessing
      (Rendering|Material|SetScalarParameterValue "/Game/Gameplay/Colliders/Events/MPC_MaterialVariables.MPC_MaterialVariables" "KariLowBlessing" (Math|Curves|GetFloatValue (Variables|Default|GetLowBlessing) (Class|DefaultStatComponent|Normalized (Variables|Default|GetBlessing))) :!class /Script/Engine.KismetMaterialLibrary))
    (:then_1
      (CallFunction|CheckTorchRequirement)
      ;[1 1 1] Called at actor creation
      (Development|SetHiddeninGame (Variables|Default|GetPlayerHUD) (Variables|Default|GetStartWithoutHUD) false)
      (bind _aspc_default_player_controller (Utilities|Casting|CastToPC_DefaultPlayerController (Game|GetPlayerController 0)))
      (Variables|Default|SetDefaultPlayerControllerReference _aspc_default_player_controller))
    (:then_2
      (bind _returnvalue (UserInterface|CreateWidget "/Game/UI/HUD/WBP_ScreenHUD.WBP_ScreenHUD_C"))
      (UserInterface|Viewport|AddtoViewport _returnvalue 0)
      (bind _output_get (Variables|Default|SetScreenHUD _returnvalue))
      (Widget|SetVisibility _output_get "Collapsed"))))

(event EventTick
  (params (DeltaSeconds :type Float%20%28single-precision%29))
  (bind _defaultplayercontrollerreference (Variables|Default|GetDefaultPlayerControllerReference))
  (|CallParentFunction DeltaSeconds)
  (Utilities|IsValid _defaultplayercontrollerreference
    (:Is%20Valid
      (Widget|SetVisibility (Variables|Default|GetScreenHUD) (select (Math|Boolean|ANDBoolean (Class|DefaultPlayer|IsInputEnabled) (Class|DefaultPlayerController|IsInputEnabled _defaultplayercontrollerreference) (Default|CanContinue _defaultplayercontrollerreference) (not (Class|DefaultPlayer|IsInteracting))) "Visible" "Collapsed")))))

(event EventGameBegin
  ;[1 1 1] Called on game start (default Blessing drain rate)
  (bind _returnvalue (Class|DefaultStatComponent|ApplyEffectUnique (Variables|Default|GetBlessing) self (Variables|Default|GetBlessingDecreaseRate)))
  (Variables|Default|SetDefaultBlessingDecreaseEffectId _returnvalue))

(event EventRespawn
  (bind _blessing (Variables|Default|GetBlessing))
  (|CallParentFunction)
  (Animation|Montage|PlayMontage (Variables|Character|GetMesh) "/Game/Characters/Playable/Kari/ANIMON_Kari_Respawn.ANIMON_Kari_Respawn"
    (:then
      (Class|DefaultStatComponent|ClearEffects _blessing)
      (Class|DefaultStatComponent|SetCurrent _blessing (Variables|/Script/Kari.DefaultStatComponent|GetMax _blessing))
      (bind _returnvalue (Class|DefaultStatComponent|ApplyEffectUnique (Variables|Default|GetBlessing) self (Variables|Default|GetBlessingDecreaseRate)))
      (Variables|Default|SetDefaultBlessingDecreaseEffectId _returnvalue)
      (|RespawnVFX))))

(event EventOnInventoryChange
  (|CallParentFunction)
  (CallFunction|CheckTorchRequirement))

(event EventOnInteract
  (params (Interactable :type Actor%20Object%20Reference))
  ;[1 1 1] Despawns Interact Tutorial
  (|CallParentFunction Interactable)
  (Default|CallDespawnInteractTutorial))

(event Input|AxisEvents|InputAxisMoveX
  (params (AxisValue :type Float%20%28single-precision%29))
  (if (!= AxisValue 0.0)
    (Default|StopAutoWalking (Variables|Default|GetDefaultPlayerControllerReference))))

(event Input|AxisEvents|InputAxisMoveY
  (params (AxisValue :type Float%20%28single-precision%29))
  (if (!= AxisValue 0.0)
    (Default|StopAutoWalking (Variables|Default|GetDefaultPlayerControllerReference))))

(fn ConstructionScript)

(fn EquipablePickedUp
  (params (ResistBuff :type Array%20of%20Booleans)))

(fn StartCameraFade
  (CameraFades|StartCameraFade :self (Game|GetPlayerCameraManager 0) :ToAlpha 1.0 :Duration 1.5 :bHoldWhenFinished true))

(fn DoRespawn
  (Class|SaveLibrary|Respawn true))

(fn StopCameraFade
  (CameraFades|StartCameraFade :self (Game|GetPlayerCameraManager 0) :FromAlpha 1.0 :Duration 1.5))

(fn CheckTorchRequirement
  (bind _gameinstance (Variables|Default|GetGameInstance))
  (Utilities|IsValid _gameinstance
    (:Is%20Valid
      (bind _output_get (LocalVariables|SetGI _gameinstance)))
    (:Is%20Not%20Valid
      (bind _asgi_default_game_instance (Utilities|Casting|CastToGI_DefaultGameInstance (Game|GetGameInstance)))
      (LocalVariables|SetGI _asgi_default_game_instance)))
  ;[1 1 1] Set torch to visible if torch item is in inventory, torch BP does the day/night check
  (bind _returnvalue (Class|Inventory|CountItem (Variables|/Script/Kari.DefaultGameInstance|GetInventory _output_get) 23))
  (Utilities|IsValid (Variables|Default|GetBPTorch)
    (:Is%20Valid
      _)
    (:Is%20Not%20Valid
      (bind _asbp_player_torch (Utilities|Casting|CastToBP_PlayerTorch (Variables|/Script/Engine.ChildActorComponent|GetChildActor (Variables|Default|GetTorch))))
      (Variables|Default|SetBPTorch _asbp_player_torch)))
  (Default|SetVisible (Variables|Default|GetBPTorch) (> _returnvalue 0)))

(fn Interactwith
  (params (Interactable :type Interactable%20Component%20Object%20Reference))
  (bind _returnvalue (Transformation|GetActorLocation))
  (bind _returnvalue_2 (Components|GetOwner Interactable))
  (bind (_origin _boxextent) (Collision|GetActorBounds _returnvalue_2 false false))
  (Utilities|IsValid Interactable
    (:Is%20Valid
      (if (< (Math|Vector|Distance(Vector) (Math|Vector|FindClosestPointonSegment _returnvalue (+ _origin (* _boxextent -1.0)) (+ _origin _boxextent)) _returnvalue) (Components|Sphere|GetScaledSphereRadius (Variables|Default|GetInteractionRange)))
        (Default|StopAutoWalking (Variables|Default|GetDefaultPlayerControllerReference))
        (Class|InteractableComponent|BroadCastonInteract Interactable)
        (return true)
        (else
          _)))
    (:Is%20Not%20Valid
      _))
  (return false))