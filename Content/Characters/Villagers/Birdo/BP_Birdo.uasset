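; Birdo villager character Blueprint holding movement and survival-stat functions, with stats named for Kari; its event graph has no active logic.
; Movement is blocked in menus and ignores control yaw, keeping north-south and west-east on world axes.
; Energy drains when moving or sprinting; moving without enough energy, or running out of faith, passes drain into health.
; Sprinting alone skips the energy clamp, and death only prints a debug message.
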(event EventTick
  (params (DeltaSeconds :type Float%20%28single-precision%29)))

(fn ConstructionScript)

(fn MoveNorthSouth
  (params (ScaleValue :type Float%20%28single-precision%29))
  (if (not (Variables|Default|GetInMenu))
    (Pawn|Input|AddMovementInput (Math|Vector|GetForwardVector (Math|Rotator|MakeRotator 0.0 (.Pitch (Math|Rotator|BreakRotator (Pawn|GetControlRotation :!class /Script/Engine.Pawn))) 0.0)) ScaleValue false)))

(fn MoveWestEast
  (params (ScaleValue :type Float%20%28single-precision%29))
  (if (not (Variables|Default|GetInMenu))
    (Pawn|Input|AddMovementInput (Math|Vector|GetRightVector (Math|Rotator|MakeRotator 0.0 (.Pitch (Math|Rotator|BreakRotator (Pawn|GetControlRotation :!class /Script/Engine.Pawn))) 0.0)) ScaleValue false)))

(fn EnergyDrain
  (if (Variables|Default|GetKari_IsMoving)
    (if (< (- (Variables|Default|GetKari_Energy) (Variables|Default|GetKari_Energy_Drain)) 0.0)
      (Variables|Default|SetKari_Energy 0.0)
      (CallFunction|HealthDrain (Variables|Default|GetKari_Energy_Drain))
      (else
        (Variables|Default|SetKari_Energy (- (Variables|Default|GetKari_Energy) (Variables|Default|GetKari_Energy_Drain)) :!label _label)
        (Development|PrintText (Utilities|Text|ToText(Float) (Variables|Default|GetKari_Energy) "HalfToEven"))
        (Variables|Default|SetKari_IsMoving false)))
    (elif (Variables|Default|GetKari_IsSprinting)
      (goto _label))))

(fn HealthDrain
  (params (Damage :type Float%20%28single-precision%29))
  (if (< (- (Variables|Default|GetKari_Health) Damage) 0.0)
    (Variables|Default|SetKari_Health 0.0)
    (Development|PrintString "Death: Hello" true true "(R=0.487500,G=0.000000,B=0.028777,A=1.000000)")
    (else
      (bind _output_get (Variables|Default|SetKari_Health (- (Variables|Default|GetKari_Health) Damage)))
      (Development|PrintString (Utilities|String|ToString(Float) _output_get)))))

(fn FaithDrain
  (if (< (- (Variables|Default|GetKari_Faith) (Variables|Default|GetKari_Faith_Drain)) 0.0)
    (Variables|Default|SetKari_Faith 0.0)
    (CallFunction|HealthDrain (Variables|Default|GetKari_Faith_Drain))
    (else
      (bind _output_get (Variables|Default|SetKari_Faith (- (Variables|Default|GetKari_Faith) (Variables|Default|GetKari_Faith_Drain))))
      (Development|PrintString (Utilities|String|ToString(Float) _output_get)))))