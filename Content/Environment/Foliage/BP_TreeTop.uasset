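; BP_TreeTop is a foliage actor that gives its leaf plane a randomly chosen mask shape.
; On BeginPlay it creates a dynamic MI_PlaneLeaves material and sets its Mask from MaskTextures, with a random range that can overrun the array by one.
; It also caches BP_WorldLightController, but the logic rotating it to the light direction is disconnected.
; Seeded scattering of instanced branches in the construction script is likewise disconnected.
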(event EventBeginPlay
  (bind _masktextures (Variables|Default|GetMaskTextures))
  (bind _returnvalue (Actor|GetActorOfClass "/Game/General/Lighting/BP_WorldLightController.BP_WorldLightController_C"))
  (Variables|Default|SetWorldLight _returnvalue)
  (if (> (Utilities|Array|Length (Variables|Default|GetMaskTextures)) 0)
    (bind _returnvalue_2 (Rendering|Material|CreateDynamicMaterialInstance (Variables|Default|GetStaticMesh) 0 "/Game/Environment/Foliage/MI_PlaneLeaves.MI_PlaneLeaves" "None" :!class /Script/Engine.PrimitiveComponent))
    (Rendering|Material|SetTextureParameterValue _returnvalue_2 "Mask" (Utilities|Array|Get(acopy) _masktextures (Math|Random|RandomIntegerinRange 0 (Utilities|Array|Length _masktextures))))))

(event Collision|EventActorBeginOverlap
  (params (OtherActor :type Actor%20Object%20Reference)))

(event EventTick
  (params (DeltaSeconds :type Float%20%28single-precision%29)))

(fn ConstructionScript)