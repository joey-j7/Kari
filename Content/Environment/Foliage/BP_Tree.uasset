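; BP_Tree is a foliage tree Blueprint that draws one tree through two static mesh components, TreeVisible and TreeShadow.
; An Init event assigns the same TreeMesh to both components.
; The construction script is empty, and disconnected nodes outline an unused setup that would make TreeShadow a hidden shadow caster with a shadow-fade material while changing shadow casting on TreeVisible.
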(event Custom|Init
  (bind _treemesh (Variables|Default|GetTreeMesh))
  (Components|StaticMesh|SetStaticMesh (Variables|Default|GetTree_Visible) _treemesh)
  (Components|StaticMesh|SetStaticMesh (Variables|Default|GetTree_Shadow) _treemesh))

(fn ConstructionScript)