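; Placer actor that spawns a tree resin pickup, flagged as on-tree, and respawns it once it is gone.
; BeginPlay spawns the resin at the ItemCheckBox transform, then starts a one-shot timer with either a random or fixed delay.
; When the timer fires, OverlapCheck spawns a replacement if no pickup overlaps the box and the last resin is invalid, otherwise it restarts the timer.
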(event Custom|OverlapCheck
  (bind _itemcheckbox (Variables|Default|GetItemCheckBox))
  ;[1 1 1] Checks if there is already a pickup, if not repeats the spawn process.
  (if (and (not (Collision|IsOverlappingActor _itemcheckbox (Utilities|Array|Get(acopy) (Collision|GetOverlappingActors _itemcheckbox (Variables|Default|GetPickups) :!class /Script/Engine.PrimitiveComponent)) :!class /Script/Engine.PrimitiveComponent)) (not (Utilities|IsValid (Variables|Default|GetSpawnedResin))))
    (CallFunction|SpawnPickup)
    (else
      ;[1 1 1] Check if random timer is enabled
      (if (Variables|Default|GetRandomTimer)
        ;[1 1 1] Set Random Timer
        (Utilities|Time|SetTimerbyEvent (delegate Custom|OverlapCheck) (Math|Random|RandomFloatinRange (Variables|Default|GetRandomRespawnTimeMinimum) (Variables|Default|GetRandomRespawnTimeMaximum)))
        (else
          ;[1 1 1] Set constant timer
          (Utilities|Time|SetTimerbyEvent (delegate Custom|OverlapCheck) (Variables|Default|GetNonRandomRespawnTime)))))))

(event Custom|SpawnPickup
  ;[1 1 1] Spawns the Actor
  (bind _returnvalue (Game|SpawnActorfromClass "/Game/Environment/Props/Pickups/Tree_Resin/BP_TreeResin.BP_TreeResin_C" (Transformation|GetWorldTransform (Variables|Default|GetItemCheckBox)) "AlwaysSpawn" 0 true 0))
  (Variables|Default|SetSpawnedResin _returnvalue)
  ;[1 1 1] Check if random timer is enabled
  (if (Variables|Default|GetRandomTimer)
    ;[1 1 1] Set Random Timer
    (Utilities|Time|SetTimerbyEvent (delegate Custom|OverlapCheck) (Math|Random|RandomFloatinRange (Variables|Default|GetRandomRespawnTimeMinimum) (Variables|Default|GetRandomRespawnTimeMaximum)))
    (else
      ;[1 1 1] Set constant timer
      (Utilities|Time|SetTimerbyEvent (delegate Custom|OverlapCheck) (Variables|Default|GetNonRandomRespawnTime)))))

(event EventBeginPlay
  ;[1 1 1] Spawns the Actor
  (bind _returnvalue (Game|SpawnActorfromClass "/Game/Environment/Props/Pickups/Tree_Resin/BP_TreeResin.BP_TreeResin_C" (Transformation|GetWorldTransform (Variables|Default|GetItemCheckBox)) "AlwaysSpawn" 0 true 0))
  (Variables|Default|SetSpawnedResin _returnvalue)
  ;[1 1 1] Check if random timer is enabled
  (if (Variables|Default|GetRandomTimer)
    ;[1 1 1] Set Random Timer
    (Utilities|Time|SetTimerbyEvent (delegate Custom|OverlapCheck) (Math|Random|RandomFloatinRange (Variables|Default|GetRandomRespawnTimeMinimum) (Variables|Default|GetRandomRespawnTimeMaximum)))
    (else
      ;[1 1 1] Set constant timer
      (Utilities|Time|SetTimerbyEvent (delegate Custom|OverlapCheck) (Variables|Default|GetNonRandomRespawnTime)))))

(fn ConstructionScript)