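; BP_Cotton is a cotton pickup prop that adapts its look when it is on a plant.
; On BeginPlay, if OnPlant is set, it swaps its mesh to the cotton balls model and shifts the interactable component's position offset.
; It then calls the parent BeginPlay, with no other active logic of its own.
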(event EventBeginPlay
  (if (Variables|Default|GetOnPlant)
    (Components|StaticMesh|SetStaticMesh (Variables|Default|GetMeshComponent) "/Game/Environment/Props/Pickups/Cotton/SM_CottonBalls.SM_CottonBalls")
    (Variables|/Script/Kari.InteractableComponent|SetPositionOffset (Variables|Default|GetInteractableComponent) "100.000000,-75.000000, 0"))
  (|CallParentFunction))

(event Collision|EventActorBeginOverlap
  (params (OtherActor :type Actor%20Object%20Reference))
  (|CallParentFunction OtherActor) ; This node is disabled and will not be called.\nDrag off pins to build functionality.
)

(event EventTick
  (params (DeltaSeconds :type Float%20%28single-precision%29))
  (|CallParentFunction DeltaSeconds) ; This node is disabled and will not be called.\nDrag off pins to build functionality.
)

(fn ConstructionScript
  (|CallParentFunction))