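; Cloudberry berry pickup prop, a child Blueprint that relies on its parent for its remaining behavior.
; On BeginPlay, when OnBush is set, it swaps the mesh to the cloudberries static mesh and shifts the InteractableComponent's position offset before running the parent's BeginPlay.
; The construction script only calls the parent, and the overlap and tick events are disabled stubs.
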(event EventBeginPlay
  (if (Variables|Default|GetOnBush)
    (Components|StaticMesh|SetStaticMesh (Variables|Default|GetMeshComponent) "/Game/Environment/Props/Pickups/Berries/SM_Cloudberries_01.SM_Cloudberries_01")
    (Variables|/Script/Kari.InteractableComponent|SetPositionOffset (Variables|Default|GetInteractableComponent) "65.000000,-85.000000, 0"))
  (|CallParentFunction))

(event Collision|EventActorBeginOverlap
  (params (OtherActor :type Actor%20Object%20Reference))
  (|CallParentFunction OtherActor) ; This node is disabled and will not be called.\nDrag off pins to build functionality.
)

(event EventTick
  (params (DeltaSeconds :type Float%20%28single-precision%29))
  (|CallParentFunction DeltaSeconds) ; This node is disabled and will not be called.\nDrag off pins to build functionality.
)

(fn ConstructionScript
  (|CallParentFunction))