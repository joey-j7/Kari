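; BP_Billberry is a berry pickup prop that builds on a parent class for its core startup and item-use behavior.
; On BeginPlay, if OnBush is set, it swaps its mesh to SM_Berries and shifts the interactable component's position offset before running the parent logic.
; Using the item runs the parent's OnItemUse, reports the item to an Achievement call, and returns the parent's result.
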(event EventBeginPlay
  (if (Variables|Default|GetOnBush)
    (Components|StaticMesh|SetStaticMesh (Variables|Default|GetMeshComponent) "/Game/Environment/Props/Pickups/Berries/SM_Berries.SM_Berries")
    (Variables|/Script/Kari.InteractableComponent|SetPositionOffset (Variables|Default|GetInteractableComponent) "275.000000,-75.000000, 0"))
  (|CallParentFunction))

(event Collision|EventActorBeginOverlap
  (params (OtherActor :type Actor%20Object%20Reference))
  (|CallParentFunction OtherActor) ; This node is disabled and will not be called.\nDrag off pins to build functionality.
)

(event EventTick
  (params (DeltaSeconds :type Float%20%28single-precision%29))
  (|CallParentFunction DeltaSeconds) ; This node is disabled and will not be called.\nDrag off pins to build functionality.
)

(fn ConstructionScript
  (|CallParentFunction))

(fn OnItemUse
  (bind _canuse_out (|CallParentFunction))
  (CallFunction|Achievement 0 self -1 false -1)
  (return _canuse_out))