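; Cloudberry bush prop that spawns and respawns a cloudberry pickup on itself.
; On BeginPlay it spawns BP_Cloudberry_01 at the Plant transform, flagged as on-bush, then starts a one-shot timer with either a random or fixed delay.
; When the timer fires, an overlap check on ItemCheckBox restarts the timer if a pickup is still present, otherwise spawns a new berry and restarts it.
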(event Custom|OverlapCheck
  (bind _itemcheckbox (Variables|Default|GetItemCheckBox))
  ;[1 1 1] Checks if there is already a pickup, if not repeats the spawn process.
  (if (Collision|IsOverlappingActor _itemcheckbox (Utilities|Array|Get(acopy) (Collision|GetOverlappingActors _itemcheckbox (Variables|Default|GetPickups) :!class /Script/Engine.PrimitiveComponent)) :!class /Script/Engine.PrimitiveComponent)
    ;[1 1 1] Check if random timer is enabled
    (if (Variables|Default|GetRandomTimer)
      ;[1 1 1] Set Random Timer
      (Utilities|Time|SetTimerbyEvent (delegate Custom|OverlapCheck) (Math|Random|RandomFloatinRange (Variables|Default|GetRandomRespawnTimeMinimum) (Variables|Default|GetRandomRespawnTimeMaximum)))
      (else
        ;[1 1 1] Set constant timer
        (Utilities|Time|SetTimerbyEvent (delegate Custom|OverlapCheck) (Variables|Default|GetNonRandomRespawnTime))))
    (else
      (CallFunction|SpawnPickup))))

(event Custom|SpawnPickup
  ;[1 1 1] Spawns the Actor
  (Game|SpawnActorfromClass "/Game/Environment/Props/Pickups/Berries/BP_Cloudberry_01.BP_Cloudberry_01_C" (Transformation|GetWorldTransform (Variables|Default|GetPlant)) "AlwaysSpawn" 0 true 0)
  ;[1 1 1] Check if random timer is enabled
  (if (Variables|Default|GetRandomTimer)
    ;[1 1 1] Set Random Timer
    (Utilities|Time|SetTimerbyEvent (delegate Custom|OverlapCheck) (Math|Random|RandomFloatinRange (Variables|Default|GetRandomRespawnTimeMinimum) (Variables|Default|GetRandomRespawnTimeMaximum)))
    (else
      ;[1 1 1] Set constant timer
      (Utilities|Time|SetTimerbyEvent (delegate Custom|OverlapCheck) (Variables|Default|GetNonRandomRespawnTime)))))

(event EventBeginPlay
  ;[1 1 1] Spawns the Actor
  (Game|SpawnActorfromClass "/Game/Environment/Props/Pickups/Berries/BP_Cloudberry_01.BP_Cloudberry_01_C" (Transformation|GetWorldTransform (Variables|Default|GetPlant)) "AlwaysSpawn" 0 true 0)
  ;[1 1 1] Check if random timer is enabled
  (if (Variables|Default|GetRandomTimer)
    ;[1 1 1] Set Random Timer
    (Utilities|Time|SetTimerbyEvent (delegate Custom|OverlapCheck) (Math|Random|RandomFloatinRange (Variables|Default|GetRandomRespawnTimeMinimum) (Variables|Default|GetRandomRespawnTimeMaximum)))
    (else
      ;[1 1 1] Set constant timer
      (Utilities|Time|SetTimerbyEvent (delegate Custom|OverlapCheck) (Variables|Default|GetNonRandomRespawnTime)))))

(fn ConstructionScript)