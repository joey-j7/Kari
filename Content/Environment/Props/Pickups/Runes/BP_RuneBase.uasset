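; BP_RuneBase is a base Blueprint for rune pickups that handles what happens when the item is used.
; OnItemUse spawns the rune activation Niagara effect attached to Kari's mesh at a relative offset, passing the rune's UI symbol index as a float parameter.
; It then calls Achievement on itself and returns the parent's result, both skipped if the player character is not BP_Kari.
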(event EventBeginPlay
  (|CallParentFunction) ; This node is disabled and will not be called.\nDrag off pins to build functionality.
)

(event Collision|EventActorBeginOverlap
  (params (OtherActor :type Actor%20Object%20Reference))
  (|CallParentFunction OtherActor) ; This node is disabled and will not be called.\nDrag off pins to build functionality.
)

(event EventTick
  (params (DeltaSeconds :type Float%20%28single-precision%29))
  (|CallParentFunction DeltaSeconds) ; This node is disabled and will not be called.\nDrag off pins to build functionality.
)

(fn ConstructionScript
  (|CallParentFunction))

(fn OnItemUse
  (bind _asbp_kari (Utilities|Casting|CastToBP_Kari (Game|GetPlayerCharacter 0)))
  (bind _returnvalue (Niagara|SpawnSystemAttached "/Game/VFX/ParticleSystems/PS_RuneActivation.PS_RuneActivation" (Variables|/Script/Engine.Character|GetMesh _asbp_kari) "None" (Variables|Default|GetParticleOffset) "0, 0, 0" "KeepRelativeOffset" true))
  (Niagara|SetNiagaraVariable(Float) _returnvalue "Rune" (Math|Conversions|ToFloat(Integer) (Variables|Default|GetUIRuneSymbolIndex)))
  (CallFunction|Achievement 0 self -1 false -1)
  (bind _canuse_out (|CallParentFunction))
  (return _canuse_out))