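; BP_WaterDrifter is a component that makes its owning actor bob and roll as if floating on water waves.
; BeginPlay caches its rest rotation and height, plus the larger X/Y scale of an optional WaterPlane.
; Each Tick, WaveSurge sums two time-scrolled sine waves sampled from scale-adjusted world XY.
; The inverted surge offsets the owner's height and adds a small roll to the rest rotation.
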(event EventTick
  (params (DeltaSeconds :type Float%20%28single-precision%29))
  (bind _returnvalue (Transformation|GetWorldLocation))
  (bind _returnvalue_2 (Components|GetOwner))
  (bind _returnvalue_3 (Transformation|GetActorLocation _returnvalue_2))
  (bind _out (CallFunction|WaveSurge 0.32 (* 32.0 0.008) 35.0 (/ (Math|Vector|MakeVector (.x _returnvalue) (.y _returnvalue) 0.0) (Variables|Default|GetScale))))
  (Transformation|SetActorRotation _returnvalue_2 (Math|Rotator|CombineRotators (Math|Rotator|MakeRotator (* (/ (- 32.0 _out) 32.0) 5.0) 0.0 0.0) (Variables|Default|GetRotation)))
  (Transformation|SetActorLocation _returnvalue_2 (Math|Vector|MakeVector (.x _returnvalue_3) (.y _returnvalue_3) (+ (- 32.0 _out) (Variables|Default|GetHeight))) false false))

(event EventBeginPlay
  (bind _waterplane (Variables|Default|GetWaterPlane))
  (bind _returnvalue (Transformation|GetActorScale3D _waterplane))
  (Variables|Default|SetRotation (Transformation|GetWorldRotation))
  (Variables|Default|SetHeight (.z (Transformation|GetWorldLocation)))
  (Utilities|IsValid _waterplane
    (:Is%20Valid
      (Variables|Default|SetScale (Math|Float|Max(Float) (.x _returnvalue) (.y _returnvalue))))))

(fn WaveSurge
  (params (Speed :type Float%20%28single-precision%29) (Divisor :type Float%20%28single-precision%29) (Height :type Float%20%28single-precision%29) (Location :type Vector))
  (bind _returnvalue (Utilities|Time|GetGameTimeinSeconds))
  (bind _returnvalue_2 (/ Location Divisor))
  (bind _returnvalue_3 (* _returnvalue Speed))
  (return (* (+ (* (+ (Math|Trig|Sin(Degrees) (* (+ (.x _returnvalue_2) _returnvalue_3) 3.6e+02)) 1.0) 0.5) (* (+ (Math|Trig|Sin(Degrees) (* (+ (.y _returnvalue_2) _returnvalue_3) 3.6e+02)) 1.0) 0.5)) Height)))