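; BP_RespawnRay is a respawn light ray effect built from two god ray meshes, a spotlight and a particle component.
; Its construction script pushes two colour parameters into both meshes' materials and sets the spotlight's colour from the second colour.
; It also applies the configurable intensity and cone angle to the spotlight and sets the god ray particles to auto-activate.
; A Niagara initialisation check is left unconnected.
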(fn ConstructionScript
  (bind _spotlight (Variables|Default|GetSpotLight))
  (Rendering|Material|SetVectorParameterValueonMaterials (Variables|Default|GetSM_VFX_GodRay1) "Colour2" (Math|Conversions|ToVector(LinearColor) (Variables|Default|GetColour2)))
  (Rendering|Material|SetVectorParameterValueonMaterials (Variables|Default|GetSM_VFX_GodRay) "Colour1" (Math|Conversions|ToVector(LinearColor) (Variables|Default|GetColour1)))
  (Rendering|Components|Light|SetLightColor _spotlight (Variables|Default|GetColour2) true)
  (Rendering|Components|Light|SetIntensity _spotlight (Variables|Default|GetLightIntensity))
  (Rendering|Lighting|SetOuterConeAngle _spotlight (Variables|Default|GetOuterConeAngle))
  (Components|Activation|SetAutoActivate (Variables|Default|GetPS_Godray) true))