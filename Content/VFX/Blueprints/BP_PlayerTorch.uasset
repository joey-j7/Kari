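; BP_PlayerTorch is a torch light that shows only in the evening and at night, while its Visible flag is set.
; On BeginPlay it caches the game instance and plays a timeline at double speed to animate the point light's intensity, scaled by LightIntensity.
; Day-period events toggle the light and its children, hiding them in the morning and afternoon.
; SetVisible stores the flag and calls UpdatePeriod.
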(event EventBeginPlay
  (bind _asgi_default_game_instance (Utilities|Casting|CastToGI_DefaultGameInstance (Game|GetGameInstance)))
  (Variables|Default|SetGameInstance _asgi_default_game_instance)
  ;[1 0.5057 0] Light Intensity Animation
  (Components|Timeline|SetPlayRate (Variables|Default|GetTorchTimeline) 2.0)
  (bind _light_intensity (Timeline|TorchTimeline Play)
    (:Update
      (Rendering|Components|Light|SetIntensity (Variables|Default|GetPointLight) (* _light_intensity (Variables|Default|GetLightIntensity))))))

(event Collision|EventActorBeginOverlap
  (params (OtherActor :type Actor%20Object%20Reference)))

(event EventTick
  (params (DeltaSeconds :type Float%20%28single-precision%29)))

(event EventOnEvening
  (if (Variables|Default|GetVisible)
    (Rendering|SetVisibility (Variables|Default|GetPointLight) true true)
    (else
      (Rendering|SetVisibility (Variables|Default|GetPointLight) false true))))

(event EventOnNight
  (if (Variables|Default|GetVisible)
    (Rendering|SetVisibility (Variables|Default|GetPointLight) true true)
    (else
      (Rendering|SetVisibility (Variables|Default|GetPointLight) false true))))

(event EventOnMorning
  (Rendering|SetVisibility (Variables|Default|GetPointLight) false true))

(event EventOnAfternoon
  (Rendering|SetVisibility (Variables|Default|GetPointLight) false true))

(fn ConstructionScript)

(fn SetVisible
  (params (Visible :type Boolean))
  (Variables|Default|SetVisible Visible)
  (Class|TimedActor|UpdatePeriod))