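; Cooking fire VFX actor built from four plane fire meshes and a flickering point light.
; The construction script writes random floats into three custom primitive data slots on the fire meshes, presumably to vary their material.
; On BeginPlay, a sped-up timeline drives the light's intensity and horizontal movement, each scaled by a multiplier variable, while its height stays fixed.
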(event EventBeginPlay
  (bind _pointlight (Variables|Default|GetPointLight))
  ;[1 0.422 0] Light Intensity Animation
  (Components|Timeline|SetPlayRate (Variables|Default|GetFireTimeline) 2.0)
  (bind (_direction _light_intensity _lightmovement) (Timeline|FireTimeline Play)
    (:Update
      (Rendering|Components|Light|SetIntensity _pointlight (* _light_intensity (Variables|Default|GetLightIntensity)))
      (Transformation|SetRelativeLocation _pointlight (Math|Vector|MakeVector (.x (* _lightmovement (Variables|Default|GetLightMovementIntensity))) (.y (* _lightmovement (Variables|Default|GetLightMovementIntensity))) 28.0) false false))))

(fn ConstructionScript
  ;[1 0.1378 0] Put random value in primitive data of each fire mesh
  (Variables|Default|SetFireMeshArray (Utilities|Array|MakeArray (Variables|Default|GetSM_PlaneFire1) (Variables|Default|GetSM_PlaneFire2) (Variables|Default|GetSM_PlaneFire3) (Variables|Default|GetSM_PlaneFire4)))
  (Rendering|Material|SetCustomPrimitiveDataFloat (Variables|Default|GetFireMeshArray) 0 (Math|Random|RandomFloat))
  (Rendering|Material|SetCustomPrimitiveDataFloat (Variables|Default|GetFireMeshArray) 1 (Math|Random|RandomFloat))
  (Rendering|Material|SetCustomPrimitiveDataFloat (Variables|Default|GetFireMeshArray) 2 (Math|Random|RandomFloat)))