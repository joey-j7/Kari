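; Brazier VFX actor that shows a fire built from ten plane meshes with an animated point light.
; The construction script writes random floats into three custom primitive data slots on the fire meshes, a way to vary them without separate material instances.
; On BeginPlay, a timeline plays at double rate and drives the light's flicker by scaling its curve with a base intensity variable.
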(event EventBeginPlay
  ;[1 0.5057 0] Light Intensity Animation
  (Components|Timeline|SetPlayRate (Variables|Default|GetCampfireTimeline) 2.0)
  (bind _light_intensity (Timeline|CampfireTimeline Play)
    (:Update
      (Rendering|Components|Light|SetIntensity (Variables|Default|GetPointLight) (* _light_intensity (Variables|Default|GetLightIntensity))))))

(fn ConstructionScript
  ;[1 0.1378 0] Put random value in primitive data of each fire mesh
  (Variables|Default|SetFireMeshArray (Utilities|Array|MakeArray (Variables|Default|GetSM_PlaneFire1) (Variables|Default|GetSM_PlaneFire2) (Variables|Default|GetSM_PlaneFire3) (Variables|Default|GetSM_PlaneFire4) (Variables|Default|GetSM_PlaneFire5) (Variables|Default|GetSM_PlaneFire6) (Variables|Default|GetSM_PlaneFire7) (Variables|Default|GetSM_PlaneFire8) (Variables|Default|GetSM_PlaneFire9) (Variables|Default|GetSM_PlaneFire10)))
  (Rendering|Material|SetCustomPrimitiveDataFloat (Variables|Default|GetFireMeshArray) 0 (Math|Random|RandomFloat))
  (Rendering|Material|SetCustomPrimitiveDataFloat (Variables|Default|GetFireMeshArray) 1 (Math|Random|RandomFloat))
  (Rendering|Material|SetCustomPrimitiveDataFloat (Variables|Default|GetFireMeshArray) 2 (Math|Random|RandomFloat)))