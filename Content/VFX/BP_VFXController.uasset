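; BP_VFXController sets up a post-process scene blur effect when play begins.
; On BeginPlay it casts the player character to BP_Kari and stores it, continuing only if the cast succeeds.
; It then creates and stores a dynamic instance of M_SceneBlur and assigns it as a full-weight blendable in its PostProcess settings.
; Tick and the construction script are empty, and no blur parameters are changed here.
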(event EventBeginPlay
  (bind _asbp_kari (Utilities|Casting|CastToBP_Kari (Game|GetPlayerCharacter 0)))
  (Variables|Default|SetPlayer _asbp_kari)
  (bind _returnvalue (Rendering|Material|CreateDynamicMaterialInstance "/Game/VFX/Materials/M_SceneBlur.M_SceneBlur" "None" :!class /Script/Engine.KismetMaterialLibrary))
  (bind _output_get (Variables|Default|SetSceneBlurMI _returnvalue))
  (Utilities|Struct|SetmembersinPostProcessSettings (Variables|/Script/Engine.PostProcessComponent|GetSettings (Variables|Default|GetPostProcess)) (Utilities|Struct|MakeWeightedBlendables (Utilities|Array|MakeArray (Utilities|Struct|MakeWeightedBlendable 1.0 _output_get)))))

(event EventTick
  (params (DeltaSeconds :type Float%20%28single-precision%29)))

(fn ConstructionScript)