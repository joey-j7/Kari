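; Base player controller that drives point-and-click or touch movement and interaction for the BP_Kari character.
; Holding Click traces the cursor or first touch to the world, sets a waypoint there, and Tick feeds movement input toward it, easing off near arrival.
; A short click with little cursor drift also runs a capsule trace and tries InteractWith on hit actors that have an InteractableComponent.
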(event Custom|StopAutoWalking
  (Variables|Default|SetWalkToTarget false)
  (Default|SetWaypoint (CallFunction|GetCharacter) false "0, 0, 0"))

(event Custom|FollowCursor
  (bind _kari (CallFunction|GetCharacter))
  (bind (_screenposition _returnvalue) (CallFunction|GetCursorScreenLocation))
  (bind (_worldposition _worlddirection _returnvalue_2) (CallFunction|GetCursorWorldLocation _screenposition))
  (bind _returnvalue_3 (* _worlddirection 1e+05))
  (bind _returnvalue_4 (+ _worldposition _returnvalue_3))
  (bind (_position _found) (CallFunction|GetCursorLandscapeLocation _worldposition _returnvalue_4))
  (Utilities|IsValid _kari
    (:Is%20Valid
      (if (Math|Boolean|ANDBoolean (Class|DefaultPlayerController|IsInputEnabled) (< (Class|DefaultPlayer|GetInteractionCharacterID _kari) 0) (Class|DefaultPlayer|IsInputEnabled _kari))
        (if (Variables|Default|GetJustClicked)
          (Variables|Default|SetJustClicked false)
          (Variables|Default|SetCursorStartLocation _screenposition))
        (if (and _returnvalue _returnvalue_2)
          (Variables|Default|SetCursorLastLocation _screenposition)
          (if _found
            (Variables|Default|SetWalkToTarget true)
            (bind _output_get (Variables|Default|SetTargetPoint _position))
            (Default|SetWaypoint (CallFunction|GetCharacter) true _output_get)
            (else
              (CallFunction|StopAutoWalking))))))))

(event EventTick
  (params (DeltaSeconds :type Float%20%28single-precision%29))
  (bind _returnvalue (Pawn|GetControlledPawn))
  (bind _kari (CallFunction|GetCharacter))
  (bind _targetpoint (Variables|Default|GetTargetPoint))
  (bind _returnvalue_2 (Transformation|GetActorLocation _returnvalue))
  (bind _returnvalue_3 (* _targetpoint "1.000000,1.000000, 0"))
  (bind _returnvalue_4 (* _returnvalue_2 "1.000000,1.000000, 0"))
  (bind _returnvalue_5 (Math|Vector|Distance(Vector) _returnvalue_4 _returnvalue_3))
  (bind _returnvalue_6 (Math|Rotator|FindLookatRotation _returnvalue_4 _returnvalue_3))
  (bind _returnvalue_7 (Math|Vector|GetForwardVector _returnvalue_6))
  (bind _returnvalue_8 (* _returnvalue_5 0.005))
  (bind _returnvalue_9 (Math|Float|Clamp(Float) _returnvalue_8))
  (bind _returnvalue_10 (* _returnvalue_7 _returnvalue_9))
  (if (Variables|Default|GetIsClicked)
    (CallFunction|FollowCursor))
  (if (Variables|Default|GetWalkToTarget)
    (if (< _returnvalue_5 2e+01)
      (CallFunction|StopAutoWalking)
      (else
        (Pawn|Input|AddMovementInput _kari _returnvalue_10 1.0 false)
        (Variables|/Script/Kari.DefaultPlayer|SetLastInputMovementDirection _kari _returnvalue_10)))))

(event Input|ActionEvents|InputActionClick
  (params (Key :type Key%20Structure :default "None"))
  (bind _cursorstartlocation (Variables|Default|GetCursorStartLocation))
  (bind _cursorlastlocation (Variables|Default|GetCursorLastLocation))
  (bind (_worldposition _worlddirection _returnvalue) (CallFunction|GetCursorWorldLocation _cursorlastlocation))
  (bind _returnvalue_2 (Math|Vector|Distance2D(Vector) _cursorlastlocation _cursorstartlocation))
  (:Pressed
    (Variables|Default|SetCursorStartTime (Utilities|Time|GetGameTimeinSeconds))
    (Variables|Default|SetJustClicked true)
    (Variables|Default|SetIsClicked true)
    (CallFunction|FollowCursor))
  (:Released
    (Variables|Default|SetIsClicked false)
    (if (<= (- (Utilities|Time|GetGameTimeinSeconds) (Variables|Default|GetCursorStartTime)) 0.5)
      (Development|PrintString (Utilities|String|ToString(Float) _returnvalue_2))
      (if (and (<= _returnvalue_2 5e+01) _returnvalue)
        (CallFunction|GetCursorInteractable _worldposition (+ _worldposition (* _worlddirection 1e+05)) 5e+01)))))

(fn ConstructionScript)

(fn GetCharacter
  (Utilities|IsValid (Variables|Default|GetKari)
    (:Is%20Valid
      (return (Variables|Default|GetKari)))
    (:Is%20Not%20Valid
      (bind _asbp_kari (Utilities|Casting|CastToBP_Kari (Game|GetPlayerCharacter 0)))
      (bind _output_get (Variables|Default|SetKari _asbp_kari))
      (return _output_get))))

(fn GetCursorLandscapeLocation
  (params (Start :type Vector) (End :type Vector))
  (bind _output_get (LocalVariables|SetLocation Start))
  (bind (_outhit _returnvalue) (Collision|LineTraceByChannel _output_get End "TraceTypeQuery1" false (Utilities|Array|MakeArray (CallFunction|GetCharacter)) "None"))
  (if _returnvalue
    (LocalVariables|SetLocation (.impactpoint _outhit))
    (LocalVariables|SetDidFind true)
    (return (LocalVariables|GetLocation) (LocalVariables|GetDidFind))))

(fn GetCursorInteractable
  (params (Start :type Vector) (End :type Vector) (Radius :type Float%20%28single-precision%29))
  (bind _outhits (Class|KismetSystemLibrary|CapsuleTraceMultiforObjects Start End Radius 0.0 (Utilities|Array|MakeArray "ObjectTypeQuery1" "ObjectTypeQuery3" "ObjectTypeQuery2") false (Utilities|Array|MakeArray (CallFunction|GetCharacter)) "None" true))
  (bind _array_element (Utilities|Array|ForEachLoopwithBreak _outhits :!label _label)
    (:LoopBody
      (Utilities|IsValid (Actor|GetComponentbyClass (.hitactor _array_element) "/Script/Kari.InteractableComponent")
        (:Is%20Valid
          (bind _succeeded (Default|Interactwith (CallFunction|GetCharacter) (Actor|GetComponentbyClass (.hitactor _array_element) "/Script/Kari.InteractableComponent")))
          (if _succeeded
            (LocalVariables|SetDidFind true)
            (goto _label Break)))))
    (:Completed
      (return (LocalVariables|GetDidFind)))))

(fn GetCursorWorldLocation
  (params (ScreenPosition :type Vector%202D%20Structure))
  (bind _returnvalue (Game|GetPlayerController 0))
  (bind (_worldposition _worlddirection _returnvalue_2) (Class|GameplayStatics|DeprojectScreentoWorld _returnvalue ScreenPosition))
  (return _worldposition _worlddirection _returnvalue_2))

(fn GetCursorScreenLocation
  (bind (_locationx _locationy _returnvalue) (Game|Player|GetMousePosition))
  (bind (_locationx_2 _locationy_2 _biscurrentlypressed) (Class|PlayerController|GetInputTouchState "Touch1"))
  (if _biscurrentlypressed
    (return (Math|Vector2D|MakeVector2D _locationx_2 _locationy_2) true)
    (else
      (return (Math|Vector2D|MakeVector2D _locationx _locationy) _returnvalue))))