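; World light controller that drives time-of-day lighting, sky and post-processing from the TimeManager date and clock.
; Each tick it calls UpdateLight, publishes light color and intensities to MPC_MaterialVariables, and blends four time-of-day post-process weights through one RGBA curve.
; UpdateWorldSphere writes normalized day time to MPC_Time and colors BP_DefaultSkySphere from sun rotation and moon intensity.
; Mobile overrides intensity scalars; construction sets storm flicker intensity.
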(event EventBeginPlay
  (bind _aspc_default_player_controller (Utilities|Casting|CastToPC_DefaultPlayerController (Game|GetPlayerController 0))
    (:then
      (if (Variables|/Script/Kari.DefaultPlayerController|GetbIsMobile _aspc_default_player_controller)
        (Variables|Default|SetIntensityScalar 0.1)
        (Variables|Default|SetSkyIntensityScalar 5.0)))
    (:CastFailed
      _))
  (bind _returnvalue (Actor|GetActorOfClass "/Game/General/Lighting/BP_DefaultSkySphere.BP_DefaultSkySphere_C"))
  (bind _output_get (Variables|Default|SetSkySphere _returnvalue))
  (Utilities|IsValid _output_get))

(event EventUpdateWorldSphere
  (bind _skysphere (Variables|Default|GetSkySphere))
  (bind _skysphere_2 (Variables|Default|GetSkySphere))
  (bind _skysphere_3 (Variables|Default|GetSkySphere))
  (bind _moonlight (Variables|Default|GetMoonLight))
  (bind _skysphere_4 (Variables|Default|GetSkySphere))
  (bind _skysphere_5 (Variables|Default|GetSkySphere))
  (bind _skysphere_6 (Variables|Default|GetSkySphere))
  (bind _sky_material (Variables|/Game/General/Lighting/BP_DefaultSkySphere.BP_DefaultSkySphere_C|GetSky%20material _skysphere_5))
  (bind _sky_material_2 (Variables|/Game/General/Lighting/BP_DefaultSkySphere.BP_DefaultSkySphere_C|GetSky%20material _skysphere_4))
  (Rendering|Material|SetScalarParameterValue "/Game/General/Materials/MPC_Time.MPC_Time" "Time" (Class|TimeManager|GetNormalizedDayTime (Class|WorldLightController|GetTimeManager)) :!class /Script/Engine.KismetMaterialLibrary)
  (Utilities|IsValid (Variables|Default|GetSkySphere)
    (:Is%20Valid
      (Rendering|Material|SetVectorParameterValue _sky_material "Light direction" (Math|Conversions|ToLinearColor(Vector) (Math|Rotator|GetRotationXVector (Transformation|GetWorldRotation (Variables|Default|GetSunLight)))) :!class /Script/Engine.MaterialInstanceDynamic)
      (Rendering|Material|SetVectorParameterValue _sky_material "Sun color" (Math|Color|Lerp(LinearColor) (Math|Conversions|ToLinearColor(Color) (Variables|/Script/Engine.LightComponentBase|GetLightColor (Variables|Default|GetSunLight))) (Math|Conversions|ToLinearColor(Color) (Variables|/Script/Engine.LightComponentBase|GetLightColor _moonlight)) (Math|Float|Lerp 0.0 1.0 (/ (Variables|/Script/Engine.LightComponentBase|GetIntensity _moonlight) (Math|Curves|GetFloatValue (Variables|Default|GetIntensityCurve) (Math|Vector|DotProduct (Math|Vector|GetForwardVector (Transformation|GetWorldRotation (Variables|Default|GetSunLight))) "0, 0,-1.000000"))))) :!class /Script/Engine.MaterialInstanceDynamic)
      (Variables|/Game/General/Lighting/BP_DefaultSkySphere.BP_DefaultSkySphere_C|SetSun%20height (Variables|Default|GetSkySphere) (Math|Float|MapRangeUnclamped (.Pitch (Math|Rotator|BreakRotator (Transformation|GetWorldRotation (Variables|Default|GetSunLight)))) 0.0 -9e+01 0.0 1.0))
      (Rendering|Material|SetVectorParameterValue _sky_material_2 "Horizon color" (Class|CurveLinearColor|GetClampedLinearColorValue (Variables|/Game/General/Lighting/BP_DefaultSkySphere.BP_DefaultSkySphere_C|GetHorizon%20color%20curve _skysphere) (Variables|/Game/General/Lighting/BP_DefaultSkySphere.BP_DefaultSkySphere_C|GetSun%20height _skysphere)) :!class /Script/Engine.MaterialInstanceDynamic)
      (Rendering|Material|SetVectorParameterValue _sky_material_2 "Zenith color" (Class|CurveLinearColor|GetClampedLinearColorValue (Variables|/Game/General/Lighting/BP_DefaultSkySphere.BP_DefaultSkySphere_C|GetZenith%20color%20curve _skysphere_2) (Variables|/Game/General/Lighting/BP_DefaultSkySphere.BP_DefaultSkySphere_C|GetSun%20height _skysphere_2)) :!class /Script/Engine.MaterialInstanceDynamic)
      (Rendering|Material|SetVectorParameterValue _sky_material_2 "Cloud color" (Class|CurveLinearColor|GetClampedLinearColorValue (Variables|/Game/General/Lighting/BP_DefaultSkySphere.BP_DefaultSkySphere_C|GetCloud%20color%20curve _skysphere_3) (Variables|/Game/General/Lighting/BP_DefaultSkySphere.BP_DefaultSkySphere_C|GetSun%20height _skysphere_3)) :!class /Script/Engine.MaterialInstanceDynamic)
      (Rendering|Material|SetScalarParameterValue _sky_material_2 "Horizon falloff" (Variables|/Game/General/Lighting/BP_DefaultSkySphere.BP_DefaultSkySphere_C|GetHorizon%20Falloff _skysphere_6) :!class /Script/Engine.MaterialInstanceDynamic)
      (Rendering|Material|SetScalarParameterValue _sky_material_2 "Sun height" (Math|Float|SelectFloat (Math|Float|Absolute(Float) (Variables|/Game/General/Lighting/BP_DefaultSkySphere.BP_DefaultSkySphere_C|GetSun%20height _skysphere_6)) 0.0 (< (Variables|/Game/General/Lighting/BP_DefaultSkySphere.BP_DefaultSkySphere_C|GetSun%20height _skysphere_6) 0.0)) :!class /Script/Engine.MaterialInstanceDynamic))))

(event EventTick
  (params (DeltaSeconds :type Float%20%28single-precision%29))
  (bind _returnvalue (Class|WorldLightController|GetTimeManager))
  (bind _returnvalue_2 (Class|TimeManager|GetDate _returnvalue))
  (Class|WorldLightController|UpdateLight (.year _returnvalue_2) (.month _returnvalue_2) (.day _returnvalue_2) (.hour _returnvalue_2) (.minute _returnvalue_2) (.second _returnvalue_2))
  ;[1 1 1] Apply values for use in materials
  (Rendering|Material|SetVectorParameterValue "/Game/Gameplay/Colliders/Events/MPC_MaterialVariables.MPC_MaterialVariables" "WorldLightColor" (Variables|Default|GetCurrentColor) :!class /Script/Engine.KismetMaterialLibrary)
  (Rendering|Material|SetScalarParameterValue "/Game/Gameplay/Colliders/Events/MPC_MaterialVariables.MPC_MaterialVariables" "WorldLightIntensity" (Variables|Default|GetCurrentIntensity) :!class /Script/Engine.KismetMaterialLibrary)
  (Rendering|Material|SetScalarParameterValue "/Game/Gameplay/Colliders/Events/MPC_MaterialVariables.MPC_MaterialVariables" "WorldSkyLightIntensity" (Variables|Default|GetCurrentShadowIntensity) :!class /Script/Engine.KismetMaterialLibrary)
  (CallFunction|UpdatePostProcess))

(fn ConstructionScript
  (Rendering|Material|SetScalarParameterValue "/Game/StormSystem/Materials/MPC_Storm.MPC_Storm" "Light Flicker Intensity" (Variables|Default|GetLightFlickerIntensity) :!class /Script/Engine.KismetMaterialLibrary))

(fn UpdatePostProcess
  (bind _returnvalue (Class|WorldLightController|GetTimeManager))
  (bind _postprocessing (Variables|Default|GetPostProcessing))
  (bind _returnvalue_2 (Class|TimeManager|GetDate _returnvalue))
  (bind _returnvalue_3 (Math|Conversions|ToFloat(Integer) (.hour _returnvalue_2)))
  (bind _returnvalue_4 (Math|Conversions|ToFloat(Integer) (.minute _returnvalue_2)))
  (bind _returnvalue_5 (/ _returnvalue_4 6e+01))
  (bind _returnvalue_6 (+ _returnvalue_3 _returnvalue_5))
  (bind _returnvalue_7 (Math|Curves|GetLinearColorValue _postprocessing _returnvalue_6))
  (Variables|/Script/Engine.PostProcessComponent|SetBlendWeight (Variables|Default|GetMorning) (.r _returnvalue_7))
  (Variables|/Script/Engine.PostProcessComponent|SetBlendWeight (Variables|Default|GetNoon) (.g _returnvalue_7))
  (Variables|/Script/Engine.PostProcessComponent|SetBlendWeight (Variables|Default|GetEvening) (.b _returnvalue_7))
  (Variables|/Script/Engine.PostProcessComponent|SetBlendWeight (Variables|Default|GetNight) (.a _returnvalue_7)))