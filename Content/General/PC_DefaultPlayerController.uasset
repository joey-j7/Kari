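; Default player controller that opens the inventory, quest log and pause menus from input actions or toggle events.
; Each handler stops auto-walking, checks CanContinue, creates its widget and sets InMenu, which a destroy callback clears.
; CanContinue blocks menus and the parent's cursor-follow while a menu is open or OnShrine is set.
; Opening the inventory or quest log also calls its tutorial.
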(event Custom|OnPauseDestroy
  (Variables|Default|SetPauseWidget 0)
  (Variables|Default|SetInMenu false))

(event Custom|OnQuestLogDestroy
  (Variables|Default|SetQuestLogWidget 0)
  (Variables|Default|SetInMenu false))

(event Custom|OnInventoryDestroy
  (Variables|Default|SetInventoryWidget 0)
  (Variables|Default|SetInMenu false))

(event Custom|TogglePause
  (CallFunction|StopAutoWalking)
  (if (CallFunction|CanContinue)
    (Utilities|IsValid (Variables|Default|GetPauseWidget)
      (:Is%20Not%20Valid
        ;[1 1 1] Pauses the game
        (bind _returnvalue (UserInterface|CreateWidget "/Game/UI/Pause/WBP_Pause.WBP_Pause_C" (Game|GetPlayerController 0)))
        (UserInterface|Viewport|AddtoViewport _returnvalue 0)
        (Variables|Default|SetPauseWidget _returnvalue)
        (EventDispatchers|BindEventtoOnDestroy _returnvalue (delegate Custom|OnPauseDestroy))
        (Variables|Default|SetInMenu true)))))

(event Custom|ToggleQuest
  (CallFunction|StopAutoWalking)
  (if (CallFunction|CanContinue)
    (Default|CallQuestTutorial)
    (Utilities|IsValid (Variables|Default|GetQuestLogWidget)
      (:Is%20Not%20Valid
        (bind _returnvalue (UserInterface|CreateWidget "/Game/UI/QuestLog/WBP_QuestLogWidget.WBP_QuestLogWidget_C" (Game|GetPlayerController 0)))
        (UserInterface|Viewport|AddtoViewport _returnvalue 0)
        (bind _output_get (Variables|Default|SetQuestLogWidget _returnvalue))
        (EventDispatchers|BindEventtoOnDestroy _returnvalue (delegate Custom|OnQuestLogDestroy))
        (Variables|Default|SetInMenu true)))))

(event Custom|ToggleBag
  (CallFunction|StopAutoWalking)
  ;[1 1 1] Fixes per-frame overlap
  (if (CallFunction|CanContinue)
    (Default|CallBagTutorial)
    (Utilities|IsValid (Variables|Default|GetInventoryWidget)
      (:Is%20Not%20Valid
        (bind _returnvalue (UserInterface|CreateWidget "/Game/UI/Inventory/WBP_Inventory.WBP_Inventory_C" (Game|GetPlayerController 0)))
        (UserInterface|Viewport|AddtoViewport _returnvalue 0)
        (bind _output_get (Variables|Default|SetInventoryWidget _returnvalue))
        (EventDispatchers|BindEventtoOnDestroy _output_get (delegate Custom|OnInventoryDestroy))
        (Variables|Default|SetInMenu true)))))

(event EventFollowCursor
  (if (CallFunction|CanContinue)
    (|CallParentFunction)))

(event Input|ActionEvents|InputActionPause
  (params (Key :type Key%20Structure :default "None"))
  (:Pressed
    (CallFunction|StopAutoWalking)
    (if (CallFunction|CanContinue)
      (Utilities|IsValid (Variables|Default|GetPauseWidget)
        (:Is%20Not%20Valid
          ;[1 1 1] Pauses the game
          (bind _returnvalue (UserInterface|CreateWidget "/Game/UI/Pause/WBP_Pause.WBP_Pause_C" (Game|GetPlayerController 0)))
          (UserInterface|Viewport|AddtoViewport _returnvalue 0)
          (Variables|Default|SetPauseWidget _returnvalue)
          (EventDispatchers|BindEventtoOnDestroy _returnvalue (delegate Custom|OnPauseDestroy))
          (Variables|Default|SetInMenu true))))))

(event Input|ActionEvents|InputActionQuestLog
  (params (Key :type Key%20Structure :default "None"))
  (:Pressed
    (CallFunction|StopAutoWalking)
    (if (CallFunction|CanContinue)
      (Default|CallQuestTutorial)
      (Utilities|IsValid (Variables|Default|GetQuestLogWidget)
        (:Is%20Not%20Valid
          (bind _returnvalue (UserInterface|CreateWidget "/Game/UI/QuestLog/WBP_QuestLogWidget.WBP_QuestLogWidget_C" (Game|GetPlayerController 0)))
          (UserInterface|Viewport|AddtoViewport _returnvalue 0)
          (bind _output_get (Variables|Default|SetQuestLogWidget _returnvalue))
          (EventDispatchers|BindEventtoOnDestroy _returnvalue (delegate Custom|OnQuestLogDestroy))
          (Variables|Default|SetInMenu true))))))

(event Input|ActionEvents|InputActionToggleInventory
  (params (Key :type Key%20Structure :default "None"))
  (:Pressed
    (CallFunction|StopAutoWalking)
    ;[1 1 1] Fixes per-frame overlap
    (if (CallFunction|CanContinue)
      (Default|CallBagTutorial)
      (Utilities|IsValid (Variables|Default|GetInventoryWidget)
        (:Is%20Not%20Valid
          (bind _returnvalue (UserInterface|CreateWidget "/Game/UI/Inventory/WBP_Inventory.WBP_Inventory_C" (Game|GetPlayerController 0)))
          (UserInterface|Viewport|AddtoViewport _returnvalue 0)
          (bind _output_get (Variables|Default|SetInventoryWidget _returnvalue))
          (EventDispatchers|BindEventtoOnDestroy _output_get (delegate Custom|OnInventoryDestroy))
          (Variables|Default|SetInMenu true))))))

(fn ConstructionScript)

(fn CanContinue
  (return (and (not (Variables|Default|GetOnShrine)) (not (Variables|Default|GetInMenu)))))