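; Default game mode that handles level startup, player state transitions and narrative event responses.
; BeginPlay sets up the blizzard, fade controller and per-level breathing particles; transitions lock input behind screen fades, with death stats and achievements.
; Dialogue, task and time events drive quests, inventory, trading, day/night, storms, saving, character visibility and the ending cutscene.
; Quest and story changes for the character being talked to are queued as pending on its StoryComponent.
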(event OnEnter(AddQuestDialogueEvent)
  (params (DialogueEvent :type Dialogue%20Event%20Structure))
  (bind (_eventname _dialogueid _characterid _value) (Utilities|Struct|BreakDialogueEvent DialogueEvent))
  ;[1 1 1] Dialogue Events
  (bind _asbp_kari (Utilities|Casting|CastToBP_Kari (Game|GetPlayerCharacter 0)))
  (if (== (Class|DefaultPlayer|GetInteractionCharacterID _asbp_kari) _characterid)
    (bind _outactors (Actor|GetAllActorsOfClass "/Script/Kari.DefaultCharacter"))
    (for _array_element _outactors
      (Utilities|IsValid (Actor|GetComponentbyClass _array_element "/Script/Kari.CharacterComponent")
        (:Is%20Valid
          (if (== (Class|TableComponent|TableID (Actor|GetComponentbyClass _array_element "/Script/Kari.CharacterComponent")) _characterid)
            (Utilities|IsValid (Actor|GetComponentbyClass _array_element "/Script/Kari.StoryComponent")
              (:Is%20Valid
                (Class|StoryComponent|AddPendingQuestID (Actor|GetComponentbyClass _array_element "/Script/Kari.StoryComponent") _value)))))))
    (else
      (bind _asdefault_game_instance (Utilities|Casting|CastToDefaultGameInstance (Game|GetGameInstance)))
      (Class|QuestLog|AddQuest (Variables|/Script/Kari.DefaultGameInstance|GetQuestLog _asdefault_game_instance) _value _characterid))))

(event OnEnter(CompleteTaskDialogueEvent)
  (params (DialogueEvent :type Dialogue%20Event%20Structure))
  ;[1 1 1] Dialogue Events
  (bind _asdefault_game_instance (Utilities|Casting|CastToDefaultGameInstance (Game|GetGameInstance)))
  (Class|QuestLog|CompleteTask (Variables|/Script/Kari.DefaultGameInstance|GetQuestLog _asdefault_game_instance) (.Value (Utilities|Struct|BreakDialogueEvent DialogueEvent))))

(event OnEnter(RemoveItemDialogueEvent)
  (params (DialogueEvent :type Dialogue%20Event%20Structure))
  (bind (_eventname _dialogueid _characterid _value _secondaryvalue) (Utilities|Struct|BreakDialogueEvent DialogueEvent))
  ;[1 1 1] Dialogue Events
  (bind _asdefault_game_instance (Utilities|Casting|CastToDefaultGameInstance (Game|GetGameInstance)))
  (Class|Inventory|RemoveItemsbyType (Variables|/Script/Kari.DefaultGameInstance|GetInventory _asdefault_game_instance) _value _secondaryvalue))

(event OnEnter(FreezeTaskDialogueEvent)
  (params (DialogueEvent :type Dialogue%20Event%20Structure))
  ;[1 1 1] Dialogue Events
  (Class|QuestLog|FreezeTask (Variables|/Script/Kari.DefaultGameInstance|GetQuestLog (Variables|Default|GetGameInstance)) (.Value (Utilities|Struct|BreakDialogueEvent DialogueEvent))))

(event OnEnter(HideCharacterTimeEvent)
  (params (TimeEvent :type Time%20Event%20Structure))
  ;[1 1 1] Time Events
  (bind _outactors (Actor|GetAllActorsOfClass "/Script/Kari.DefaultCharacter"))
  (for _array_element _outactors
    (Utilities|IsValid (Actor|GetComponentbyClass _array_element "/Script/Kari.CharacterComponent")
      (:Is%20Valid
        (if (== (Class|TableComponent|TableID (Actor|GetComponentbyClass _array_element "/Script/Kari.CharacterComponent")) (.characterid TimeEvent))
          (Class|DefaultCharacter|HideOffScreen _array_element))))))

(event OnEnter(ShowCharacterTimeEvent)
  (params (TimeEvent :type Time%20Event%20Structure))
  ;[1 1 1] Time Events
  (bind _outactors (Actor|GetAllActorsOfClass "/Script/Kari.DefaultCharacter"))
  (for _array_element _outactors
    (Utilities|IsValid (Actor|GetComponentbyClass _array_element "/Script/Kari.CharacterComponent")
      (:Is%20Valid
        (if (== (Class|TableComponent|TableID (Actor|GetComponentbyClass _array_element "/Script/Kari.CharacterComponent")) (.characterid TimeEvent))
          (Class|DefaultCharacter|ShowOffScreen _array_element))))))

(event OnEnter(AddTabDialogueEvent)
  (params (DialogueEvent :type Dialogue%20Event%20Structure))
  ;[1 1 1] Dialogue Events
  (bind _asdefault_game_instance (Utilities|Casting|CastToDefaultGameInstance (Game|GetGameInstance)))
  (Class|Inventory|AddTab (Variables|/Script/Kari.DefaultGameInstance|GetInventory _asdefault_game_instance) (.Value (Utilities|Struct|BreakDialogueEvent DialogueEvent))))

(event OnExit(ActivateStormDialogueEvent)
  (params (DialogueEvent :type Dialogue%20Event%20Structure))
  ;[1 1 1] Task Events
  (bind _returnvalue (Actor|GetActorOfClass "/Game/StormSystem/BP_BlizzardSystem.BP_BlizzardSystem_C"))
  (Utilities|IsValid _returnvalue
    (:Is%20Valid
      (if (== (.value DialogueEvent) 1)
        (Default|ApplyStormState _returnvalue)
        (else
          (Default|RevertStormState _returnvalue))))))

(event OnEnter(FreezeTaskTaskEvent)
  (params (TaskEvent :type Task%20Event%20Structure))
  ;[1 1 1] Task Events
  (Class|QuestLog|FreezeTask (Variables|/Script/Kari.DefaultGameInstance|GetQuestLog (Variables|Default|GetGameInstance)) (.Value (Utilities|Struct|BreakTaskEvent TaskEvent))))

(event OnEnter(SaveGameDialogueEvent)
  (params (DialogueEvent :type Dialogue%20Event%20Structure))
  ;[1 1 1] Dialogue Events
  (Class|SaveLibrary|SaveGame)
  (bind _foundwidgets (Widget|GetAllWidgetsOfClass "/Game/UI/Gameplay/WBP_SavingIcon.WBP_SavingIcon_C" true))
  (Default|ShowSavingIcon (Utilities|Array|Get(acopy) _foundwidgets)))

(event OnExit(PlayEndingDialogueEvent)
  (params (DialogueEvent :type Dialogue%20Event%20Structure))
  (bind _gameinstance (Variables|Default|GetGameInstance))
  (bind _audiomanager (Variables|/Script/Kari.DefaultGameInstance|GetAudioManager _gameinstance))
  (bind _returnvalue (Class|AudioManager|GetOverrideBGM _audiomanager))
  ;[1 1 1] Dialogue Events
  (bind _returnvalue_2 (Actor|GetActorOfClass "/Game/General/BP_FadeController.BP_FadeController_C"))
  (Class|FadeController|ScreenFadeOut _returnvalue_2 0.0)
  (Utilities|FlowControl|Sequence
    (:then_0
      (Utilities|IsValid _returnvalue
        (:Is%20Valid
          (Class|BPFLBaseDefaultFunctionLibrary|FadeAudio _returnvalue (Variables|/Script/Kari.FadeController|GetFadeSpeed _returnvalue_2)))))
    (:then_1
      (EventDispatchers|BindEventtoOnScreenFaded _returnvalue_2 (delegate Custom|OnEndingScreenFaded)))))

(event OnEnter(CurrentCharacterRevisionTaskEvent)
  (params (TaskEvent :type Task%20Event%20Structure))
  (bind (_eventname _taskid _characterid _value) (Utilities|Struct|BreakTaskEvent TaskEvent))
  ;[1 1 1] Task Events
  (bind _asbp_kari (Utilities|Casting|CastToBP_Kari (Game|GetPlayerCharacter 0)))
  (bind _asdefault_game_instance (Utilities|Casting|CastToDefaultGameInstance (Game|GetGameInstance)))
  (if (== (Class|DefaultPlayer|GetInteractionCharacterID _asbp_kari) _characterid)
    (bind _outactors (Actor|GetAllActorsOfClass "/Script/Kari.DefaultCharacter"))
    (for _array_element _outactors
      (Utilities|IsValid (Actor|GetComponentbyClass _array_element "/Script/Kari.CharacterComponent")
        (:Is%20Valid
          (if (== (Class|TableComponent|TableID (Actor|GetComponentbyClass _array_element "/Script/Kari.CharacterComponent")) _characterid)
            (Utilities|IsValid (Actor|GetComponentbyClass _array_element "/Script/Kari.StoryComponent")
              (:Is%20Valid
                (Class|QuestLog|AddRevisionIDChangetoTask (Variables|/Script/Kari.DefaultGameInstance|GetQuestLog _asdefault_game_instance) _taskid _characterid (.storyid (.revision (Class|Revisioning|GetCharacterRevision (Variables|/Script/Kari.DefaultGameInstance|GetRevisioning _asdefault_game_instance) _characterid))))
                (Class|StoryComponent|SetPendingStoryID (Actor|GetComponentbyClass _array_element "/Script/Kari.StoryComponent") _value)
                (bind _returnvalue (Class|TableBPFunctions|GetTableString "characters" "name" _characterid))
                (bind _returnvalue_2 (Class|TableBPFunctions|GetTableString "stories" "title" _value))
                (Development|PrintString (Utilities|String|Append _returnvalue "'s story is pending to be set to " _returnvalue_2 " after dialogue"))))))))
    (else
      (Class|QuestLog|AddRevisionIDChangetoTask (Variables|/Script/Kari.DefaultGameInstance|GetQuestLog _asdefault_game_instance) _taskid _characterid (.storyid (.revision (Class|Revisioning|GetCharacterRevision (Variables|/Script/Kari.DefaultGameInstance|GetRevisioning _asdefault_game_instance) _characterid))))
      (Class|Revisioning|SetCharacterRevision (Variables|/Script/Kari.DefaultGameInstance|GetRevisioning _asdefault_game_instance) _characterid (Utilities|Struct|MakeCharacterRevision _value false "0.000000,0.000000,0.000000" "0.000000,0.000000,0.000000" false))
      (bind _returnvalue_3 (Class|TableBPFunctions|GetTableString "characters" "name" _characterid))
      (bind _returnvalue_4 (Class|TableBPFunctions|GetTableString "stories" "title" _value))
      (Development|PrintString (Utilities|String|Append _returnvalue_3 "'s story has been set to " _returnvalue_4)))))

(event OnEnter(CompleteQuestDialogueEvent)
  (params (DialogueEvent :type Dialogue%20Event%20Structure))
  ;[1 1 1] Dialogue Events
  (bind _asdefault_game_instance (Utilities|Casting|CastToDefaultGameInstance (Game|GetGameInstance)))
  (Class|QuestLog|CompleteQuest (Variables|/Script/Kari.DefaultGameInstance|GetQuestLog _asdefault_game_instance) (.Value (Utilities|Struct|BreakDialogueEvent DialogueEvent))))

(event OnEnter(AddItemDialogueEvent)
  (params (DialogueEvent :type Dialogue%20Event%20Structure))
  (bind (_eventname _dialogueid _characterid _value _secondaryvalue) (Utilities|Struct|BreakDialogueEvent DialogueEvent))
  ;[1 1 1] Dialogue Events
  (bind _asdefault_game_instance (Utilities|Casting|CastToDefaultGameInstance (Game|GetGameInstance)))
  (bind _returnvalue (Class|Inventory|AddItemsbyType (Variables|/Script/Kari.DefaultGameInstance|GetInventory _asdefault_game_instance) _value _secondaryvalue true))
  (if _returnvalue
    (bind _returnvalue_2 (Class|DefaultGameInstance|GetHUDLog _asdefault_game_instance))
    (Class|ActionLogWidget|AddMessage _returnvalue_2 _value "Item added to the pouch" "E_NONE" 1 3.0)
    (else
      (bind _returnvalue_3 (Class|DefaultGameInstance|GetHUDLog _asdefault_game_instance))
      (Class|ActionLogWidget|AddMessage _returnvalue_3 _value "Item couldn't be added to your bag" "E_ITEM_ADD" 1 3.0))))

(event OnClick(ChangeCycleDialogueOptionEvent)
  (params (DialogueOptionEvent :type Dialogue%20Option%20Event%20Structure))
  ;[1 1 1] Dialogue Option Events
  (Variables|Default|SetDayNightOption (Math|Conversions|ToBoolean(Integer) (.Value (Utilities|Struct|BreakDialogueOptionEvent DialogueOptionEvent)))))

(event OnClick(OpenCraftMenuDialogueOptionEvent)
  (params (DialogueOptionEvent :type Dialogue%20Option%20Event%20Structure))
  (bind (_eventname _dialogueoptionid _characterid _value) (Utilities|Struct|BreakDialogueOptionEvent DialogueOptionEvent))
  ;[1 1 1] Dialogue Option Events
  (bind _outactors (Actor|GetAllActorsOfClass "/Game/Characters/Villagers/BP_Trader.BP_Trader_C"))
  (bind _array_element (Utilities|Array|ForEachLoopwithBreak _outactors :!label _label)
    (:LoopBody
      (if (== (Class|TableComponent|TableID (Variables|/Script/Kari.DefaultNPC|GetCharacterComponent _array_element)) _characterid)
        (Class|DefaultCraftingComponent|SetNextDialogueId (Variables|/Script/Kari.DefaultMerchant|GetTradeComponent _array_element) _value)
        (Class|ICraftable|ShowMenu (Variables|/Script/Kari.DefaultMerchant|GetTradeComponent _array_element))
        (goto _label Break)))))

(event OnClick(FreezeTaskDialogueOptionEvent)
  (params (DialogueOptionEvent :type Dialogue%20Option%20Event%20Structure))
  ;[1 1 1] Dialogue Option Events
  (Class|QuestLog|FreezeTask (Variables|/Script/Kari.DefaultGameInstance|GetQuestLog (Variables|Default|GetGameInstance)) (.Value (Utilities|Struct|BreakDialogueOptionEvent DialogueOptionEvent))))

(event OnExit(ChangeCycleDialogueEvent)
  (params (DialogueEvent :type Dialogue%20Event%20Structure))
  (bind _fadecontroller (Variables|Default|GetFadeController))
  ;[1 1 1] Dialogue Events
  (Utilities|FlowControl|Sequence
    (:then_0
      (Class|KariGameModeBase|OnExit DialogueEvent)
      (Class|FadeController|ScreenFadeOut _fadecontroller 0.0)
      (EventDispatchers|BindEventtoOnScreenFaded _fadecontroller (delegate Custom|OnFaded%20Event)))
    (:then_1
      (CallFunction|Achievement 0 0 -1 false (.CharacterID (Utilities|Struct|BreakDialogueEvent DialogueEvent))))))

(event OnEnter(CurrentCharacterRevisionDialogueEvent)
  (params (DialogueEvent :type Dialogue%20Event%20Structure))
  (bind (_eventname _dialogueid _characterid _value) (Utilities|Struct|BreakDialogueEvent DialogueEvent))
  ;[1 1 1] Dialogue Events
  (bind _asdefault_game_instance (Utilities|Casting|CastToDefaultGameInstance (Game|GetGameInstance)))
  (bind _asbp_kari (Utilities|Casting|CastToBP_Kari (Game|GetPlayerCharacter 0)))
  (if (== (Class|DefaultPlayer|GetInteractionCharacterID _asbp_kari) _characterid)
    (bind _outactors (Actor|GetAllActorsOfClass "/Script/Kari.DefaultCharacter"))
    (for _array_element _outactors
      (Utilities|IsValid (Actor|GetComponentbyClass _array_element "/Script/Kari.CharacterComponent")
        (:Is%20Valid
          (if (== (Class|TableComponent|TableID (Actor|GetComponentbyClass _array_element "/Script/Kari.CharacterComponent")) _characterid)
            (Utilities|IsValid (Actor|GetComponentbyClass _array_element "/Script/Kari.StoryComponent")
              (:Is%20Valid
                (Class|StoryComponent|SetPendingStoryID (Actor|GetComponentbyClass _array_element "/Script/Kari.StoryComponent") _value)))))))
    (else
      (Class|Revisioning|SetCharacterRevision (Variables|/Script/Kari.DefaultGameInstance|GetRevisioning _asdefault_game_instance) _characterid (Utilities|Struct|MakeCharacterRevision _value false "0.000000,0.000000,0.000000" "0.000000,0.000000,0.000000" false))
      (bind _returnvalue (Class|TableBPFunctions|GetTableString "characters" "name" _characterid))
      (bind _returnvalue_2 (Class|TableBPFunctions|GetTableString "stories" "title" _value))
      (Development|PrintString (Utilities|String|Append _returnvalue "'s story has been set to " _returnvalue_2))
      (Development|PrintString _eventname))))

(event Custom|OnEndingScreenFaded
  ;[1 1 1] Dialogue Events
  (bind _asgi_default_game_instance (Utilities|Casting|CastToGI_DefaultGameInstance (Game|GetGameInstance)))
  (Variables|/Script/Kari.DefaultGameInstance|SetIsStormActive _asgi_default_game_instance false)
  (Utilities|FlowControl|Sequence
    (:then_0
      (Utilities|IsValid (Class|AudioManager|GetOverrideBGM (Variables|/Script/Kari.DefaultGameInstance|GetAudioManager _asgi_default_game_instance))
        (:Is%20Valid
          (Class|AudioManager|StopBGM (Variables|/Script/Kari.DefaultGameInstance|GetAudioManager _asgi_default_game_instance))
          (Class|AudioManager|SetOverrideBGM (Variables|/Script/Kari.DefaultGameInstance|GetAudioManager _asgi_default_game_instance)))))
    (:then_1
      (Class|AudioManager|CleanupBGMs (Variables|/Script/Kari.DefaultGameInstance|GetAudioManager _asgi_default_game_instance))
      (Game|OpenLevel(byName) "/Game/Levels/Saerkyn/Cutscene/L_EndingCutscene"))))

(event Custom|EnablePlayerInput
  (Input|EnableInput (Game|GetPlayerCharacter 0) 0)
  (Input|EnableInput (Game|GetPlayerController 0) 0))

(event Custom|OnFaded%20Event
  (bind _fadecontroller (Variables|Default|GetFadeController))
  (bind _gameinstance (Variables|Default|GetGameInstance))
  (bind _timemanager (Variables|/Script/Kari.DefaultGameInstance|GetTimeManager _gameinstance))
  ;[1 1 1] Dialogue Events
  (if (== (.Value (Utilities|Struct|BreakDialogueEvent (Variables|Default|GetDialogueEvent))) 0)
    (Class|TimeManager|ToggleTimeOfDay _timemanager "E_MORNING")
    (else
      (Class|TimeManager|ToggleTimeOfDay _timemanager "E_NIGHT")))
  (Class|FadeController|ScreenFadein _fadecontroller 1.5)
  (EventDispatchers|BindEventtoOnScreenClear _fadecontroller (delegate Custom|EnablePlayerInput)))

(event EventBeginPlay
  ;[1 1 1] steam bs
  (bind _returnvalue (Class|SteamUErBPLibrary|SteamUErIsSteamConnected))
  (if _returnvalue
    (bind _returnvalue_2 (Class|SteamUErBPLibrary|SteamUErRequestGlobalStats 1))
    (if _returnvalue_2
      _
      (else
        _)))
  (Utilities|FlowControl|Sequence
    (:then_0
      (bind _asgi_default_game_instance (Utilities|Casting|CastToGI_DefaultGameInstance (Game|GetGameInstance)))
      (if (Variables|/Script/Kari.DefaultGameInstance|GetIsStormActive _asgi_default_game_instance)
        (bind _returnvalue_3 (Actor|GetActorOfClass "/Game/StormSystem/BP_BlizzardSystem.BP_BlizzardSystem_C"))
        (Utilities|IsValid _returnvalue_3
          (:Is%20Not%20Valid
            (Game|SpawnActorfromClass "/Game/StormSystem/BP_BlizzardSystem.BP_BlizzardSystem_C" (Math|Transform|MakeTransform "0, 0, 0" "0, 0, 0" "1,1,1") "Undefined" 0 0)))))
    (:then_1
      (bind _returnvalue_4 (Actor|GetActorOfClass "/Game/General/BP_FadeController.BP_FadeController_C"))
      (bind _output_get (Variables|Default|SetFadeController _returnvalue_4))
      (Utilities|IsValid _output_get
        (:Is%20Valid
          _)
        (:Is%20Not%20Valid
          (bind _returnvalue_5 (Game|SpawnActorfromClass "/Game/General/BP_FadeController.BP_FadeController_C" (Math|Transform|MakeTransform "0, 0, 0" "0, 0, 0" "1,1,1") "Undefined" 0 0))
          (Variables|Default|SetFadeController _returnvalue_5)))
      (bind _returnvalue_6 (Game|GetCurrentLevelName true))
      (if (or (Utilities|Enum|Equal(Enum) _returnvalue_6 "L_Battlefield") (Utilities|Enum|Equal(Enum) _returnvalue_6 "L_Mountain"))
        (bind _returnvalue_7 (Class|NiagaraFunctionLibrary|GetNiagaraParameterCollection "/Game/VFX/ParticleSystems/NPC_Breathing.NPC_Breathing"))
        (Effects|Components|ParticleSystem|SetIntParameter _returnvalue_7 "SpawnCount" 2)
        (else
          (bind _returnvalue_8 (Class|NiagaraFunctionLibrary|GetNiagaraParameterCollection "/Game/VFX/ParticleSystems/NPC_Breathing.NPC_Breathing"))
          (Effects|Components|ParticleSystem|SetIntParameter _returnvalue_8 "SpawnCount" 0))))))

(event EventOnTraversal
  (bind _fadecontroller (Variables|Default|GetFadeController))
  (CallFunction|Achievement 0 0 -1 true -1)
  (|CallParentFunction)
  (Development|PrintString "On Traversal")
  (Input|DisableInput (Game|GetPlayerCharacter 0) 0)
  (Input|DisableInput (Game|GetPlayerController 0) 0)
  (Class|FadeController|SetScreenFade _fadecontroller 1.0)
  (Class|FadeController|ScreenFadein _fadecontroller 1.5)
  (EventDispatchers|AssignOnScreenClear (Variables|Default|GetFadeController) (delegate Custom|EnablePlayerInput)))

(event EventOnLoading
  (bind _fadecontroller (Variables|Default|GetFadeController))
  (|CallParentFunction)
  (Development|PrintString "On Loading")
  (Input|DisableInput (Game|GetPlayerCharacter 0) 0)
  (Input|DisableInput (Game|GetPlayerController 0) 0)
  (Class|FadeController|SetScreenFade _fadecontroller 1.0)
  (Class|FadeController|ScreenFadein _fadecontroller 1.5)
  (EventDispatchers|AssignOnScreenClear (Variables|Default|GetFadeController) (delegate Custom|EnablePlayerInput)))

(event EventOnRespawning
  (bind _fadecontroller (Variables|Default|GetFadeController))
  (CallFunction|UpdateStat "DEATH" 1 false true)
  (CallFunction|Unlock "ACH_DEATH_RESPAWN")
  (|CallParentFunction)
  (Input|DisableInput (Game|GetPlayerCharacter 0) 0)
  (Input|DisableInput (Game|GetPlayerController 0) 0)
  (Development|PrintString "On Respawning")
  (Class|FadeController|SetScreenFade _fadecontroller 1.0)
  (Class|FadeController|ScreenFadein _fadecontroller 1.5))

(event EventOnNewGame
  (bind _fadecontroller (Variables|Default|GetFadeController))
  (CallFunction|UpdateStat "DEATH" 0 false true)
  (|CallParentFunction)
  (Development|PrintString "On New Game")
  (Input|DisableInput (Game|GetPlayerCharacter 0) 0)
  (Input|DisableInput (Game|GetPlayerController 0) 0)
  (Class|FadeController|SetScreenFade _fadecontroller 1.0)
  (Class|FadeController|ScreenFadein _fadecontroller 1.5)
  (EventDispatchers|AssignOnScreenClear (Variables|Default|GetFadeController) (delegate Custom|EnablePlayerInput)))

(fn ConstructionScript)