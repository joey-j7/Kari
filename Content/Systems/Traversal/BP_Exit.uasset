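; BP_Exit is a level exit trigger that moves the player to a named entrance in another level.
; When BP_Kari's capsule overlaps its bound box, it starts a screen fade-out through BP_FadeController and fades the current BGM at that controller's speed.
; Once the screen has faded, it stops the music, cleans up BGMs via the game instance's AudioManager and calls Traverse.
; An override BGM is exempt from the fade and stop.
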(event OnComponentBeginOverlap(BoundBox)
  (params (OverlappedComponent :type Primitive%20Component%20Object%20Reference) (OtherActor :type Actor%20Object%20Reference) (OtherComp :type Primitive%20Component%20Object%20Reference) (OtherBodyIndex :type Integer) (bFromSweep :type Boolean) (SweepResult :type Hit%20Result%20Structure%20%28by%20ref%29))
  (bind _asbp_kari (Utilities|Casting|CastToBP_Kari OtherActor))
  (if (== (Variables|/Script/Engine.Character|GetCapsuleComponent _asbp_kari) OtherComp)
    (bind _asgi_default_game_instance (Utilities|Casting|CastToGI_DefaultGameInstance (Game|GetGameInstance)))
    (bind _returnvalue (Actor|GetActorOfClass "/Game/General/BP_FadeController.BP_FadeController_C"))
    (Class|FadeController|ScreenFadeOut _returnvalue 0.0)
    (Utilities|FlowControl|Sequence
      (:then_0
        (Utilities|IsValid (Class|AudioManager|GetBGM (Variables|/Script/Kari.DefaultGameInstance|GetAudioManager _asgi_default_game_instance))
          (:Is%20Valid
            (if (not (== (Class|AudioManager|GetBGM (Variables|/Script/Kari.DefaultGameInstance|GetAudioManager _asgi_default_game_instance)) (Class|AudioManager|GetOverrideBGM (Variables|/Script/Kari.DefaultGameInstance|GetAudioManager _asgi_default_game_instance))))
              (Class|BPFLBaseDefaultFunctionLibrary|FadeAudio (Class|AudioManager|GetBGM (Variables|/Script/Kari.DefaultGameInstance|GetAudioManager _asgi_default_game_instance)) (Variables|/Script/Kari.FadeController|GetFadeSpeed _returnvalue))))))
      (:then_1
        (EventDispatchers|BindEventtoOnScreenFaded _returnvalue (delegate Custom|OnExit))))))

(event Custom|OnExit
  (bind _asgi_default_game_instance (Utilities|Casting|CastToGI_DefaultGameInstance (Game|GetGameInstance)))
  (Utilities|FlowControl|Sequence
    (:then_0
      (Utilities|IsValid (Class|AudioManager|GetBGM (Variables|/Script/Kari.DefaultGameInstance|GetAudioManager _asgi_default_game_instance))
        (:Is%20Valid
          (if (not (== (Class|AudioManager|GetBGM (Variables|/Script/Kari.DefaultGameInstance|GetAudioManager _asgi_default_game_instance)) (Class|AudioManager|GetOverrideBGM (Variables|/Script/Kari.DefaultGameInstance|GetAudioManager _asgi_default_game_instance))))
            (Class|AudioManager|StopBGM (Variables|/Script/Kari.DefaultGameInstance|GetAudioManager _asgi_default_game_instance))))))
    (:then_1
      (Class|AudioManager|CleanupBGMs (Variables|/Script/Kari.DefaultGameInstance|GetAudioManager _asgi_default_game_instance))
      (Class|SaveLibrary|Traverse (Variables|Default|GetLevelName) (Variables|Default|GetExitName) (Variables|Default|GetFadeAudio)))))

(event EventBeginPlay
  (Actor|GetActorOfClass "/Game/General/BP_FadeController.BP_FadeController_C"))

(fn ConstructionScript)