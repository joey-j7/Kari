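; Steam achievement handler that unlocks achievements for level discovery, eaten items and items crafted in Saerkyn, and tracks shrine and inn visit stats.
; Achievement routes inputs to per-category checks, which match IDs through UnlockIf into a connection-checked Unlock.
; InteractedWith ORs visits into bitmask stats via UpdateStat, then stores the set-bit count.
; TalkToAchievement's NPC and inn logic is disconnected from its entry, so never runs.
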(fn ConsumeAchievement
  (params (Item%20ID :type Integer))
  (Utilities|FlowControl|Sequence
    (:then_0
      (bind _status (Steam|Unlockif Item%20ID "(TableName=\"items\",ColumnName=\"name\",ID=51)" "ACH_LITTLE_SNACK"))
      (CallFunction|UnlockPrint _status))
    (:then_1
      (Steam|Unlockif Item%20ID "(TableName=\"items\",ColumnName=\"name\",ID=36)" "ACH_RUNE"))
    (:then_2
      (Steam|Unlockif Item%20ID "(TableName=\"items\",ColumnName=\"name\",ID=37)" "ACH_RUNE"))
    (:then_3
      (Steam|Unlockif Item%20ID "(TableName=\"items\",ColumnName=\"name\",ID=38)" "ACH_RUNE"))
    (:then_4
      (Steam|Unlockif Item%20ID "(TableName=\"items\",ColumnName=\"name\",ID=40)" "ACH_RUNE"))
    (:then_5
      (Steam|Unlockif Item%20ID "(TableName=\"items\",ColumnName=\"name\",ID=41)" "ACH_RUNE"))
    (:then_6
      (Steam|Unlockif Item%20ID "(TableName=\"items\",ColumnName=\"name\",ID=42)" "ACH_RUNE"))
    (:then_7
      (Steam|Unlockif Item%20ID "(TableName=\"items\",ColumnName=\"name\",ID=43)" "ACH_RUNE"))
    (:then_8
      (Steam|Unlockif Item%20ID "(TableName=\"items\",ColumnName=\"name\",ID=44)" "ACH_RUNE"))
    (:then_9
      (Steam|Unlockif Item%20ID "(TableName=\"items\",ColumnName=\"name\",ID=45)" "ACH_RUNE"))
    (:then_10
      (Steam|Unlockif Item%20ID "(TableName=\"items\",ColumnName=\"name\",ID=46)" "ACH_RUNE"))
    (:then_11
      (Steam|Unlockif Item%20ID "(TableName=\"items\",ColumnName=\"name\",ID=47)" "ACH_RUNE"))
    (:then_12
      (Steam|Unlockif Item%20ID "(TableName=\"items\",ColumnName=\"name\",ID=48)" "ACH_RUNE"))
    (:then_13
      (Steam|Unlockif Item%20ID "(TableName=\"items\",ColumnName=\"name\",ID=49)" "ACH_RUNE"))
    (:then_14
      (Steam|Unlockif Item%20ID "(TableName=\"items\",ColumnName=\"name\",ID=39)" "ACH_RUNE"))
    (:then_15
      (bind _status_2 (Steam|Unlockif Item%20ID "(TableName=\"items\",ColumnName=\"name\",ID=28)" "ACH_EYE_ODIN"))
      (CallFunction|UnlockPrint _status_2))))

(fn Unlock
  (params (Achievement :type String))
  (bind _returnvalue (CallFunction|SteamUErIsSteamConnected))
  (if _returnvalue
    (bind _returnvalue_2 (CallFunction|SteamUErGetAchievement Achievement))
    (if _returnvalue_2
      (Development|PrintString 0 "Player has achivemnt already")
      (return false)
      (else
        (bind _returnvalue_3 (CallFunction|SteamUErSetAchievement Achievement))
        (return _returnvalue_3)))
    (else
      (Development|PrintString 0 "Not connected to steam")
      (return false))))

(fn TalktoAchievement
  (params (NPC%20ID :type Integer) (InnCheck :type Boolean)))

(fn Unlockif
  (params (ID :type Integer) (DatabaseEntry :type Database%20ID%20Pin%20Structure) (Achievement :type String))
  (if (== ID (Class|DatabaseIDFunctionLibrary|GetDatabaseID DatabaseEntry))
    (bind _status (Steam|Unlock Achievement))
    (return _status)
    (else
      (return false))))

(fn Achievement
  (params (CharacterComp :type Character%20Component%20Object%20Reference) (Item :type BP%20Item%20Base%20Object%20Reference) (CraftItemID :type Integer) (CheckLevelName :type Boolean) (CharID :type Integer))
  (if CheckLevelName
    (Achievements|DiscoveredLevelAchievement)
    (else
      ;[1 1 1] inn achivment
      (if (!= CharID -1)
        (Achievements|TalktoAchievement CharID true)
        (Development|PrintString 0 "inn talk")
        (else
          (Utilities|IsValid CharacterComp
            (:Is%20Valid
              ;[1 1 1] talk to
              (Achievements|TalktoAchievement (Class|TableComponent|TableID CharacterComp) false))
            (:Is%20Not%20Valid
              (Utilities|IsValid Item
                (:Is%20Valid
                  ;[1 1 1] consume
                  (bind _returnvalue (Class|ItemBase|GetID Item))
                  (Achievements|ConsumeAchievement _returnvalue))
                (:Is%20Not%20Valid
                  (if (!= CraftItemID -1)
                    (Achievements|CraftItemAchievement CraftItemID)
                    (Development|PrintString 0 "carfted item")))))))))))

(fn UnlockPrint
  (params (In :type Boolean))
  (if In
    (Development|PrintString 0 "Unlock!")
    (return true)
    (else
      (Development|PrintString 0 "Failed Unlock!")
      (return false))))

(fn CraftItemAchievement
  (params (Crafted%20Item%20ID :type Integer))
  (bind _returnvalue (Game|GetCurrentLevelName 0))
  (if (Utilities|Enum|Equal(Enum) _returnvalue "L_Saerkyn")
    (bind _status (Steam|Unlockif Crafted%20Item%20ID "(TableName=\"items\",ColumnName=\"name\",ID=23)" "ACH_SEARKYN_VILLAGE"))
    (CallFunction|UnlockPrint _status)
    (else
      (Development|PrintString 0 "Noooo"))))

(fn DiscoveredLevelAchievement
  (bind _returnvalue (Game|GetCurrentLevelName 0))
  (switch string _returnvalue
    (:L_Mountain
      (Steam|Unlock "ACH_MOUNTAIN")
      (CallFunction|UnlockPrint false))
    (:L_Battlefield
      (Steam|Unlock "ACH_BATTLEFIELD")
      (CallFunction|UnlockPrint false))
    (:L_Forest
      (Steam|Unlock "ACH_FOREST")
      (CallFunction|UnlockPrint false))))

(fn Interactedwith
  (params (Type :type String) (Bit%20id :type Integer))
  (bind _returnvalue (CallFunction|SteamUErIsSteamConnected))
  (if _returnvalue
    (switch string Type
      (:SHRINE
        (Development|PrintString 0 (Utilities|String|ToString(Integer) Bit%20id))
        (bind (_status _result) (CallFunction|UpdateStat "SHRINES" Bit%20id false false))
        ;[1 1 1] shrines
        (if _status
          (LocalVariables|SetCounter 0)
          (bind _enumvalue (|ForEachBP_SHRINES)
            (:LoopBody
              (if (Math|Conversions|ToBoolean(Integer) (Class|KismetMathLibrary|AndIntInt _result (Math|Float|Floor (Math|Float|Power 2.0 (Math|Conversions|ToFloat(Byte) _enumvalue)))))
                (bind _result_2 (Math|Integer|IncrementInt (LocalVariables|GetCounter))
                  (:%20%20
                    (Development|PrintString 0 (Utilities|String|JoinStringArray (Utilities|Array|MakeArray "Begin:" (Utilities|String|ToString(Float) (Math|Conversions|ToFloat(Byte) _enumvalue)) "|" (Utilities|String|ToString(Integer) (Math|Float|Floor (Math|Float|Power 2.0 (Math|Conversions|ToFloat(Byte) _enumvalue)))) " Counter: " (Utilities|String|ToString(Integer) (LocalVariables|GetCounter)) "Orginal" (Utilities|String|ToString(Integer) _result)) "  "))))
                (else
                  (Development|PrintString 0 (Utilities|String|EnumtoString _enumvalue)))))
            (:then
              (CallFunction|UpdateStat "SHRINEVISITED" _result_2 false true)))
          (else
            (Development|PrintString 0 "Failed to update the SHRINES"))))
      (:INN
        (bind (_status_2 _result_3) (CallFunction|UpdateStat "INNS" Bit%20id false false))
        ;[1 1 1] Innes
        (if _status_2
          (LocalVariables|SetCounter 0)
          (bind _enumvalue_2 (|ForEachBP_INNS)
            (:LoopBody
              (if (Math|Conversions|ToBoolean(Integer) (Class|KismetMathLibrary|AndIntInt _result_3 (Math|Float|Floor (Math|Float|Power 2.0 (Math|Conversions|ToFloat(Byte) _enumvalue_2)))))
                (bind _result_4 (Math|Integer|IncrementInt (LocalVariables|GetCounter)))))
            (:then
              (Development|PrintString 0 (Utilities|String|ToString(Integer) _result_4))
              (bind _status_3 (CallFunction|UpdateStat "ALLINNS" _result_4 false true))
              (Development|PrintString 0 (Utilities|String|ToString(Boolean) _status_3))))
          (else
            (Development|PrintString 0 "Failed to update the INNS")))))))

(fn UpdateStat
  (params (Stats :type String) (Input :type Integer) (Addition :type Boolean) (Replace :type Boolean))
  (bind _returnvalue (CallFunction|SteamUErIsSteamConnected))
  (if _returnvalue
    (bind _returnvalue_2 (CallFunction|SteamUErGlobalStatsReady))
    (if _returnvalue_2
      (bind (_value _returnvalue_3) (CallFunction|SteamUErGetStatIntBool Stats))
      (if _returnvalue_3
        (if Replace
          ;[1 1 1] replace
          (bind _returnvalue_4 (CallFunction|SteamUErSetStatInt Stats Input))
          (return _returnvalue_4 Input)
          (else
            ;[1 1 1] Add
            (if Addition
              (bind _returnvalue_5 (CallFunction|SteamUErSetStatInt Stats (+ _value Input)))
              (return _returnvalue_5 (+ _value Input))
              (else
                ;[1 1 1] binary OR
                (bind _returnvalue_6 (CallFunction|SteamUErSetStatInt Stats (Class|KismetMathLibrary|OrIntInt _value Input)))
                (return _returnvalue_6 (Class|KismetMathLibrary|OrIntInt _value Input))))))
        (else
          (Development|PrintString 0 "could not get stat")
          (return false 0)))
      (else
        (Development|PrintString 0 "global data not ready")
        (return _returnvalue_2 0)))
    (else
      (Development|PrintString 0 "not connected to steam")
      (return _returnvalue 0))))