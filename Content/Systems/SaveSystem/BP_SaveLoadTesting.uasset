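; Debug actor for manually testing the save system through keyboard shortcuts.
; It enables player input on BeginPlay, then binds separate keys to save, load, respawn, check whether a save exists, and delete the save.
; Each key prints an on-screen confirmation, or the result for the existence check.
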(event EventBeginPlay
  (Input|EnableInput (Game|GetPlayerController 0)))

(event Collision|EventActorBeginOverlap
  (params (OtherActor :type Actor%20Object%20Reference)))

(event EventTick
  (params (DeltaSeconds :type Float%20%28single-precision%29)))

(event Input|KeyboardEvents|K
  (params (Key :type Key%20Structure :default "None"))
  (:Pressed
    (Class|SaveLibrary|SaveGame)
    (Development|PrintString "Saved")))

(event Input|KeyboardEvents|L
  (params (Key :type Key%20Structure :default "None"))
  (:Pressed
    (Class|SaveLibrary|LoadGame)
    (Development|PrintString "Loaded")))

(event Input|KeyboardEvents|M
  (params (Key :type Key%20Structure :default "None"))
  (:Pressed
    (Class|SaveLibrary|Respawn true)
    (Development|PrintString "Respawned")))

(event Input|KeyboardEvents|T
  (params (Key :type Key%20Structure :default "None"))
  (:Pressed
    (bind _returnvalue (Class|SaveLibrary|SaveExists))
    (Development|PrintString (Utilities|String|ToString(Boolean) _returnvalue))))

(event Input|KeyboardEvents|Y
  (params (Key :type Key%20Structure :default "None"))
  (:Pressed
    (Class|SaveLibrary|DeleteSave)
    (Development|PrintString "Delete saved game")))

(fn ConstructionScript)